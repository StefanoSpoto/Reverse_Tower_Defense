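; BP_UnitSpawner is an actor that repeatedly spawns BP_Unit at its own transform, with no limit on the count.
; BeginPlay waits SpawnDelay, then sets the CanSpawn flag.
; Tick checks that flag, clears it, spawns a unit and sets it again after another SpawnDelay, forming a timed loop without a timer.
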(event EventTick
  (params (DeltaSeconds :type Float%20%28single-precision%29))
  (if (Variables|Default|GetcanSpawn)
    (Variables|Default|SetcanSpawn false)
    (Game|SpawnActorfromClass "/Game/BluePrint/Units/BP_Unit.BP_Unit_C" (Transformation|GetActorTransform) "Undefined" "MultiplyWithRoot" 0 0)
    (Utilities|FlowControl|Delay (Variables|Spawn|GetspawnDelay))
    (Variables|Default|SetcanSpawn true)))

(event EventBeginPlay
  (Utilities|FlowControl|Delay (Variables|Spawn|GetspawnDelay))
  (Variables|Default|SetcanSpawn true))

(fn ConstructionScript)