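; BP_Unit is a unit that walks forward along path blocks, attacks barricades in its way and is destroyed at zero health.
; A downward trace finds the BP_PathBlock below and snaps rotation to its orientation near the cell center, skipping one specific orientation.
; Each tick, a forward trace detects BP_NewBarricade, halting movement and applying damage every frame until it is destroyed.
; Movement is an unswept per-frame offset, not scaled by delta time.
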(event Custom|TakeDamage
  (params (damage :type Float%20%28double-precision%29))
  (Variables|Unit|Sethealth (- (Variables|Unit|Gethealth) damage))
  (if (<= (Variables|Unit|Gethealth) 0.0)
    (Variables|Unit|Sethealth 0.0)
    (Actor|DestroyActor)))

(event EventBeginPlay
  (CallFunction|CheckforPath))

(event EventTick
  (params (DeltaSeconds :type Float%20%28single-precision%29))
  (Utilities|IsValid (Variables|Default|GetbarricateReference)
    (:Is%20Valid
      (if (Variables|/Game/BluePrint/Barricate/BP_NewBarricade.BP_NewBarricade_C|GetisDestroyed (Variables|Default|GetbarricateReference))
        (Variables|Default|SetcanMove true)
        (Variables|Default|SetbarricateReference 0)
        (else
          (CallFunction|CheckforWall :!label _label))))
    (:Is%20Not%20Valid
      (goto _label)))
  (if (Variables|Default|GetcanMove)
    (Transformation|AddActorWorldOffset (* (Transformation|GetActorForwardVector) (Variables|Unit|Getspeed)))
    (CallFunction|CheckforPath)))

(fn ConstructionScript)

(fn CheckforPath
  (bind _returnvalue (Transformation|GetActorLocation))
  (bind _outhit (Collision|LineTraceByChannel _returnvalue (+ _returnvalue "0.000000,0.000000,-200.000000") "TraceTypeQuery1" false 0 "None"))
  (bind _asbp_path_block (Utilities|Casting|CastToBP_PathBlock (.HitActor (Collision|BreakHitResult _outhit))))
  (bind _rotation (Default|GetPathCellOrientation _asbp_path_block))
  (if (not (Utilities|Operators|EqualEqual _rotation "180.000000,0.000000,0.000000" 0.0))
    (if (<= (- (Math|Vector|Distance(Vector) (Transformation|GetActorLocation) (Transformation|GetActorLocation (.HitActor (Collision|BreakHitResult _outhit)))) 1e+02) 0.01)
      (Transformation|SetActorRotation _rotation))))

(fn CheckforWall
  (bind _returnvalue (Transformation|GetActorLocation))
  (bind _outhit (Collision|LineTraceByChannel _returnvalue (+ _returnvalue (* (Transformation|GetActorForwardVector) (Variables|Default|GetforwardRaycastLength))) "TraceTypeQuery1" false 0 "None"))
  (bind _asbp_new_barricade (Utilities|Casting|CastToBP_NewBarricade (.HitActor (Collision|BreakHitResult _outhit))))
  (Variables|Default|SetbarricateReference _asbp_new_barricade)
  (if (Variables|/Game/BluePrint/Barricate/BP_NewBarricade.BP_NewBarricade_C|GetisDestroyed _asbp_new_barricade)
    (Variables|Default|SetcanMove true)
    (else
      (Variables|Default|SetcanMove false)
      (Default|TakeDamage _asbp_new_barricade (Variables|Unit|Getdamage))))
  (return))