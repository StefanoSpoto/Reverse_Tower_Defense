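; Grid path block actor whose cube shows a path direction and can be switched by clicking.
; SetPathBlock supplies the starting orientation, two alternate orientations and whether switching is allowed.
; Clicking the cube toggles between the two alternates when permitted, printing a debug message either way.
; Each orientation maps to a fixed world rotation of the cube: compass directions turn it, while Stationary flips it over.
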(event OnClicked(Cube)
  (params (TouchedComponent :type Primitive%20Component%20Object%20Reference) (ButtonPressed :type Key%20Structure :default "None"))
  (CallFunction|SwitchOrientation))

(event EventBeginPlay)

(event Collision|EventActorBeginOverlap
  (params (OtherActor :type Actor%20Object%20Reference)))

(fn ConstructionScript)

(fn SetPathBlock
  (params (defaultOrientation :type E_PathOrientation%20Enum :default "NewEnumerator0") (canSwitch :type Boolean) (orientation_A :type E_PathOrientation%20Enum :default "NewEnumerator0") (orientation_B :type E_PathOrientation%20Enum :default "NewEnumerator0"))
  (bind _output_get (Variables|Path|Setorientation defaultOrientation))
  (Variables|OrientationSwitch|SetcanSwitch canSwitch)
  (Variables|OrientationSwitch|Setorientation_A orientation_A)
  (Variables|OrientationSwitch|Setorientation_B orientation_B)
  (CallFunction|SetPathCellOrientation _output_get))

(fn SetPathCellOrientation
  (params (orientation :type E_PathOrientation%20Enum :default "NewEnumerator0"))
  (bind _output_get (Variables|Path|Setorientation orientation))
  (switch Utilities|FlowControl|Switch|SwitchonE_PathOrientation _output_get
    (:NewEnumerator0
      (CallFunction|SetCellRotation "0, 0, 0"))
    (:NewEnumerator1
      (CallFunction|SetCellRotation "0.000000,180.000000,0.000000"))
    (:NewEnumerator2
      (CallFunction|SetCellRotation "0.000000,90.000000,0.000000"))
    (:NewEnumerator3
      (CallFunction|SetCellRotation "0.000000,270.000000,0.000000"))
    (:NewEnumerator4
      (CallFunction|SetCellRotation "180.000000,0.000000,0.000000"))))

(fn SetCellRotation
  (params (rotation :type Rotator))
  (Transformation|SetWorldRotation (Variables|Default|GetCube) rotation false false))

(fn GetPathCellOrientation
  (return (Transformation|GetWorldRotation (Variables|Default|GetCube))))

(fn SwitchOrientation
  (if (Variables|OrientationSwitch|GetcanSwitch)
    (Development|PrintString "switch")
    (if (Utilities|Enum|Equal(Enum) (Variables|Path|Getorientation) (Variables|OrientationSwitch|Getorientation_A))
      (Variables|Path|Setorientation (Variables|OrientationSwitch|Getorientation_B))
      (else
        (Variables|Path|Setorientation (Variables|OrientationSwitch|Getorientation_A))))
    (CallFunction|SetPathCellOrientation (Variables|Path|Getorientation))
    (else
      (Development|PrintString "cant switc !!!"))))