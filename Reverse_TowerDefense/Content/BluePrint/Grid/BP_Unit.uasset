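; BP_Unit is a grid unit that walks itself along path blocks and destroys itself on reaching a BP_FinalBlock.
; North, west and east probe points trace downward for BPI_IPath actors, collecting hit locations as candidate steps.
; CheckPosition picks the next target, skipping the recorded previous location when several candidates exist, and faces it.
; Tick moves the unit forward by a per-frame offset, rechecking upon arrival.
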(event EventBeginPlay
  (CallFunction|CheckPosition))

(event EventTick
  (params (DeltaSeconds :type Float%20%28single-precision%29))
  (if (Variables|Default|GetcanMove)
    (if (< (Math|Vector|Distance(Vector) (Transformation|GetActorLocation) (Variables|Default|GetnewLocation)) 2.0)
      (Variables|Default|SetcanMove false)
      (CallFunction|CheckPosition)
      (else
        (Transformation|AddActorWorldOffset (* (Variables|Default|GetmoveDirection) (Variables|Unit|Getspeed)))))))

(fn ConstructionScript)

(fn CheckRaycastforPath
  (params (RaycastStartingPoint :type Vector))
  (bind _outhit (Collision|LineTraceByChannel RaycastStartingPoint (+ RaycastStartingPoint "0.000000,0.000000,-200.000000") "TraceTypeQuery1" false 0 "None"))
  (if (Utilities|DoesObjectImplementInterface (.HitActor (Collision|BreakHitResult _outhit)) "/Game/BluePrint/Grid/BPI_IPath.BPI_IPath_C")
    (Utilities|Array|Add (Variables|Default|GetpathPositions) (.Location (Collision|BreakHitResult _outhit)))))

(fn CheckPosition
  (CallFunction|CheckRaycastforPath (Transformation|GetWorldLocation (Variables|Default|GetN_RaycastPoint)))
  (CallFunction|CheckRaycastforPath (Transformation|GetWorldLocation (Variables|Default|GetW_RaycastPoint)))
  (CallFunction|CheckRaycastforPath (Transformation|GetWorldLocation (Variables|Default|GetE_RaycastPoint)))
  (if (== (Utilities|Array|Length (Variables|Default|GetpathPositions)) 1)
    (bind _output_get (Variables|Default|SetnewLocation (Utilities|Array|Get(acopy) (Variables|Default|GetpathPositions))))
    (Variables|Default|SetnewLocation (Math|Vector|MakeVector (.x _output_get) (.y _output_get) (.z (Transformation|GetActorLocation))))
    (CallFunction|CheckforPreviousLocation)
    (Transformation|SetActorRotation (Math|Conversions|RotationFromXVector (Math|Vector|Normalize (- (Variables|Default|GetnewLocation) (Transformation|GetActorLocation)))))
    (Variables|Default|SetmoveDirection (Transformation|GetActorForwardVector))
    (Variables|Default|SetcanMove true)
    (else
      (for _array_element (Variables|Default|GetpathPositions)
        (if (Utilities|Operators|EqualEqual _array_element (Variables|Default|GetpreviousLocation) 0.0)
          (Utilities|Array|RemoveItem (Variables|Default|GetpathPositions) _array_element)
          (else
            (bind _output_get_2 (Variables|Default|SetnewLocation _array_element))
            (Variables|Default|SetnewLocation (Math|Vector|MakeVector (.x _output_get_2) (.y _output_get_2) (.z (Transformation|GetActorLocation)))))))
      (CallFunction|CheckforPreviousLocation)
      (Transformation|SetActorRotation (Math|Conversions|RotationFromXVector (Math|Vector|Normalize (- (Variables|Default|GetnewLocation) (Transformation|GetActorLocation)))))
      (Variables|Default|SetmoveDirection (Transformation|GetActorForwardVector))
      (Variables|Default|SetcanMove true))))

(fn CheckforPreviousLocation
  (bind _outhit (Collision|LineTraceByChannel (Transformation|GetActorLocation) (+ (Transformation|GetActorLocation) "0.000000,0.000000,-200.000000") "TraceTypeQuery1" false 0 "None"))
  (Utilities|Casting|CastToBP_Unit (.HitActor (Collision|BreakHitResult _outhit))
    (:CastFailed
      (Utilities|Casting|CastToBP_PathBlock (.HitActor (Collision|BreakHitResult _outhit))
        (:then
          (Variables|Default|SetpreviousLocation (.Location (Collision|BreakHitResult _outhit))))
        (:CastFailed
          (Utilities|Casting|CastToBP_FinalBlock (.HitActor (Collision|BreakHitResult _outhit)))
          (Actor|DestroyActor))))))