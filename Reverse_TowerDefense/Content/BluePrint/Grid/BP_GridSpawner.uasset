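; Grid spawner actor that builds a block grid on BeginPlay and carves a predefined path into it.
; Nested row and column loops spawn GridBlock actors by offset, recording indices and references in Grid; each new row resets Y to zero.
; PlacePath matches Path coordinates against Grid, destroying matched blocks and spawning BP_PathBlock in their place, or BP_FinalBlock for the last path entry.
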(event EventBeginPlay
  (Variables|Grid|SetcurrentPos (Variables|Grid|GetstartingPos))
  (for _index (range 1 (Variables|Grid|Getrows))
    (for _index_2 (range 1 (Variables|Grid|Getcolumns))
      (bind _returnvalue (Game|SpawnActorfromClass (Variables|Grid|GetgridBlock) (Math|Transform|MakeTransform (Variables|Grid|GetcurrentPos) "0, 0, 0" "1.000000,1.000000,1.000000") "AlwaysSpawn" "MultiplyWithRoot" 0 0))
      (Utilities|Array|Add (Variables|Default|Getgrid) (Utilities|Struct|MakeBS_GridIndex _index _index_2 _returnvalue))
      (Variables|Grid|SetcurrentPos (Math|Vector|MakeVector (.x (+ (Math|Vector|MakeVector (.x (Variables|Grid|GetcurrentPos)) (.y (Variables|Grid|GetcurrentPos)) (.z (Variables|Grid|GetcurrentPos))) (Math|Vector|MakeVector 0.0 (.y (Variables|Grid|Getoffset)) 0.0))) (.y (+ (Math|Vector|MakeVector (.x (Variables|Grid|GetcurrentPos)) (.y (Variables|Grid|GetcurrentPos)) (.z (Variables|Grid|GetcurrentPos))) (Math|Vector|MakeVector 0.0 (.y (Variables|Grid|Getoffset)) 0.0))) (.z (+ (Math|Vector|MakeVector (.x (Variables|Grid|GetcurrentPos)) (.y (Variables|Grid|GetcurrentPos)) (.z (Variables|Grid|GetcurrentPos))) (Math|Vector|MakeVector 0.0 (.y (Variables|Grid|Getoffset)) 0.0)))))
      (if (== _index_2 (Variables|Grid|Getcolumns))
        (Variables|Grid|SetcurrentPos (Math|Vector|MakeVector (+ (.x (Variables|Grid|GetcurrentPos)) (.x (Variables|Grid|Getoffset))) 0.0 (.z (Variables|Grid|GetcurrentPos)))))))
  (CallFunction|PlacePath (Variables|Grid|Getpath) (Variables|Default|Getgrid)))

(fn ConstructionScript)

(fn PlacePath
  (params (path :type Array%20of%20BS%20Grid%20Index%20Structures) (grid :type Array%20of%20BS%20Grid%20Index%20Structures))
  (for (_array_element _array_index) path
    (for _array_element_2 grid
      (if (and (== (.x _array_element_2) (.x _array_element)) (== (.y _array_element_2) (.y _array_element)))
        (if (== (Utilities|Array|LastIndex path) _array_index)
          (Game|SpawnActorfromClass "/Game/BluePrint/Grid/BP_FinalBlock.BP_FinalBlock_C" (Math|Transform|MakeTransform (Transformation|GetActorLocation (.block _array_element_2)) "0, 0, 0" "1.000000,1.000000,1.000000") "AlwaysSpawn" "MultiplyWithRoot" 0 0)
          (else
            (Game|SpawnActorfromClass "/Game/BluePrint/Grid/BP_PathBlock.BP_PathBlock_C" (Math|Transform|MakeTransform (Transformation|GetActorLocation (.block _array_element_2)) "0, 0, 0" "1.000000,1.000000,1.000000") "Undefined" "MultiplyWithRoot" 0 0)))
        (Actor|DestroyActor (.block _array_element_2))))))