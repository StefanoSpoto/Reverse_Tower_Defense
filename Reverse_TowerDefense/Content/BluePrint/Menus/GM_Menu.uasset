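; GM_Menu is the menu game mode that drives the pre-game hero and army selection screens.
; On BeginPlay it creates and shows W_HeroSelection, then lazily creates W_ArmySelection on first use and afterwards just makes it visible again.
; Going back hides the army menu and reveals hero selection.
; Add and remove troop functions cast to the army widget and forward the troop to it.
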(event EventBeginPlay
  (bind _returnvalue (UserInterface|CreateWidget "/Game/BluePrint/Menus/W_HeroSelection.W_HeroSelection_C"))
  (UserInterface|Viewport|AddtoViewport _returnvalue 0)
  (Variables|UI|SetheroSelectionMenu _returnvalue))

(fn ConstructionScript)

(fn GotoArmySelection
  (Utilities|IsValid (Variables|UI|GetarmySelectionMenu)
    (:Is%20Valid
      (Widget|SetVisibility (Variables|UI|GetarmySelectionMenu) "Visible"))
    (:Is%20Not%20Valid
      (bind _returnvalue (UserInterface|CreateWidget "/Game/BluePrint/Menus/W_ArmySelection.W_ArmySelection_C"))
      (UserInterface|Viewport|AddtoViewport _returnvalue 0)
      (Variables|UI|SetarmySelectionMenu _returnvalue))))

(fn GoBacktoChampionSelection
  (Widget|SetVisibility (Variables|UI|GetarmySelectionMenu) "Hidden")
  (Widget|SetVisibility (Variables|UI|GetheroSelectionMenu) "Visible"))

(fn AddTrooptoArmy
  (params (troop :type DA%20Troop%20Object%20Reference))
  (bind _asw_army_selection (Utilities|Casting|CastToW_ArmySelection (Variables|UI|GetarmySelectionMenu)))
  (Default|AddTroop _asw_army_selection troop))

(fn RemoveTrooptoArmy
  (params (troop :type DA%20Troop%20Object%20Reference))
  (bind _asw_army_selection (Utilities|Casting|CastToW_ArmySelection (Variables|UI|GetarmySelectionMenu)))
  (Default|RemoveTroop _asw_army_selection troop))