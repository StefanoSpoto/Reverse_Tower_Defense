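; BP_GridSpawner is a Blueprint that builds a grid of GridBlock actors when play begins.
; Nested loops over Rows and Columns spawn each block from StartingPos, stepping along Y by the Offset after every spawn and ignoring collisions.
; At the end of each row it advances X by the Offset and resets Y to world zero rather than to the starting Y.
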(event EventBeginPlay
  (Variables|Grid|SetcurrentPos (Variables|Grid|GetstartingPos))
  (for _index (range 1 (Variables|Grid|Getrows))
    (for _index_2 (range 1 (Variables|Grid|Getcolumns))
      (Game|SpawnActorfromClass (Variables|Grid|GetgridBlock) (Math|Transform|MakeTransform (Variables|Grid|GetcurrentPos) "0, 0, 0" "1.000000,1.000000,1.000000") "AlwaysSpawn" "MultiplyWithRoot" 0 0)
      (Variables|Grid|SetcurrentPos (Math|Vector|MakeVector (.x (+ (Math|Vector|MakeVector (.x (Variables|Grid|GetcurrentPos)) (.y (Variables|Grid|GetcurrentPos)) (.z (Variables|Grid|GetcurrentPos))) (Math|Vector|MakeVector 0.0 (.y (Variables|Grid|Getoffset)) 0.0))) (.y (+ (Math|Vector|MakeVector (.x (Variables|Grid|GetcurrentPos)) (.y (Variables|Grid|GetcurrentPos)) (.z (Variables|Grid|GetcurrentPos))) (Math|Vector|MakeVector 0.0 (.y (Variables|Grid|Getoffset)) 0.0))) (.z (+ (Math|Vector|MakeVector (.x (Variables|Grid|GetcurrentPos)) (.y (Variables|Grid|GetcurrentPos)) (.z (Variables|Grid|GetcurrentPos))) (Math|Vector|MakeVector 0.0 (.y (Variables|Grid|Getoffset)) 0.0)))))
      (if (== _index_2 (Variables|Grid|Getcolumns))
        (Variables|Grid|SetcurrentPos (Math|Vector|MakeVector (+ (.x (Variables|Grid|GetcurrentPos)) (.x (Variables|Grid|Getoffset))) 0.0 (.z (Variables|Grid|GetcurrentPos))))))))

(fn ConstructionScript)