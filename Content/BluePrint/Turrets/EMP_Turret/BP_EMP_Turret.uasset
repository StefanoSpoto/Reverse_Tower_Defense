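; EMP turret Blueprint, built on a parent turret, that emits an expanding area-of-effect pulse when its turret effect fires.
; The effect spawns an area actor at the range collision's location, passing it the expansion duration and contact damage.
; A timeline, rate-scaled by the expansion duration at BeginPlay, lerps the actor's range from a small starting size out to the range sphere's radius.
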(event EventTurretEffect
  (bind _returnvalue (Game|SpawnActorfromClass (Variables|SpecialEffect|GetArea%20Of%20Effect) (Math|Transform|MakeTransform (Transformation|GetWorldLocation (Variables|Default|GetRangeCollision)) "0, 0, 0" "1.000000,1.000000,1.000000") "AlwaysSpawn" "MultiplyWithRoot" 0 1e+02 (Variables|SpecialEffect|GetExpansion%20Duration) (Variables|Default|Getdamage) 1.0 0))
  (bind _output_get (Variables|Default|SetAreaOfEffect _returnvalue))
  (Default|SetDuration _output_get)
  (bind _alpha (Timeline|AreaOfEffect%20Expansion%20Timeline PlayFromStart)
    (:Update
      (Default|SetRange (Variables|Default|GetAreaOfEffect) (Math|Float|Lerp 1e+02 (Variables|/Script/Engine.SphereComponent|GetSphereRadius (Variables|Default|GetRangeCollision)) _alpha)))))

(event EventBeginPlay
  (|CallParentFunction)
  (Components|Timeline|SetPlayRate (Variables|Default|GetAreaOfEffect%20Expansion%20Timeline) (/ 1.0 (Variables|SpecialEffect|GetExpansion%20Duration))))

(fn ConstructionScript
  (|CallParentFunction))