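; Slowing area for the slowing turret that reduces the speed of units it affects.
; Its SpecialEffect event sets a unit's speed to its Speed value scaled by SlowingPercentage.
; When a BP_Unit stops overlapping CollisionArea, SetSpeed is called with the unscaled Speed value.
; The trigger for SpecialEffect lies outside this graph, which has no active BeginPlay, overlap-begin or Tick logic.
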(event OnComponentEndOverlap(CollisionArea)
  (params (OverlappedComponent :type Primitive%20Component%20Object%20Reference) (OtherActor :type Actor%20Object%20Reference) (OtherComp :type Primitive%20Component%20Object%20Reference) (OtherBodyIndex :type Integer))
  (bind _asbp_unit (Utilities|Casting|CastToBP_Unit OtherActor))
  (Default|SetSpeed _asbp_unit (Variables|/Game/BluePrint/Units/BP_Unit.BP_Unit_C|Getspeed _asbp_unit)))

(event EventBeginPlay
  (|CallParentFunction) ; This node is disabled and will not be called.\nDrag off pins to build functionality.
)

(event Collision|EventActorBeginOverlap
  (params (OtherActor :type Actor%20Object%20Reference))
  (|CallParentFunction OtherActor) ; This node is disabled and will not be called.\nDrag off pins to build functionality.
)

(event EventTick
  (params (DeltaSeconds :type Float%20%28single-precision%29))
  (|CallParentFunction DeltaSeconds) ; This node is disabled and will not be called.\nDrag off pins to build functionality.
)

(event EventSpecialEffect
  (params (Unit :type BP%20Unit%20Object%20Reference))
  (Default|SetSpeed Unit (* (Variables|/Game/BluePrint/Units/BP_Unit.BP_Unit_C|Getspeed Unit) (Variables|SpecialEffect|GetslowingPercentage))))

(fn ConstructionScript
  (|CallParentFunction))