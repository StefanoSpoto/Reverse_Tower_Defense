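; Turret actor that fires projectiles at BP_Unit actors inside its range sphere.
; Overlaps maintain the target list; Shoot runs on entry and after recharge, picks an aggro-able unit, then calls TurretEffect to spawn a BulletType projectile.
; Tick turns the shoot pivot toward the target on enabled axes.
; Game mode events sync time dilation and prune targets; hover events toggle range mesh and info widget.
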(event OnComponentEndOverlap(RangeCollision)
  (params (OverlappedComponent :type Primitive%20Component%20Object%20Reference) (OtherActor :type Actor%20Object%20Reference) (OtherComp :type Primitive%20Component%20Object%20Reference) (OtherBodyIndex :type Integer))
  ;[1 1 0.2812] Enter range
  (bind _asbp_unit (Utilities|Casting|CastToBP_Unit OtherActor))
  (Utilities|IsValid _asbp_unit
    (:Is%20Valid
      (if (Utilities|Array|ContainsItem (Variables|Turret|GetTarget) _asbp_unit)
        (Utilities|Array|RemoveItem (Variables|Turret|GetTarget) _asbp_unit)
        (Variables|/Game/BluePrint/Units/BP_Unit.BP_Unit_C|SetisAggroed _asbp_unit false)))))

(event OnComponentBeginOverlap(RangeCollision)
  (params (OverlappedComponent :type Primitive%20Component%20Object%20Reference) (OtherActor :type Actor%20Object%20Reference) (OtherComp :type Primitive%20Component%20Object%20Reference) (OtherBodyIndex :type Integer) (bFromSweep :type Boolean) (SweepResult :type Hit%20Result%20Structure%20%28by%20ref%29))
  ;[1 1 0.2812] Enter range
  (bind _asbp_unit (Utilities|Casting|CastToBP_Unit OtherActor))
  (Utilities|IsValid _asbp_unit
    (:Is%20Valid
      (Utilities|Array|Add (Variables|Turret|GetTarget) _asbp_unit)
      (CallFunction|Shoot))))

(event Custom|Change%20Custom%20Time%20Dilation
  (params (newTimeDilation :type Float%20%28double-precision%29))
  (Variables|Default|SetCustomTimeDilation newTimeDilation))

(event Custom|RemoveFromTargets
  (params (unit :type BP%20Unit%20Object%20Reference))
  (if (Utilities|Array|ContainsItem (Variables|Turret|GetTarget) unit)
    (Utilities|Array|RemoveItem (Variables|Turret|GetTarget) unit)))

(event Custom|Turret%20Effect
  ;[0.3499 0.1172 0.5] Turret Effect
  (CallFunction|ShootProjectile))

(event Custom|On%20Unhover%20Actor
  (params (Actor%20Being%20Hovered :type Actor%20Object%20Reference))
  (if (not (== Actor%20Being%20Hovered self))
    (CallFunction|SetUnhover)))

(event Custom|Shoot
  ;[1 0.3021 0.3021] Shoot
  (Utilities|IsValid (Utilities|Array|Get(acopy) (Variables|Turret|GetTarget) (Variables|Turret|GettargetIndex))
    (:Is%20Valid
      (if (Variables|/Game/BluePrint/Units/BP_Unit.BP_Unit_C|GetcanBeAggro (Utilities|Array|Get(acopy) (Variables|Turret|GetTarget) (Variables|Turret|GettargetIndex)))
        (Utilities|IsValid (Utilities|Array|Get(acopy) (Variables|Turret|GetTarget) (Variables|Turret|GettargetIndex)) :!label _label
          (:Is%20Valid
            (if (Variables|Default|GetcheckAnotherUnit)
              (if (== (Variables|Turret|GettargetIndex) 0)
                (Variables|Default|SetcheckAnotherUnit false)
                (else
                  (Variables|/Game/BluePrint/Units/BP_Unit.BP_Unit_C|SetisAggroed (Utilities|Array|Get(acopy) (Variables|Turret|GetTarget) (Variables|Turret|GettargetIndex)) true :!label _label_2)
                  (CallFunction|TurretEffect)
                  (Variables|Turret|SettargetIndex 0)
                  (Variables|Default|SetcheckAnotherUnit false)))
              (else
                (goto _label_2)))))
        (else
          (Variables|Default|SetcheckAnotherUnit true)
          (bind (_array_element _array_index) (Utilities|Array|ForEachLoopwithBreak (Variables|Turret|GetTarget) :!label _label_3)
            (:LoopBody
              (if (Variables|/Game/BluePrint/Units/BP_Unit.BP_Unit_C|GetcanBeAggro _array_element)
                (Variables|Turret|SettargetIndex _array_index)
                (goto _label_3 Break)))
            (:Completed
              (goto _label))))))))

(event Custom|Rotate%20Shoot%20Point%20Towards%20Target
  (bind _targetindex (Variables|Turret|GettargetIndex))
  (bind _target (Variables|Turret|GetTarget))
  (bind _rotatingaxis (Variables|Turret|GetrotatingAxis))
  (bind _output (Utilities|Array|Get(acopy) _target _targetindex))
  (Utilities|IsValid _output
    (:Is%20Valid
      (Utilities|FlowControl|Sequence
        (:then_0
          (if (.xroll _rotatingaxis)
            (CallFunction|RotateAxisX _output)))
        (:then_1
          (if (.ypitch _rotatingaxis)
            (CallFunction|RotateAxisY _output)))
        (:then_2
          (if (.zyaw _rotatingaxis)
            (CallFunction|RotateAxisZ _output)))))))

(event Custom|First%20Turn%20Towards%20Target
  (params (UnitTarget :type Actor%20Object%20Reference))
  (bind _turret_shootpointobject (Variables|Default|GetTurret%20ShootPointObject))
  (bind _returnvalue (Transformation|GetWorldRotation _turret_shootpointobject))
  (bind _alpha (Timeline|RotateToTarget%20Timeline PlayFromStart)
    (:Update
      (Transformation|SetWorldRotation (Variables|Default|GetTurret%20ShootPointObject) (Math|Rotator|Lerp(Rotator) (Transformation|GetWorldRotation (Variables|Default|GetTurret%20ShootPointObject)) (Math|Rotator|MakeRotator (.roll _returnvalue) (.pitch _returnvalue) (.yaw (Math|Rotator|FindLookatRotation (Transformation|GetWorldLocation _turret_shootpointobject) (Transformation|GetActorLocation UnitTarget)))) _alpha true) false false))))

(event EventTick
  (params (DeltaSeconds :type Float%20%28single-precision%29))
  (Utilities|FlowControl|Sequence
    (:then_0
      ;[0.401 1 0.401] Shoot recharge timer
      (bind _output_get (Variables|Default|SetrechargeCurrentTime (+ DeltaSeconds (Variables|Default|GetrechargeCurrentTime))))
      (if (> _output_get (Variables|Turret|GetshootRechargeTime))
        (if (Variables|Default|GetcanShoot)
          (if (> (Utilities|Array|Length (Variables|Turret|GetTarget)) 0)
            (CallFunction|Shoot)))))
    (:then_1
      (CallFunction|RotateShootPointTowardsTarget))))

(event EventBeginPlay
  (EventDispatchers|BindEventtoOnChangeTimeDilation (CallFunction|GetGMLevelGameMode) (delegate Custom|Change%20Custom%20Time%20Dilation))
  (bind _asw_turret_name (Utilities|Casting|CastToW_TurretName (UserInterface|GetWidget (Variables|Default|GetTurretInfo))))
  (Default|SetStats _asw_turret_name (Variables|Turret|Getname) (Variables|Turret|Getdamage))
  (EventDispatchers|BindEventtoOnRemoveUnitfromTurretTargets (CallFunction|GetGMLevelGameMode) (delegate Custom|RemoveFromTargets))
  (EventDispatchers|BindEventtoOnUnhoverAllHoverableActors (CallFunction|GetBPLevelPlayerController) (delegate Custom|On%20Unhover%20Actor)))

(event EventSetHover
  ;[0 1 1] Hover
  (Rendering|SetVisibility (Variables|Default|GetRange%20Mesh) true false)
  (Rendering|SetVisibility (Variables|Default|GetTurretInfo) true false))

(event EventSetUnhover
  ;[0 1 1] Hover
  (Rendering|SetVisibility (Variables|Default|GetRange%20Mesh) false false)
  (Rendering|SetVisibility (Variables|Default|GetTurretInfo) false false)
  (CallFunction|ShowOutline false))

(event EventShowOutline
  (params (show :type Boolean))
  ;[0 1 1] Hover
  (Rendering|SetRenderCustomDepth (Variables|Default|GetTurret%20Body) show))

(fn ConstructionScript
  (bind _range (Variables|Turret|Getrange))
  (bind _returnvalue (/ _range 5e+01))
  (Components|Sphere|SetSphereRadius (Variables|Default|GetRangeCollision) _range true)
  (Transformation|SetWorldScale3D (Variables|Default|GetRange%20Mesh) (Math|Vector|MakeVector _returnvalue _returnvalue 0.01)))

(fn ShootProjectile
  (bind _bullettype (Variables|Turret|GetbulletType))
  (if (Utilities|IsValidClass _bullettype)
    (bind _returnvalue (Game|SpawnActorfromClass _bullettype (Math|Transform|MakeTransform (Transformation|GetWorldLocation (Variables|Default|GetArrow)) "0, 0, 0" "1.000000,1.000000,1.000000") "AlwaysSpawn" "MultiplyWithRoot" 0 0))
    (Default|SetProjectileStats _returnvalue (Variables|Turret|Getdamage) (Variables|Turret|GetprojectileSpeed) (Variables|/Game/BluePrint/Units/BP_Unit.BP_Unit_C|GetDefaultSceneRoot (Utilities|Array|Get(acopy) (Variables|Turret|GetTarget) (Variables|Turret|GettargetIndex))) (Variables|Default|GetCustomTimeDilation))
    (Variables|Default|SetrechargeCurrentTime 0.0)))

(fn RotateAxisX
  (params (Unit%20Target :type Actor%20Object%20Reference))
  (bind _shootpointpivot (Variables|Default|GetShootPointPivot))
  (bind _returnvalue (Transformation|GetWorldRotation _shootpointpivot))
  (Transformation|SetWorldRotation (Variables|Default|GetShootPointPivot) (Math|Rotator|MakeRotator (.roll (Math|Rotator|FindLookatRotation (Transformation|GetWorldLocation (Variables|Default|GetShootPointPivot)) (Transformation|GetActorLocation Unit%20Target))) (.pitch _returnvalue) (.yaw _returnvalue)) false false))

(fn RotateAxisY
  (params (Unit%20Target :type Actor%20Object%20Reference))
  (bind _shootpointpivot (Variables|Default|GetShootPointPivot))
  (bind _returnvalue (Transformation|GetWorldRotation _shootpointpivot))
  (Transformation|SetWorldRotation (Variables|Default|GetShootPointPivot) (Math|Rotator|MakeRotator (.roll _returnvalue) (.pitch (Math|Rotator|FindLookatRotation (Transformation|GetWorldLocation (Variables|Default|GetShootPointPivot)) (Transformation|GetActorLocation Unit%20Target))) (.yaw _returnvalue)) false false))

(fn RotateAxisZ
  (params (Unit%20Target :type Actor%20Object%20Reference))
  (bind _shootpointpivot (Variables|Default|GetShootPointPivot))
  (bind _returnvalue (Transformation|GetWorldRotation _shootpointpivot))
  (Transformation|SetWorldRotation (Variables|Default|GetShootPointPivot) (Math|Rotator|MakeRotator (.roll _returnvalue) (.pitch _returnvalue) (.yaw (Math|Rotator|FindLookatRotation (Transformation|GetWorldLocation (Variables|Default|GetShootPointPivot)) (Transformation|GetActorLocation Unit%20Target)))) false false))

(fn GetHoverDelay
  (return (Variables|UI|GethoverDelay)))