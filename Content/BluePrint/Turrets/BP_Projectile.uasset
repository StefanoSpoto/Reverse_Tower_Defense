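; BP_Projectile is a homing turret projectile that damages the first BP_Unit it overlaps, then destroys itself.
; SetProjectileStats supplies damage, speed, target and time dilation, then activates the homing movement.
; On hit, SpecialEffect optionally spawns a DamageArea actor before KillUnit receives the kill result.
; Custom time dilation follows game mode changes and passes to the spawned area, while Niagara receives it only at setup.
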(event OnComponentBeginOverlap(Sphere)
  (params (OverlappedComponent :type Primitive%20Component%20Object%20Reference) (OtherActor :type Actor%20Object%20Reference) (OtherComp :type Primitive%20Component%20Object%20Reference) (OtherBodyIndex :type Integer) (bFromSweep :type Boolean) (SweepResult :type Hit%20Result%20Structure%20%28by%20ref%29))
  (bind _asbp_unit (Utilities|Casting|CastToBP_Unit OtherActor))
  (bind (_iskilled _unit) (Default|TakeDamage _asbp_unit (Variables|Projectile|GetcontactDamage)))
  (CallFunction|SpecialEffect _unit)
  (Default|KillUnit _unit _iskilled)
  (Actor|DestroyActor))

(event Custom|Change%20Custom%20Time%20Dilation
  (params (newTimeDilation :type Float%20%28double-precision%29))
  (Variables|Default|SetCustomTimeDilation newTimeDilation))

(event Custom|SpecialEffect
  (params (unit :type BP%20Unit%20Object%20Reference))
  (bind _damagearea (Variables|Projectile|GetdamageArea))
  (if (Utilities|IsValidClass _damagearea)
    (Game|SpawnActorfromClass _damagearea (Transformation|GetActorTransform) "AlwaysSpawn" "MultiplyWithRoot" 0 2e+02 1.0 2e+01 (Variables|Default|GetCustomTimeDilation) 0)))

(event EventBeginPlay
  (EventDispatchers|BindEventtoOnChangeTimeDilation (CallFunction|GetGMLevelGameMode) (delegate Custom|Change%20Custom%20Time%20Dilation)))

(fn ConstructionScript)

(fn SetProjectileStats
  (params (damage :type Float%20%28double-precision%29) (speed :type Float%20%28double-precision%29) (target :type Scene%20Component%20Object%20Reference) (New%20Custom%20Time%20Dilation :type Float%20%28single-precision%29))
  (bind _projectilemovement (Variables|Default|GetProjectileMovement))
  (bind _projectilemovement_2 (Variables|Default|GetProjectileMovement))
  (bind _output_get (Variables|Default|SetCustomTimeDilation New%20Custom%20Time%20Dilation))
  (Class|NiagaraComponent|SetCustomTimeDilation (Variables|Default|GetNiagara) _output_get)
  (Variables|/Script/Engine.ProjectileMovementComponent|SetHomingTargetComponent _projectilemovement_2 target)
  (Variables|/Script/Engine.ProjectileMovementComponent|SetbIsHomingProjectile _projectilemovement_2 true)
  (Variables|Projectile|SetcontactDamage damage)
  (Variables|/Script/Engine.ProjectileMovementComponent|SetInitialSpeed _projectilemovement speed)
  (Variables|/Script/Engine.ProjectileMovementComponent|SetMaxSpeed _projectilemovement speed)
  (Components|Activation|Activate (Variables|Default|GetProjectileMovement) false))