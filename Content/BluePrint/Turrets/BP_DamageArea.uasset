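; Timed spherical damage area for turrets that hurts each BP_Unit entering it.
; On overlap it applies ContactDamage, calls the empty SpecialEffect hook, then passes the kill result to KillUnit.
; The construction script sizes the collision sphere and mesh from Range and sets the actor's lifespan from Duration.
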(event OnComponentBeginOverlap(CollisionArea)
  (params (OverlappedComponent :type Primitive%20Component%20Object%20Reference) (OtherActor :type Actor%20Object%20Reference) (OtherComp :type Primitive%20Component%20Object%20Reference) (OtherBodyIndex :type Integer) (bFromSweep :type Boolean) (SweepResult :type Hit%20Result%20Structure%20%28by%20ref%29))
  (bind _asbp_unit (Utilities|Casting|CastToBP_Unit OtherActor))
  (bind (_iskilled _unit) (Default|TakeDamage _asbp_unit (Variables|Area|GetContactDamage)))
  (CallFunction|SpecialEffect _asbp_unit)
  (Default|KillUnit _asbp_unit _iskilled))

(event Custom|SpecialEffect
  (params (Unit :type BP%20Unit%20Object%20Reference)))

(event EventBeginPlay)

(event Collision|EventActorBeginOverlap
  (params (OtherActor :type Actor%20Object%20Reference)))

(event EventTick
  (params (DeltaSeconds :type Float%20%28single-precision%29)))

(fn ConstructionScript
  (bind _range (Variables|Default|Getrange))
  (bind _returnvalue (/ _range 5e+01))
  (Components|Sphere|SetSphereRadius (Variables|Default|GetCollisionArea) _range true)
  (Transformation|SetWorldScale3D (Variables|Default|GetMesh) (Math|Vector|MakeVector _returnvalue _returnvalue _returnvalue))
  (Actor|SetLifeSpan (Variables|Area|GetDuration)))