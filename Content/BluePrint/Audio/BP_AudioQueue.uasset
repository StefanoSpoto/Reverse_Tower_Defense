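; BP_AudioQueue is a shuffled soundtrack player that starts a random track from the SoundTrack array on BeginPlay.
; Each time the Audio component finishes, it re-rolls random picks until it finds one absent from SoundTrackPlayed, so tracks avoid repeating within a cycle.
; When the play count reaches the array length, it clears that history and starts a new cycle with a track different from LastPlayedTrack.
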(event OnAudioFinished(Audio)
  (bind _audio (Variables|Default|GetAudio))
  (bind _audio_2 (Variables|Default|GetAudio))
  (bind _result (Math|Integer|IncrementInt (Variables|Audio|GetAudioPlayedCount))
    (:%20%20
      (if (== _result (Utilities|Array|Length (Variables|Audio|GetSoundTrack)))
        (Variables|Audio|SetAudioPlayedCount 0)
        (Utilities|Array|Clear (Variables|Audio|GetSoundTrackPlayed))
        (while (== (Variables|Audio|GetlastPlayedTrack) (Variables|Audio|GetselectedSoundTrack))
          (Variables|Audio|SetselectedSoundTrack (.OutItem (Utilities|Array|Random (Variables|Audio|GetSoundTrack)))))
        (Audio|Components|Audio|SetSound _audio (Variables|Audio|GetselectedSoundTrack))
        (Audio|Components|Audio|Play _audio 0.0)
        (Utilities|Array|Add (Variables|Audio|GetSoundTrackPlayed) (Variables|Audio|GetselectedSoundTrack))
        (else
          (Variables|Audio|SetselectedSoundTrack (.OutItem (Utilities|Array|Random (Variables|Audio|GetSoundTrack))))
          (while (Utilities|Array|ContainsItem (Variables|Audio|GetSoundTrackPlayed) (Variables|Audio|GetselectedSoundTrack))
            (Variables|Audio|SetselectedSoundTrack (.OutItem (Utilities|Array|Random (Variables|Audio|GetSoundTrack)))))
          (Audio|Components|Audio|SetSound _audio_2 (Variables|Audio|GetselectedSoundTrack))
          (Audio|Components|Audio|Play _audio_2 0.0)
          (Utilities|Array|Add (Variables|Audio|GetSoundTrackPlayed) (Variables|Audio|GetselectedSoundTrack))
          (Variables|Audio|SetlastPlayedTrack (Variables|Audio|GetselectedSoundTrack)))))))

(event EventBeginPlay
  (bind _audio (Variables|Default|GetAudio))
  (bind _output_get (Variables|Audio|SetselectedSoundTrack (.OutItem (Utilities|Array|Random (Variables|Audio|GetSoundTrack)))))
  (Audio|Components|Audio|SetSound _audio _output_get)
  (Audio|Components|Audio|Play _audio 0.0)
  (Utilities|Array|Add (Variables|Audio|GetSoundTrackPlayed) (Variables|Audio|GetselectedSoundTrack)))

(fn ConstructionScript)