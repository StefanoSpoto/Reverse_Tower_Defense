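; BP_CoinBag is a spinning coin pickup whose value is set through SetCoinsAmount.
; On BeginPlay it enables sphere overlaps after a short delay and binds to the level game mode's time dilation change, copying the new value to its CustomTimeDilation.
; When a BP_Unit overlaps the sphere, the unit collects the coins and the bag destroys itself.
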(event OnComponentBeginOverlap(Sphere)
  (params (OverlappedComponent :type Primitive%20Component%20Object%20Reference) (OtherActor :type Actor%20Object%20Reference) (OtherComp :type Primitive%20Component%20Object%20Reference) (OtherBodyIndex :type Integer) (bFromSweep :type Boolean) (SweepResult :type Hit%20Result%20Structure%20%28by%20ref%29))
  (bind _asbp_unit (Utilities|Casting|CastToBP_Unit OtherActor))
  (Default|CollectCoin _asbp_unit (Variables|Default|GetcoinsValue))
  (Actor|DestroyActor))

(event Custom|Change%20Custom%20Time%20Dilation
  (params (newTimeDilation :type Float%20%28double-precision%29))
  (Variables|Default|SetCustomTimeDilation newTimeDilation))

(event EventBeginPlay
  (EventDispatchers|BindEventtoOnChangeTimeDilation (CallFunction|GetGMLevelGameMode) (delegate Custom|Change%20Custom%20Time%20Dilation))
  (Utilities|FlowControl|Delay 0.5)
  (Variables|/Script/Engine.PrimitiveComponent|SetbGenerateOverlapEvents (Variables|Default|GetSphere) true))

(event EventTick
  (params (DeltaSeconds :type Float%20%28single-precision%29))
  (Class|Actor|AddActorWorldRotation (Math|Rotator|MakeRotator 0.0 0.0 (* DeltaSeconds (Variables|Default|GetrotationSpeed)))))

(fn ConstructionScript)

(fn SetCoinsAmount
  (params (coins :type Integer))
  (Variables|Default|SetcoinsValue coins))