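; BP_StructureSpawner places the level's turrets and strongholds at BeginPlay, scaling their stats for difficulty progression.
; Spawn-point counts per turret type fill a weighted pool; random picks land on randomly chosen, non-repeating platforms, though MINIGUN spawns a Standard turret.
; Strongholds spawn above random path blocks, rotated by block orientation.
; Game-instance percentages raise damage and stronghold resistance and shorten turret recharge time.
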(event EventBeginPlay
  (bind _asgi_reverse_td (CallFunction|GetGIReverseTD))
  (bind _turret_stats_increasment (Default|GetTurretStatsIncrementPercentage _asgi_reverse_td))
  (Variables|Default|SetturretStatsIncreasment _turret_stats_increasment)
  (bind _stronghold_stats_increasment (Default|GetStrongholdStatsIncrementPercentage _asgi_reverse_td))
  (Variables|Default|SetstrongholdStatsIncreasment _stronghold_stats_increasment)
  (CallFunction|FillTurretWeight)
  (CallFunction|SpawnTurret)
  (CallFunction|SpawnStronghold))

(fn ConstructionScript)

(fn FillTurretWeight
  (for _index (range 1 (Utilities|Struct|BreakS_StructureSpawnVariables (Variables|TurretSpawnPercentage|GetcurrentStructureVariables)))
    (Utilities|Array|Add (Variables|Default|GetturretWeights) "NewEnumerator0"))
  (for _index_2 (range 1 (Utilities|Struct|BreakS_StructureSpawnVariables (Variables|TurretSpawnPercentage|GetcurrentStructureVariables)))
    (Utilities|Array|Add (Variables|Default|GetturretWeights) "NewEnumerator1"))
  (for _index_3 (range 1 (Utilities|Struct|BreakS_StructureSpawnVariables (Variables|TurretSpawnPercentage|GetcurrentStructureVariables)))
    (Utilities|Array|Add (Variables|Default|GetturretWeights) "NewEnumerator2"))
  (for _index_4 (range 1 (Utilities|Struct|BreakS_StructureSpawnVariables (Variables|TurretSpawnPercentage|GetcurrentStructureVariables)))
    (Utilities|Array|Add (Variables|Default|GetturretWeights) "NewEnumerator3"))
  (for _index_5 (range 1 (Utilities|Struct|BreakS_StructureSpawnVariables (Variables|TurretSpawnPercentage|GetcurrentStructureVariables)))
    (Utilities|Array|Add (Variables|Default|GetturretWeights) "NewEnumerator5"))
  (for _index_6 (range 1 (Utilities|Struct|BreakS_StructureSpawnVariables (Variables|TurretSpawnPercentage|GetcurrentStructureVariables)))
    (Utilities|Array|Add (Variables|Default|GetturretWeights) "NewEnumerator6"))
  (for _index_7 (range 1 (Utilities|Struct|BreakS_StructureSpawnVariables (Variables|TurretSpawnPercentage|GetcurrentStructureVariables)))
    (Utilities|Array|Add (Variables|Default|GetturretWeights) "NewEnumerator7"))
  (for _index_8 (range 1 (Utilities|Struct|BreakS_StructureSpawnVariables (Variables|TurretSpawnPercentage|GetcurrentStructureVariables)))
    (Utilities|Array|Add (Variables|Default|GetturretWeights) "NewEnumerator8"))
  (for _index_9 (range 1 (Utilities|Struct|BreakS_StructureSpawnVariables (Variables|TurretSpawnPercentage|GetcurrentStructureVariables)))
    (Utilities|Array|Add (Variables|Default|GetturretWeights) "NewEnumerator9"))
  (for _index_10 (range 1 (Utilities|Struct|BreakS_StructureSpawnVariables (Variables|TurretSpawnPercentage|GetcurrentStructureVariables)))
    (Utilities|Array|Add (Variables|Default|GetturretWeights) "NewEnumerator10")))

(fn SpawnTurret
  (bind _currentstructurevariables (Variables|TurretSpawnPercentage|GetcurrentStructureVariables))
  (bind _turretnumber (Utilities|Struct|BreakS_StructureSpawnVariables _currentstructurevariables))
  (if (> _turretnumber 0)
    (while (< (LocalVariables|GetcurrentTurretNumber) _turretnumber)
      (LocalVariables|SetselectedPlatform (.OutItem (Utilities|Array|Random (Variables|SpawnPoints|GetturretPlatforms))))
      (switch Utilities|FlowControl|Switch|SwitchonE_TurretType (.OutItem (Utilities|Array|Random (Variables|Default|GetturretWeights)))
        (:NewEnumerator0
          (bind _returnvalue (Game|SpawnActorfromClass "/Game/BluePrint/Turrets/Standard_Turret/BP_Standard_Turret.BP_Standard_Turret_C" (Math|Transform|MakeTransform (Transformation|GetActorLocation (LocalVariables|GetselectedPlatform)) "0, 0, 0" "1.000000,1.000000,1.000000") "Undefined" "MultiplyWithRoot" 0 0))
          (LocalVariables|SetcurrentTurret _returnvalue))
        (:NewEnumerator1
          (bind _returnvalue_2 (Game|SpawnActorfromClass "/Game/BluePrint/Turrets/AOE_Turret/BP_AOE_Turret.BP_AOE_Turret_C" (Math|Transform|MakeTransform (Transformation|GetActorLocation (LocalVariables|GetselectedPlatform)) "0, 0, 0" "1.000000,1.000000,1.000000") "Undefined" "MultiplyWithRoot" 0 0))
          (LocalVariables|SetcurrentTurret _returnvalue_2))
        (:NewEnumerator2
          (bind _returnvalue_3 (Game|SpawnActorfromClass "/Game/BluePrint/Turrets/Freezing_Turret/BP_Freezing_Turret.BP_Freezing_Turret_C" (Math|Transform|MakeTransform (Transformation|GetActorLocation (LocalVariables|GetselectedPlatform)) "0, 0, 0" "1.000000,1.000000,1.000000") "Undefined" "MultiplyWithRoot" 0 0))
          (LocalVariables|SetcurrentTurret _returnvalue_3))
        (:NewEnumerator3
          (bind _returnvalue_4 (Game|SpawnActorfromClass "/Game/BluePrint/Turrets/DOT_Turret/BP_DOT_Turret.BP_DOT_Turret_C" (Math|Transform|MakeTransform (Transformation|GetActorLocation (LocalVariables|GetselectedPlatform)) "0, 0, 0" "1.000000,1.000000,1.000000") "Undefined" "MultiplyWithRoot" 0 0))
          (LocalVariables|SetcurrentTurret _returnvalue_4))
        (:NewEnumerator5
          (bind _returnvalue_5 (Game|SpawnActorfromClass "/Game/BluePrint/Turrets/Standard_Turret/BP_Standard_Turret.BP_Standard_Turret_C" (Math|Transform|MakeTransform (Transformation|GetActorLocation (LocalVariables|GetselectedPlatform)) "0, 0, 0" "1.000000,1.000000,1.000000") "Undefined" "MultiplyWithRoot" 0 0))
          (LocalVariables|SetcurrentTurret _returnvalue_5))
        (:NewEnumerator6
          (bind _returnvalue_6 (Game|SpawnActorfromClass "/Game/BluePrint/Turrets/SharpShooter_Turret/SharpShooter_Turret.SharpShooter_Turret_C" (Math|Transform|MakeTransform (Transformation|GetActorLocation (LocalVariables|GetselectedPlatform)) "0, 0, 0" "1.000000,1.000000,1.000000") "Undefined" "MultiplyWithRoot" 0 0))
          (LocalVariables|SetcurrentTurret _returnvalue_6))
        (:NewEnumerator7
          (bind _returnvalue_7 (Game|SpawnActorfromClass "/Game/BluePrint/Turrets/Slowing_Turret/BP_Slowing_Turret.BP_Slowing_Turret_C" (Math|Transform|MakeTransform (Transformation|GetActorLocation (LocalVariables|GetselectedPlatform)) "0, 0, 0" "1.000000,1.000000,1.000000") "Undefined" "MultiplyWithRoot" 0 0))
          (LocalVariables|SetcurrentTurret _returnvalue_7))
        (:NewEnumerator8
          (bind _returnvalue_8 (Game|SpawnActorfromClass "/Game/BluePrint/Turrets/Lightning_Turret/BP_Lightning_Turret.BP_Lightning_Turret_C" (Math|Transform|MakeTransform (Transformation|GetActorLocation (LocalVariables|GetselectedPlatform)) "0, 0, 0" "1.000000,1.000000,1.000000") "Undefined" "MultiplyWithRoot" 0 0))
          (LocalVariables|SetcurrentTurret _returnvalue_8))
        (:NewEnumerator9
          (bind _returnvalue_9 (Game|SpawnActorfromClass "/Game/BluePrint/Turrets/Corrosive_Turret/BP_Corrosive_Turret.BP_Corrosive_Turret_C" (Math|Transform|MakeTransform (Transformation|GetActorLocation (LocalVariables|GetselectedPlatform)) "0, 0, 0" "1.000000,1.000000,1.000000") "Undefined" "MultiplyWithRoot" 0 0))
          (LocalVariables|SetcurrentTurret _returnvalue_9))
        (:NewEnumerator10
          (bind _returnvalue_10 (Game|SpawnActorfromClass "/Game/BluePrint/Turrets/EMP_Turret/BP_EMP_Turret.BP_EMP_Turret_C" (Math|Transform|MakeTransform (Transformation|GetActorLocation (LocalVariables|GetselectedPlatform)) "0, 0, 0" "1.000000,1.000000,1.000000") "Undefined" "MultiplyWithRoot" 0 0))
          (LocalVariables|SetcurrentTurret _returnvalue_10)))
      (Utilities|Array|RemoveItem (Variables|SpawnPoints|GetturretPlatforms) (LocalVariables|GetselectedPlatform))
      (bind _percentageaddedvalue (CallFunction|CalculateandAddPercentage (Variables|/Game/BluePrint/Turrets/BP_Turret.BP_Turret_C|GetshootRechargeTime (LocalVariables|GetcurrentTurret)) (Utilities|Struct|BreakS_TurretStatsRange (Variables|Default|GetturretStatsIncreasment)) false))
      (Variables|/Game/BluePrint/Turrets/BP_Turret.BP_Turret_C|SetshootRechargeTime (LocalVariables|GetcurrentTurret) _percentageaddedvalue)
      (bind _percentageaddedvalue_2 (CallFunction|CalculateandAddPercentage (Variables|/Game/BluePrint/Turrets/BP_Turret.BP_Turret_C|Getdamage (LocalVariables|GetcurrentTurret)) (Utilities|Struct|BreakS_TurretStatsRange (Variables|Default|GetturretStatsIncreasment)) true))
      (Variables|/Game/BluePrint/Turrets/BP_Turret.BP_Turret_C|Setdamage (LocalVariables|GetcurrentTurret) _percentageaddedvalue_2)
      (Math|Integer|IncrementInt (LocalVariables|GetcurrentTurretNumber)))))

(fn SpawnStronghold
  (bind _currentstructurevariables (Variables|TurretSpawnPercentage|GetcurrentStructureVariables))
  (bind _strongholdnumber (Utilities|Struct|BreakS_StructureSpawnVariables _currentstructurevariables))
  (if (> _strongholdnumber 0)
    (while (< (LocalVariables|GetcurrentStrongholdNumber) _strongholdnumber)
      (bind _output_get (LocalVariables|SetselectedPathBlock (.OutItem (Utilities|Array|Random (Variables|SpawnPoints|GetstrongholdSpawnPoints)))))
      (bind _returnvalue (Game|SpawnActorfromClass "/Game/BluePrint/Strongholds/BP_Stronghold.BP_Stronghold_C" (Math|Transform|MakeTransform (Math|Vector|MakeVector (.x (Transformation|GetActorLocation _output_get)) (.y (Transformation|GetActorLocation _output_get)) (+ (.z (Transformation|GetActorLocation _output_get)) 5e+01)) (Math|Rotator|MakeRotator 0.0 0.0 (.Value (Utilities|Map|Find (Variables|Default|GetstrongholdZRotation) (Utilities|Array|Get(acopy) (Variables|/Game/BluePrint/Path/BP_PathBlock.BP_PathBlock_C|Getorientation _output_get))))) "1.000000,1.000000,1.000000") "Undefined" "MultiplyWithRoot" 0 0))
      (bind _percentageaddedvalue (CallFunction|CalculateandAddPercentage (Variables|/Game/BluePrint/Strongholds/BP_Stronghold.BP_Stronghold_C|GetresistanceValue _returnvalue) (Utilities|Struct|BreakS_StrongholdStatsRange (Variables|Default|GetstrongholdStatsIncreasment)) true))
      (Variables|/Game/BluePrint/Strongholds/BP_Stronghold.BP_Stronghold_C|SetresistanceValue _returnvalue _percentageaddedvalue)
      (bind _percentageaddedvalue_2 (CallFunction|CalculateandAddPercentage (Variables|/Game/BluePrint/Strongholds/BP_Stronghold.BP_Stronghold_C|Getdamage _returnvalue) (Utilities|Struct|BreakS_StrongholdStatsRange (Variables|Default|GetstrongholdStatsIncreasment)) true))
      (Variables|/Game/BluePrint/Strongholds/BP_Stronghold.BP_Stronghold_C|Setdamage _returnvalue _percentageaddedvalue_2)
      (Utilities|Array|RemoveItem (Variables|SpawnPoints|GetstrongholdSpawnPoints) (LocalVariables|GetselectedPathBlock))
      (Math|Integer|IncrementInt (LocalVariables|GetcurrentStrongholdNumber)))))

(fn CalculateandAddPercentage
  (params (value :type Float%20%28double-precision%29) (percentage :type Integer) (isAddiction :type Boolean))
  (bind _returnvalue (* value percentage))
  (bind _returnvalue_2 (/ _returnvalue 1e+02))
  (if isAddiction
    (return (+ value _returnvalue_2))
    (else
      (return (- value _returnvalue_2)))))