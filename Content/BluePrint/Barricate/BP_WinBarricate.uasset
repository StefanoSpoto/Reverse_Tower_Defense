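; Barricade actor that acts as a win trigger and loads a level after it is destroyed.
; BarricateDestroyed disables the mesh's collision, toggles its visibility, prints a debug string and sets IsDestroyed, then waits DelayBeforeWin before opening PrototypeEnvironment_Scene.
; Separately, any BP_Unit that begins overlapping the Box component is destroyed, with no check on the barricade's state.
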(event OnComponentBeginOverlap(Box)
  (params (OverlappedComponent :type Primitive%20Component%20Object%20Reference) (OtherActor :type Actor%20Object%20Reference) (OtherComp :type Primitive%20Component%20Object%20Reference) (OtherBodyIndex :type Integer) (bFromSweep :type Boolean) (SweepResult :type Hit%20Result%20Structure%20%28by%20ref%29))
  (bind _asbp_unit (Utilities|Casting|CastToBP_Unit OtherActor))
  (Actor|DestroyActor _asbp_unit))

(event EventBeginPlay
  (|CallParentFunction) ; This node is disabled and will not be called.\nDrag off pins to build functionality.
)

(event Collision|EventActorBeginOverlap
  (params (OtherActor :type Actor%20Object%20Reference))
  (|CallParentFunction OtherActor) ; This node is disabled and will not be called.\nDrag off pins to build functionality.
)

(event EventTick
  (params (DeltaSeconds :type Float%20%28single-precision%29))
  (|CallParentFunction DeltaSeconds) ; This node is disabled and will not be called.\nDrag off pins to build functionality.
)

(event EventBarricateDestroyed
  (bind _barricade_mesh (Variables|Default|GetBarricade%20Mesh))
  (Collision|SetCollisionEnabled _barricade_mesh "NoCollision")
  (Rendering|ToggleVisibility _barricade_mesh false)
  (Development|PrintString "Hello")
  (Variables|Default|SetisDestroyed true)
  (Utilities|FlowControl|Delay (Variables|WinCondition|GetdelayBeforeWin))
  (Game|OpenLevel(byObjectReference) "/Game/Maps/PrototypeEnvironment_Scene.PrototypeEnvironment_Scene"))

(fn ConstructionScript
  (|CallParentFunction))