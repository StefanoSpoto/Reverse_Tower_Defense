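; Base barricade Blueprint that traps units entering it until their combined Power depletes its DefensePower.
; Each entering unit is moved to a release point, stored in a stopped list and subtracts its Power from the defense.
; At zero or below, collision turns off, the mesh switches to a rock material, and after a short pause units exit sequentially, spaced by their SpawnTime, before the mesh is hidden.
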(event Custom|UnitEnterInBarricade
  (params (Unit :type BP%20Unit%20Object%20Reference) (Power :type Float%20%28double-precision%29))
  (CallFunction|AddUnittoStopList Unit)
  (bind _destroyed (CallFunction|TakePowerDamage Power))
  (if _destroyed
    (CallFunction|DisableCollision)
    (Rendering|Material|SetMaterial (Variables|Default|GetBarricadeMesh) 0 "/Game/StarterContent/Props/Materials/M_Rock.M_Rock")
    (Utilities|FlowControl|Delay 1.0)
    (bind _array_element (Utilities|ForEachLoopwithDelay (Variables|Barricate|GetunitsStopped) (Variables|/Game/BluePrint/Units/BP_Unit.BP_Unit_C|GetspawnTime (stale _array_element)))
      (:Loop%20Body
        (Default|ExitBarricadeStructure _array_element))
      (:Completed
        (CallFunction|SetInvisible)))))

(fn ConstructionScript)

(fn AddUnittoStopList
  (params (Unit :type BP%20Unit%20Object%20Reference))
  (Default|EnterBarricadeStructure Unit)
  (Utilities|Array|Add (Variables|Barricate|GetunitsStopped) Unit)
  (Transformation|SetActorLocation Unit (Transformation|GetWorldLocation (Variables|Default|GetUnitReleasePoint)) false false))

(fn SetInvisible
  (Rendering|SetVisibility (Variables|Default|GetBarricadeMesh) false true))

(fn TakePowerDamage
  (params (Power :type Float%20%28double-precision%29))
  (bind _output_get (Variables|Barricate|SetdefensePower (- (Variables|Barricate|GetdefensePower) Power)))
  (return (<= _output_get 0.0)))

(fn DisableCollision
  (Collision|SetCollisionEnabled (Variables|Default|GetBox) "NoCollision"))