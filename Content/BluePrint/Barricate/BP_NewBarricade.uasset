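; Destructible barricade actor that tracks its own health and breaks when that health runs out.
; A TakeDamage event subtracts incoming damage, clamps health at zero and calls BarricateDestroyed.
; That event disables the mesh's collision, toggles its visibility and sets IsDestroyed, leaving the actor in the world rather than destroying it.
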(event Custom|TakeDamage
  (params (damage :type Float%20%28double-precision%29))
  (Variables|Barricate|Sethealth (- (Variables|Barricate|Gethealth) damage))
  (if (<= (Variables|Barricate|Gethealth) 0.0)
    (Variables|Barricate|Sethealth 0.0)
    (CallFunction|BarricateDestroyed)))

(event Custom|BarricateDestroyed
  (bind _barricade_mesh (Variables|Default|GetBarricade%20Mesh))
  (Collision|SetCollisionEnabled _barricade_mesh "NoCollision")
  (Rendering|ToggleVisibility _barricade_mesh false)
  (Variables|Default|SetisDestroyed true))

(event EventBeginPlay)

(event Collision|EventActorBeginOverlap
  (params (OtherActor :type Actor%20Object%20Reference)))

(event EventTick
  (params (DeltaSeconds :type Float%20%28single-precision%29)))

(fn ConstructionScript)