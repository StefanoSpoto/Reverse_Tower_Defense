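; Menu game mode that drives navigation between the main menu, champion selection and army selection screens.
; On BeginPlay it shows W_MainMenu with the mouse cursor and UI-only input.
; Navigation functions create or toggle visibility of stored widgets; army selection is reused, while champion selection is recreated on each forward visit.
; AddTroopToArmy forwards the given troop to the army selection widget.
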(event EventBeginPlay
  (bind _returnvalue (Game|GetPlayerController 0))
  (bind _returnvalue_2 (UserInterface|CreateWidget "/Game/BluePrint/Menus/W_MainMenu.W_MainMenu_C"))
  (UserInterface|Viewport|AddtoViewport _returnvalue_2 0)
  (Variables|UI|SetmainMenu _returnvalue_2)
  (Variables|/Script/Engine.PlayerController|SetbShowMouseCursor _returnvalue true)
  (Input|SetInputModeUIOnly _returnvalue 0 "DoNotLock" false))

(fn ConstructionScript)

(fn GotoArmySelection
  (Utilities|IsValid (Variables|UI|GetarmySelectionMenu)
    (:Is%20Valid
      (Widget|SetVisibility (Variables|UI|GetarmySelectionMenu) "Visible"))
    (:Is%20Not%20Valid
      (bind _returnvalue (UserInterface|CreateWidget "/Game/BluePrint/Menus/W_ArmySelection.W_ArmySelection_C"))
      (UserInterface|Viewport|AddtoViewport _returnvalue 0)
      (Variables|UI|SetarmySelectionMenu _returnvalue))))

(fn GoBacktoChampionSelection
  (Widget|SetVisibility (Variables|UI|GetarmySelectionMenu) "Hidden")
  (Widget|SetVisibility (Variables|UI|GetchampionSelectionMenu) "Visible"))

(fn AddTrooptoArmy
  (params (troop :type DA%20Troop%20Object%20Reference))
  (bind _asw_army_selection (Utilities|Casting|CastToW_ArmySelection (Variables|UI|GetarmySelectionMenu)))
  (Default|AddTroop _asw_army_selection troop))

(fn GotoChampionSelection
  (Widget|SetVisibility (Variables|UI|GetmainMenu) "Hidden")
  (bind _returnvalue (UserInterface|CreateWidget "/Game/BluePrint/Menus/W_HeroSelection.W_HeroSelection_C"))
  (UserInterface|Viewport|AddtoViewport _returnvalue 0)
  (Variables|UI|SetchampionSelectionMenu _returnvalue))

(fn GoBacktoMainMenu
  (Widget|SetVisibility (Variables|UI|GetchampionSelectionMenu) "Hidden")
  (Widget|SetVisibility (Variables|UI|GetmainMenu) "Visible"))