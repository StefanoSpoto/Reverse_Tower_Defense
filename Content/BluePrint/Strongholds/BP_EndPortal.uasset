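; End-of-level portal that stays hidden until the game mode signals that the final stronghold is destroyed.
; Units overlapping its box increment an arrival count and restart a delay timeline, which deactivates the unit when it finishes.
; When the count matches the game mode's spawned unit total, it opens the win screen.
; Only mesh visibility is toggled, and custom time dilation follows game mode changes.
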(event OnComponentBeginOverlap(Box)
  (params (OverlappedComponent :type Primitive%20Component%20Object%20Reference) (OtherActor :type Actor%20Object%20Reference) (OtherComp :type Primitive%20Component%20Object%20Reference) (OtherBodyIndex :type Integer) (bFromSweep :type Boolean) (SweepResult :type Hit%20Result%20Structure%20%28by%20ref%29))
  (bind _asbp_unit (Utilities|Casting|CastToBP_Unit OtherActor))
  (CallFunction|EnterPortal _asbp_unit))

(event Custom|EndLevelStrongholdDestroyed_Event
  (Rendering|SetVisibility (Variables|Default|GetPortalMesh) true false))

(event Custom|Enter%20Portal
  (params (Unit%20Target :type BP%20Unit%20Object%20Reference))
  (bind _result (Math|Integer|IncrementInt (Variables|EndPortal|GetunitsReachedEndCount))
    (:%20%20
      (Timeline|EnterPortalDelay%20Timeline PlayFromStart
        (:Finished
          (Default|DeactivateUnit Unit%20Target)
          (if (== (Utilities|Array|Length (Variables|/Game/BluePrint/Player/GM_LevelGameMode.GM_LevelGameMode_C|GetspawnedUnits (CallFunction|GetGMLevelGameMode))) _result)
            (Default|OpenWinScreen (CallFunction|GetGMLevelGameMode) true)))))))

(event Custom|Change%20Custom%20Time%20Dilation
  (params (newTimeDilation :type Float%20%28double-precision%29))
  (Variables|Default|SetCustomTimeDilation newTimeDilation))

(event EventBeginPlay
  (Rendering|SetVisibility (Variables|Default|GetPortalMesh) false false)
  (EventDispatchers|BindEventtoOnChangeTimeDilation (CallFunction|GetGMLevelGameMode) (delegate Custom|Change%20Custom%20Time%20Dilation))
  (EventDispatchers|AssignEndLevelStrongholdDestroyed (CallFunction|GetGMLevelGameMode) (delegate Custom|EndLevelStrongholdDestroyed_Event)))

(fn ConstructionScript)