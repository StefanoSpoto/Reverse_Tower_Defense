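; BP_EndStronghold is the level's final stronghold, whose fall ends the level in a win.
; When its life finishes, it hides the barricade mesh and has every unit it stopped save its gold.
; After a delay it passes those units and its end-level gold value to the game mode's win screen, then clears the list and destroys itself.
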(event EventFinishStrongholdLife
  (Rendering|SetVisibility (Variables|Default|GetBarricadeMesh) false true)
  (for _array_element (Variables|Default|GetunitsStopped)
    (Default|SaveGold _array_element))
  (Utilities|FlowControl|Delay (Variables|EndStronghold|GetdelayBeforeWin))
  (Default|OpenWinScreen (CallFunction|GetGMLevelGameMode) true (Variables|Default|GetunitsStopped) (Variables|EndStronghold|GetendLevelGoldValue))
  (Utilities|Array|Clear (Variables|Default|GetunitsStopped))
  (Actor|DestroyActor))

(fn ConstructionScript
  (|CallParentFunction))