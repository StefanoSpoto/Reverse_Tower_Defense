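; Stronghold barricade that traps units entering its collision and trades damage with them until it breaks.
; Trapped units move to a release point, and their summed Power drains resistance in a delay loop started on each entry, while a recurring check splits stronghold damage among them and removes the killed.
; At zero resistance it disables collision, releases survivors staggered by SpawnTime, then hides itself.
; Hover and health widgets show trapped units and resistance.
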(event OnComponentBeginOverlap(EnterCollision)
  (params (OverlappedComponent :type Primitive%20Component%20Object%20Reference) (OtherActor :type Actor%20Object%20Reference) (OtherComp :type Primitive%20Component%20Object%20Reference) (OtherBodyIndex :type Integer) (bFromSweep :type Boolean) (SweepResult :type Hit%20Result%20Structure%20%28by%20ref%29))
  (bind _asbp_unit (Utilities|Casting|CastToBP_Unit OtherActor))
  (CallFunction|UnitEnterinBarricade _asbp_unit))

(event OnBeginCursorOver(BarricadeMesh)
  (params (TouchedComponent :type Primitive%20Component%20Object%20Reference))
  (CallFunction|ShowInfoWidget true))

(event OnEndCursorOver(BarricadeMesh)
  (params (TouchedComponent :type Primitive%20Component%20Object%20Reference))
  (CallFunction|ShowInfoWidget false))

(event Custom|ReleaseUnits
  ;[1 1 1] Release units
  (bind (_array_element _array_index) (Utilities|ForEachLoopwithDelay (Variables|Barricate|GetunitsStopped) (Variables|/Game/BluePrint/Units/BP_Unit.BP_Unit_C|GetspawnTime (stale _array_element)))
    (:Loop%20Body
      (Default|ExitBarricadeStructure _array_element)
      (Default|RemoveUnit (Variables|Default|GetHover%20Widget) _array_index))
    (:Completed
      (CallFunction|DestroyBarricate))))

(event Custom|UnitEnterInBarricade
  (params (Unit :type BP%20Unit%20Object%20Reference))
  ;[1 1 1] Entering barricade
  (CallFunction|AddUnitInsideBarricate Unit)
  (CallFunction|TakeDamageOverTIme))

(event Custom|DamageCheckForUnits
  ;[1 1 1] Damage Unit
  (if (not (Variables|Default|Getdestroyed))
    (CallFunction|DamageUnitsStopped)
    (if (> (Utilities|Array|Length (Variables|Barricate|GetunitsStopped)) 0)
      (Utilities|FlowControl|Delay 1.0)
      (else
        (Utilities|FlowControl|DelayUntilNextTick)))
    (CallFunction|DamageCheckforUnits)))

(event Custom|TakeDamageOverTIme
  (if (> (Utilities|Array|Length (Variables|Barricate|GetunitsStopped)) 0)
    (Utilities|FlowControl|Delay 1.0)
    (else
      (Utilities|FlowControl|DelayUntilNextTick)))
  (bind _destroyed (CallFunction|TakePowerDamage))
  (Default|SetHealthUI (Variables|Default|GetHealth%20Bar%20Widget) (Variables|Barricate|GetresistanceValue) (Variables|Barricate|GetmaxResistanceValue))
  (if _destroyed
    (CallFunction|DisableCollision)
    (Rendering|Material|SetMaterial (Variables|Default|GetBarricadeMesh) 0 "/Game/StarterContent/Props/Materials/M_Rock.M_Rock")
    (Utilities|FlowControl|Delay 0.5)
    (CallFunction|ReleaseUnits)
    (else
      (CallFunction|TakeDamageOverTIme))))

(event Custom|StrongholdWidgetHover
  (Default|SetHover (stale EventBeginPlay _output_get)))

(event Custom|StrongholdWidgetUnhover
  (Default|SetUnhover (stale EventBeginPlay _output_get))
  (Rendering|SetVisibility (Variables|Default|GetHoverWidget) false false))

(event Custom|HealthBarHover
  (Default|SetHover (stale EventBeginPlay _output_get_2))
  (CallFunction|ShowInfoWidget true))

(event Custom|HealthBarUnhover
  (Default|SetUnhover (stale EventBeginPlay _output_get_2))
  (Rendering|SetVisibility (Variables|Default|GetHoverWidget) false false))

(event EventBeginPlay
  (bind _maxresistancevalue (Variables|Barricate|GetmaxResistanceValue))
  (bind _asw_stronghold_hover (Utilities|Casting|CastToW_StrongholdHover (UserInterface|GetWidget (Variables|Default|GetHoverWidget))))
  (bind _output_get (Variables|Default|SetHover%20Widget _asw_stronghold_hover))
  (EventDispatchers|BindEventtoOnHovered (Variables|/Game/BluePrint/_Widgets/Stronghold/W_StrongholdHover.W_StrongholdHover_C|GetButton _output_get) (delegate Custom|StrongholdWidgetHover))
  (EventDispatchers|BindEventtoOnUnhovered (Variables|/Game/BluePrint/_Widgets/Stronghold/W_StrongholdHover.W_StrongholdHover_C|GetButton _output_get) (delegate Custom|StrongholdWidgetUnhover))
  (CallFunction|DamageCheckforUnits)
  (bind _asw_stronghold_health (Utilities|Casting|CastToW_StrongholdHealth (UserInterface|GetWidget (Variables|Default|GetHealthbar))))
  (bind _output_get_2 (Variables|Default|SetHealth%20Bar%20Widget _asw_stronghold_health))
  (EventDispatchers|BindEventtoOnHovered (Variables|/Game/BluePrint/Strongholds/W_StrongholdHealth.W_StrongholdHealth_C|GetButton _output_get_2) (delegate Custom|HealthBarHover))
  (EventDispatchers|BindEventtoOnUnhovered (Variables|/Game/BluePrint/Strongholds/W_StrongholdHealth.W_StrongholdHealth_C|GetButton _output_get_2) (delegate Custom|HealthBarUnhover))
  (bind _output_get_3 (Variables|Barricate|SetresistanceValue _maxresistancevalue))
  (Default|SetHealthUI (Variables|Default|GetHealth%20Bar%20Widget) _output_get_3 _maxresistancevalue))

(fn ConstructionScript)

(fn AddUnitInsideBarricate
  (params (Unit :type BP%20Unit%20Object%20Reference))
  (Default|EnterBarricadeStructure Unit)
  (Utilities|Array|Add (Variables|Barricate|GetunitsStopped) Unit)
  (Transformation|SetActorLocation Unit (Transformation|GetWorldLocation (Variables|Default|GetUnitReleasePoint)) false false)
  (Default|AddUnit (Variables|Default|GetHover%20Widget) Unit))

(fn DestroyBarricate
  (Rendering|SetVisibility (Variables|Default|GetBarricadeMesh) false true)
  (Variables|Default|Setdestroyed true)
  (Utilities|Array|Clear (Variables|Barricate|GetunitsStopped)))

(fn TakePowerDamage
  (Variables|Barricate|SettotalStoppedUnitsPower 0.0)
  (for _array_element (Variables|Barricate|GetunitsStopped)
    (Variables|Barricate|SettotalStoppedUnitsPower (+ (Variables|Barricate|GettotalStoppedUnitsPower) (Variables|/Game/BluePrint/Units/BP_Unit.BP_Unit_C|Getpower _array_element))))
  (bind _output_get (Variables|Barricate|SetresistanceValue (- (Variables|Barricate|GetresistanceValue) (Variables|Barricate|GettotalStoppedUnitsPower))))
  (if (<= _output_get 0.0)
    (Variables|Barricate|SetresistanceValue 0.0)
    (Rendering|SetVisibility (Variables|Default|GetHealthbar) false false))
  (return (<= _output_get 0.0)))

(fn DisableCollision
  (Collision|SetCollisionEnabled (Variables|Default|GetEnterCollision) "NoCollision")
  (Collision|SetCollisionEnabled (Variables|Default|GetBarricadeMesh) "NoCollision"))

(fn DamageUnitsStopped
  (bind _unitsstopped (Variables|Barricate|GetunitsStopped))
  (bind _returnvalue (Utilities|Array|Length _unitsstopped))
  (if (> _returnvalue 0)
    (for (_array_element _array_index) _unitsstopped
      (Utilities|IsValid _array_element
        (:Is%20Valid
          (bind (_iskilled _unit) (Default|TakeDamage _array_element (/ (Variables|Barricate|GetstrongholdDamage) _returnvalue)))
          (if (and _iskilled (Utilities|IsValid _unit))
            (Default|RemoveUnit (Variables|Default|GetHover%20Widget) _array_index)
            (Default|KillUnit _unit true)
            (Utilities|Array|RemoveItem (Variables|Barricate|GetunitsStopped) _unit)
            (else
              (Utilities|IsValid (Utilities|Array|Get(acopy) (Variables|/Game/BluePrint/_Widgets/Stronghold/W_StrongholdHover.W_StrongholdHover_C|Getunits (Variables|Default|GetHover%20Widget)) _array_index)
                (:Is%20Valid
                  (Default|SetHealth (Utilities|Array|Get(acopy) (Variables|/Game/BluePrint/_Widgets/Stronghold/W_StrongholdHover.W_StrongholdHover_C|Getunits (Variables|Default|GetHover%20Widget)) _array_index) _array_element))))))))))

(fn ShowInfoWidget
  (params (show :type Boolean))
  (if show
    (Rendering|SetVisibility (Variables|Default|GetHoverWidget) true false)
    (elif (not (Variables|/Game/BluePrint/_Widgets/Stronghold/W_StrongholdHover.W_StrongholdHover_C|Gethovered (Variables|Default|GetHover%20Widget)))
      (if (not (Variables|/Game/BluePrint/Strongholds/W_StrongholdHealth.W_StrongholdHealth_C|Gethovered (Variables|Default|GetHealth%20Bar%20Widget)))
        (Rendering|SetVisibility (Variables|Default|GetHoverWidget) false false)))))