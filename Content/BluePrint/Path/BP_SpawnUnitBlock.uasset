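; Clickable spawn point for the reverse tower defense, where the player assembles an army of units to send out.
; Clicking registers it with the GameMode and toggles the troop selection UI, while hover and selection states swap Niagara effects and a hover widget.
; Army edits refresh both widget and level UI lists.
; On the GameInstance's start-spawning event, it spawns the army using per-unit delays, registers each unit, then clears the list.
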(event OnBeginCursorOver(Collider)
  (params (TouchedComponent :type Primitive%20Component%20Object%20Reference))
  (if (not (Variables|Default|Getselected))
    (Class|NiagaraComponent|SetAsset (Variables|Default|GetNiagara) "/Game/NiagaraVFX/NS_SPHover.NS_SPHover" true)
    (Rendering|SetVisibility (Variables|Default|GetHoverWidget) true false)))

(event OnEndCursorOver(Collider)
  (params (TouchedComponent :type Primitive%20Component%20Object%20Reference))
  (if (not (Variables|/Game/BluePrint/_Widgets/Spawner/Hover/W_SpawnerHover.W_SpawnerHover_C|Gethovered (Variables|Default|GetW%20Spawner%20Hover)))
    (if (not (Variables|Default|Getselected))
      (Class|NiagaraComponent|SetAsset (Variables|Default|GetNiagara) "/Game/NiagaraVFX/NS_SPNotSelected.NS_SPNotSelected" true)
      (Rendering|SetVisibility (Variables|Default|GetHoverWidget) false false))))

(event Custom|SpawnStart
  (bind _array_element (Utilities|ForEachLoopwithDelay (Variables|Default|Getarmy) (Variables|/Game/BluePrint/Units/DataAssets/DA_Unit.DA_Unit_C|GetspawnTime (stale _array_element)))
    (:Loop%20Body
      (bind _returnvalue (Game|SpawnActorfromClass "/Game/BluePrint/Units/BP_Unit.BP_Unit_C" (Transformation|GetWorldTransform (Variables|Default|GetUnitSpawnPoint)) "AlwaysSpawn" "MultiplyWithRoot" 0 0))
      (Default|SetStats _returnvalue _array_element)
      (Default|AddSpawnedUnit (CallFunction|GetGIReverseTD) _returnvalue))
    (:Completed
      (Utilities|Array|Clear (Variables|Default|Getarmy)))))

(event Custom|SpawnerWidgetHover
  (if (not (Variables|Default|Getselected))
    (Default|SetHover (Variables|Default|GetW%20Spawner%20Hover))))

(event Custom|SpawnerWidgetUnhover
  (Default|SetUnhover (Variables|Default|GetW%20Spawner%20Hover))
  (Class|NiagaraComponent|SetAsset (Variables|Default|GetNiagara) "/Game/NiagaraVFX/NS_SPNotSelected.NS_SPNotSelected" true)
  (Rendering|SetVisibility (Variables|Default|GetHoverWidget) false false))

(event Custom|DeselectSpawner
  (CallFunction|ChangeSpawnerAspect false))

(event Custom|OnOtherSpawnerSelected
  (CallFunction|ChangeSpawnerAspect false))

(event EventBeginPlay
  (|CallParentFunction)
  (EventDispatchers|BindEventtoOnStartSpawning (CallFunction|GetGIReverseTD) (delegate Custom|SpawnStart))
  (EventDispatchers|BindEventtoOnSelectSpawner (CallFunction|GetGMLevelGameMode) (delegate Custom|OnOtherSpawnerSelected))
  (bind _asw_spawner_hover (Utilities|Casting|CastToW_SpawnerHover (UserInterface|GetWidget (Variables|Default|GetHoverWidget))))
  (bind _output_get (Variables|Default|SetW%20Spawner%20Hover _asw_spawner_hover))
  (EventDispatchers|BindEventtoOnHovered (Variables|/Game/BluePrint/_Widgets/Spawner/Hover/W_SpawnerHover.W_SpawnerHover_C|GetButton _output_get) (delegate Custom|SpawnerWidgetHover))
  (EventDispatchers|BindEventtoOnUnhovered (Variables|/Game/BluePrint/_Widgets/Spawner/Hover/W_SpawnerHover.W_SpawnerHover_C|GetButton _output_get) (delegate Custom|SpawnerWidgetUnhover))
  (EventDispatchers|BindEventtoOnSelectTurret (CallFunction|GetGMLevelGameMode) (delegate Custom|DeselectSpawner)))

(event MouseInput|EventActorOnClicked
  (params (ButtonPressed :type Key%20Structure :default "None"))
  ;[1 1 1] Quando viene cliccato,viene salvata una sua reference dentro alla GameMode, in modo da essere accessibile dalla UI
  (if (Variables|Default|Getselected)
    (CallFunction|SelectSpawner false)
    (else
      (CallFunction|SelectSpawner true))))

(fn ConstructionScript
  (|CallParentFunction))

(fn ChangeSpawnerAspect
  (params (selected :type Boolean))
  (bind _output_get (Variables|Default|Setselected selected))
  (if _output_get
    (Class|NiagaraComponent|SetAsset (Variables|Default|GetNiagara) "/Game/NiagaraVFX/NS_SPClicked-HoveredUnit.NS_SPClicked-HoveredUnit" true)
    (else
      (Class|NiagaraComponent|SetAsset (Variables|Default|GetNiagara) "/Game/NiagaraVFX/NS_SPNotSelected.NS_SPNotSelected" true))))

(fn GetUnitSpawnPosition
  (return (Transformation|GetWorldLocation (Variables|Default|GetUnitSpawnHighlight))))

(fn AddUnittoArmy
  (params (Unit :type DA%20Unit%20Object%20Reference))
  (bind _asgm_level_game_mode (CallFunction|GetGMLevelGameMode))
  (bind _returnvalue (Utilities|Array|Add (Variables|Default|Getarmy) Unit))
  (Default|AddUnit (Variables|Default|GetW%20Spawner%20Hover) Unit _returnvalue)
  (Default|AddUnitinSpawnerInfo (Default|GetLevelUI _asgm_level_game_mode) Unit _returnvalue)
  (Default|UpdateSelectetUnitsCount _asgm_level_game_mode true)
  (return _returnvalue))

(fn RemoveUnitfromArmy
  (params (unitIndex :type Integer))
  (bind _asgm_level_game_mode (CallFunction|GetGMLevelGameMode))
  (bind _army (Variables|Default|Getarmy))
  (bind _w_spawner_hover (Variables|Default|GetW%20Spawner%20Hover))
  (bind _level_ui (Default|GetLevelUI _asgm_level_game_mode))
  (Utilities|Array|RemoveIndex _army unitIndex)
  (Widget|Panel|ClearChildren (Variables|/Game/BluePrint/_Widgets/W_LevelUI.W_LevelUI_C|GetVerticalBox _level_ui))
  (Widget|Panel|ClearChildren (Variables|/Game/BluePrint/_Widgets/Spawner/Hover/W_SpawnerHover.W_SpawnerHover_C|GetVerticalBox _w_spawner_hover))
  (for (_array_element _array_index) _army
    (Default|AddUnitinSpawnerInfo _level_ui _array_element _array_index)
    (Default|AddUnit _w_spawner_hover _array_element _array_index))
  (Default|UpdateSelectetUnitsCount _asgm_level_game_mode false))

(fn SelectSpawner
  (params (select :type Boolean))
  (bind _asgm_level_game_mode (CallFunction|GetGMLevelGameMode))
  (bind _asgm_level_game_mode_2 (CallFunction|GetGMLevelGameMode))
  (bind _level_ui (Default|GetLevelUI _asgm_level_game_mode))
  (bind _level_ui_2 (Default|GetLevelUI _asgm_level_game_mode_2))
  (if select
    (Default|SetClickedSpawner (CallFunction|GetGMLevelGameMode) self true)
    (Default|SetUnhover (Variables|Default|GetW%20Spawner%20Hover))
    (Class|NiagaraComponent|SetAsset (Variables|Default|GetNiagara) "/Game/NiagaraVFX/NS_SPNotSelected.NS_SPNotSelected" true)
    (Rendering|SetVisibility (Variables|Default|GetHoverWidget) false false)
    (Class|NiagaraComponent|SetAsset (Variables|Default|GetNiagara) "/Game/NiagaraVFX/NS_SPClicked-HoveredUnit.NS_SPClicked-HoveredUnit" true)
    (Default|ShowSpawnerInfo _level_ui_2 true (Variables|Default|Getarmy))
    (Default|OpenTroopSelection _level_ui_2)
    (else
      (Default|SetClickedSpawner (CallFunction|GetGMLevelGameMode) self false)
      (Class|NiagaraComponent|SetAsset (Variables|Default|GetNiagara) "/Game/NiagaraVFX/NS_SPHover.NS_SPHover" true)
      (Rendering|SetVisibility (Variables|Default|GetHoverWidget) true false)
      (Default|ShowSpawnerInfo _level_ui false)
      (Default|CloseTroopSelection _level_ui))))