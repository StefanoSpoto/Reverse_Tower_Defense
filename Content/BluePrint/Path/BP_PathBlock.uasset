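; BP_PathBlock is a path cell that points in a cardinal direction and links to the block it faces, exposing a transform for units.
; A forward line trace caches NextPathBlock, falling back to itself when nothing is hit.
; Cells with several orientations act as switches: SwitchOrientation cycles directions with a timeline rotation, then retraces the link.
; The construction script previews the first orientation, configures switch collision and material, and optionally spawns a coin.
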(event Custom|SetCellRotation
  (params (newRotation :type Rotator))
  (Variables|Path|SetnewRotation newRotation)
  (Variables|Path|SetoldRotation (Transformation|GetWorldRotation (Variables|Default|GetCube)))
  (bind _alpha (Timeline|Timeline_CellRotation PlayFromStart)
    (:Update
      (Variables|Path|SetisSwitching true)
      (Transformation|SetWorldRotation (Variables|Default|GetCube) (Math|Rotator|Lerp(Rotator) (Variables|Path|GetoldRotation) (Variables|Path|GetnewRotation) _alpha true) false false))
    (:Finished
      (Variables|Path|SetisSwitching false)
      (CallFunction|SetNextPathBlock))))

(event EventBeginPlay
  (Development|SetHiddeninGame (Variables|Default|GetBox) true false)
  (CallFunction|SetNextPathBlock)
  (Utilities|FlowControl|Sequence
    (:then_0
      (if (Variables|Block|Gettest)
        (Development|SetHiddeninGame (Variables|Default|GetCube) false false)
        (else
          (Rendering|SetVisibility (Variables|Default|GetArrow) false false))))
    (:then_1
      (if (> (Utilities|Array|Length (Variables|Path|Getorientation)) 1)
        (Rendering|SetVisibility (Variables|Default|GetArrow) true false)))))

(fn ConstructionScript
  (bind _box (Variables|Default|GetBox))
  (bind _orientation (Variables|Path|Getorientation))
  (bind _orientation_2 (Variables|Path|Getorientation))
  (bind _box_2 (Variables|Default|GetBox))
  (Components|Box|SetBoxExtent (Variables|Default|GetBox) (Variables|Default|GetswitchBlockCollisionExtents) true)
  (Construction|SetPathCellOrientationforConstruction)
  (if (Variables|Block|GethasCoin)
    (ChildActorComponent|SetChildActorClass (Variables|Default|GetCoin%20Actor) "/Game/BluePrint/Coins/BP_Coin.BP_Coin_C")
    (else
      (ChildActorComponent|SetChildActorClass (Variables|Default|GetCoin%20Actor) 0)))
  (if (> (Utilities|Array|Length (Variables|Path|Getorientation)) 1)
    (Rendering|Material|SetMaterial (Variables|Default|GetCube) 0 "/Game/Materials/TempMaterial/M_WireframeB.M_WireframeB")
    (Rendering|SetVisibility _box_2 true false)
    (Collision|SetCollisionEnabled _box_2 "QueryAndPhysics")
    (if (== (Utilities|Array|Length _orientation) 4)
      (Utilities|Array|RemoveIndex _orientation 3)
      (CallFunction|SetNextPathBlock :!label _label))
    (else
      (Rendering|SetVisibility _box false false)
      (Collision|SetCollisionEnabled _box "NoCollision")
      (if (== (Utilities|Array|Length _orientation_2) 0)
        (Utilities|Array|Add _orientation_2 "NewEnumerator2")
        (goto _label)))))

(fn SetPathCellOrientation
  (params (orientationArrayIndex :type Integer))
  (switch Utilities|FlowControl|Switch|SwitchonE_PathOrientation (Utilities|Array|Get(acopy) (Variables|Path|Getorientation) orientationArrayIndex)
    (:NewEnumerator2
      (CallFunction|SetCellRotation "0, 0, 0"))
    (:NewEnumerator3
      (CallFunction|SetCellRotation "0.000000,180.000000,0.000000"))
    (:NewEnumerator0
      (CallFunction|SetCellRotation "0.000000,-90.000000,0.000000"))
    (:NewEnumerator1
      (CallFunction|SetCellRotation "0.000000,90.000000,0.000000"))))

(fn GetPathCellOrientation
  (return (Transformation|GetWorldRotation (Variables|Default|GetCube))))

(fn SwitchOrientation
  (bind _result (Math|Integer|IncrementInt (Variables|Path|GetorientationsIndex))
    (:%20%20
      (if (< _result (Utilities|Array|Length (Variables|Path|Getorientation)))
        _
        (else
          (Variables|Path|SetorientationsIndex 0)))
      (Orientation|SetPathCellOrientation (Variables|Path|GetorientationsIndex)))))

(fn SetNextPathBlock
  (bind _cube (Variables|Default|GetCube))
  (bind _outhit (Collision|LineTraceByChannel (Transformation|GetWorldLocation _cube) (+ (Transformation|GetWorldLocation _cube) (* (Math|Vector|GetForwardVector _cube) 1e+02)) "TraceTypeQuery1" false 0 "None"))
  (if (.bblockinghit _outhit)
    (bind _asbp_path_block (Utilities|Casting|CastToBP_PathBlock (.hitactor _outhit)))
    (Variables|Path|SetnextPathBlock _asbp_path_block)
    (else
      (Variables|Path|SetnextPathBlock self))))

(fn GetUnitPathTransform
  (return (Transformation|GetWorldTransform (Variables|Default|GetUnitSpawnPoint))))

(fn IsPathSwitch
  (return (> (Utilities|Array|Length (Variables|Path|Getorientation)) 1)))

(fn SetCellRotationforConstruction
  (params (NewRotation :type Rotator))
  (Transformation|SetWorldRotation (Variables|Default|GetCube) NewRotation false false))

(fn SetPathCellOrientationforConstruction
  (params (orientationArrayIndex :type Integer))
  (switch Utilities|FlowControl|Switch|SwitchonE_PathOrientation (Utilities|Array|Get(acopy) (Variables|Path|Getorientation) orientationArrayIndex)
    (:NewEnumerator2
      (Construction|SetCellRotationforConstruction "0, 0, 0"))
    (:NewEnumerator3
      (Construction|SetCellRotationforConstruction "0.000000,180.000000,0.000000"))
    (:NewEnumerator0
      (Construction|SetCellRotationforConstruction "0.000000,-90.000000,0.000000"))
    (:NewEnumerator1
      (Construction|SetCellRotationforConstruction "0.000000,90.000000,0.000000")))
  (CallFunction|SetNextPathBlock))