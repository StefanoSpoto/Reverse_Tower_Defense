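; Path block that acts as a clickable army spawner, holding the player's per-wave unit lists and releasing them onto the path.
; On the GameMode's start event it spawns commanders or troops one by one on a delay timeline, chaining waves up to the requested one.
; Clicking and hovering drive Niagara highlights, a hover widget and the level UI's troop selection.
; Time dilation changes from the GameMode pass to spawned units, with zero blocking spawns.
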(event OnBeginCursorOver(Collider)
  (params (TouchedComponent :type Primitive%20Component%20Object%20Reference))
  ;[1 1 1] Spawn hover
  (if (not (Variables|Default|Getselected))
    (Class|NiagaraComponent|SetAsset (Variables|Default|GetNiagara) "/Game/NiagaraVFX/NS_SPHover.NS_SPHover" true)
    (if (and (not (CallFunction|AreAllWavesEmpty)) (!= (Default|GetUnitsCount (Variables|Default|GetW%20Spawner%20Hover)) 0))
      (Rendering|SetVisibility (Variables|Default|GetHoverWidget) true false))))

(event OnEndCursorOver(Collider)
  (params (TouchedComponent :type Primitive%20Component%20Object%20Reference))
  ;[1 1 1] Spawn unhover
  (if (not (Variables|/Game/BluePrint/_Widgets/Level/Spawner/Hover/W_SpawnerHover.W_SpawnerHover_C|Gethovered (Variables|Default|GetW%20Spawner%20Hover)))
    (if (not (Variables|Default|Getselected))
      (Class|NiagaraComponent|SetAsset (Variables|Default|GetNiagara) "/Game/NiagaraVFX/NS_SPNotSelected.NS_SPNotSelected" true)
      (Rendering|SetVisibility (Variables|Default|GetHoverWidget) false false))))

(event Custom|Change%20Custom%20Time%20Dilation
  (params (newTimeDilation :type Float%20%28double-precision%29))
  (bind _output_get (Variables|Default|SetCustomTimeDilation newTimeDilation))
  (Variables|Default|SetcanSpawn (!= _output_get 0.0)))

(event Custom|SpawnerWidgetHover
  (if (not (Variables|Default|Getselected))
    (Default|SetHover (Variables|Default|GetW%20Spawner%20Hover))))

(event Custom|SpawnerWidgetUnhover
  (Default|SetUnhover (Variables|Default|GetW%20Spawner%20Hover))
  (Class|NiagaraComponent|SetAsset (Variables|Default|GetNiagara) "/Game/NiagaraVFX/NS_SPNotSelected.NS_SPNotSelected" true)
  (Rendering|SetVisibility (Variables|Default|GetHoverWidget) false false))

(event Custom|OnDeselectSpawner
  (CallFunction|SelectSpawner false))

(event Custom|OnOtherSpawnerSelected
  (params (Spawner%20Actor :type BP%20Unit%20Spawner%20Path%20Block%20Object%20Reference))
  (CallFunction|ChangeSpawnerAspect false))

(event Custom|SpawnWave
  ;[1 1 1] Spawn units
  (if (Variables|Default|GetcanSpawn)
    (if (Utilities|Array|IsNotEmpty (.army (Utilities|Array|Get(acopy) (Variables|Waves|GetarmyWaves) (- (Variables|Waves|GetwaveSpawning) 1))))
      (Variables|Default|SetisSpawning true)
      (CallFunction|SpawnUnits (Utilities|Array|Get(acopy) (.army (Utilities|Array|Get(acopy) (Variables|Waves|GetarmyWaves) (- (Variables|Waves|GetwaveSpawning) 1)))))
      (Default|RemoveUnit (Variables|Default|GetW%20Spawner%20Hover))
      (Utilities|Array|RemoveIndex (.army (Utilities|Array|Get(acopy) (Variables|Waves|GetarmyWaves) (- (Variables|Waves|GetwaveSpawning) 1))))
      (if (Default|IsCurrentSpawner (CallFunction|GetGMLevelGameMode) self)
        (Default|RemoveUnitfromSpawnerInfo (CallFunction|GetWLevelUI)))
      (if (== (Utilities|Array|Length (.army (Utilities|Array|Get(acopy) (Variables|Waves|GetarmyWaves) (- (Variables|Waves|GetwaveSpawning) 1)))) 0)
        (CallFunction|SpawnWave :!label _label)
        (else
          (bind _progress (Timeline|UnitSpawnDelay%20Timeline PlayFromStart)
            (:Update
              (Default|CallOnStartUnitTimer (CallFunction|GetWLevelUI) (Variables|Waves|GetwaveSpawning) _progress))
            (:Finished
              (goto _label)))))
      (else
        (bind _structout (Utilities|Struct|SetmembersinBS_SpawnerArmyWave (Utilities|Array|Get(acopy) (Variables|Waves|GetarmyWaves) (- (Variables|Waves|GetwaveSpawning) 1)) true))
        (Utilities|Array|SetArrayElem (Variables|Waves|GetarmyWaves) (- (Variables|Waves|GetwaveSpawning) 1) _structout)
        (Default|AddSpawnedWaves (CallFunction|GetGMLevelGameMode) (Variables|Waves|GetwaveSpawning))
        (CallFunction|SpawnerWidgetUnhover)
        (Variables|Default|SetisSpawning false)
        (CallFunction|SelectSpawner false)
        (if (<= (+ (Variables|Waves|GetwaveSpawning) 1) (Utilities|Array|Length (Variables|Waves|GetarmyWaves)))
          (bind _result (Math|Integer|IncrementInt (Variables|Waves|GetwaveSpawning))
            (:%20%20
              (if (<= _result (Variables|Waves|GetwaveToReach))
                (Timeline|WaveSpawnDelay%20Timeline PlayFromStart
                  (:Finished
                    (CallFunction|SpawnWave)))))))))))

(event Custom|SpawnStart
  (params (Wave :type Integer))
  (Variables|Waves|SetwaveToReach Wave)
  (CallFunction|SelectSpawner false)
  (if (not (Variables|Default|GetisSpawning))
    (CallFunction|SpawnWave)))

(event EventBeginPlay
  (|CallParentFunction)
  (EventDispatchers|BindEventtoOnChangeTimeDilation (CallFunction|GetGMLevelGameMode) (delegate Custom|Change%20Custom%20Time%20Dilation))
  (Components|Timeline|SetPlayRate (Variables|Default|GetUnitSpawnDelay%20Timeline) (/ 1.0 (Variables|Spawner|GetspawnDelay)))
  (EventDispatchers|BindEventtoOnStartSpawning (CallFunction|GetGMLevelGameMode) (delegate Custom|SpawnStart))
  (EventDispatchers|BindEventtoOnSelectSpawner (CallFunction|GetGMLevelGameMode) (delegate Custom|OnOtherSpawnerSelected))
  (bind _asw_spawner_hover (Utilities|Casting|CastToW_SpawnerHover (UserInterface|GetWidget (Variables|Default|GetHoverWidget))))
  (bind _output_get (Variables|Default|SetW%20Spawner%20Hover _asw_spawner_hover))
  (EventDispatchers|BindEventtoOnHovered (Variables|/Game/BluePrint/_Widgets/Level/Spawner/Hover/W_SpawnerHover.W_SpawnerHover_C|GetButton _output_get) (delegate Custom|SpawnerWidgetHover))
  (EventDispatchers|BindEventtoOnUnhovered (Variables|/Game/BluePrint/_Widgets/Level/Spawner/Hover/W_SpawnerHover.W_SpawnerHover_C|GetButton _output_get) (delegate Custom|SpawnerWidgetUnhover))
  (EventDispatchers|BindEventtoOnSelectTurret (CallFunction|GetGMLevelGameMode) (delegate Custom|OnDeselectSpawner))
  (Components|Timeline|SetTimelineLength (Variables|Default|GetWaveSpawnDelay%20Timeline) (Variables|Spawner|GetspawnDelay)))

(event MouseInput|EventActorOnClicked
  (params (ButtonPressed :type Key%20Structure :default "None"))
  ;[1 1 1] Quando viene cliccato,viene salvata una sua reference dentro alla GameMode, in modo da essere accessibile dalla UI
  (Utilities|FlowControl|Sequence
    (:then_0
      (if (Default|IsNoSpawnerSelected (CallFunction|GetGMLevelGameMode))
        (Default|PlaySpawnerInfoAnimation (CallFunction|GetWLevelUI) true)))
    (:then_1
      (if (Variables|Default|Getselected)
        (CallFunction|SelectSpawner false)
        (else
          (CallFunction|SelectSpawner true)
          (Default|CallOnClickSpawnerButton (CallFunction|GetWLevelUI) (Variables|Spawner|GetspawnerIndex))
          (CallFunction|AutoSelectWavefromSpawner))))))

(fn ConstructionScript
  (|CallParentFunction))

(fn ChangeSpawnerAspect
  (params (selected :type Boolean))
  (bind _output_get (Variables|Default|Setselected selected))
  (if _output_get
    (Class|NiagaraComponent|SetAsset (Variables|Default|GetNiagara) "/Game/NiagaraVFX/NS_SPClicked-HoveredUnit.NS_SPClicked-HoveredUnit" true)
    (else
      (Class|NiagaraComponent|SetAsset (Variables|Default|GetNiagara) "/Game/NiagaraVFX/NS_SPNotSelected.NS_SPNotSelected" true))))

(fn GetUnitSpawnPosition
  (return (Transformation|GetWorldLocation (Variables|Default|GetUnitSpawnHighlight))))

(fn AddUnittoSpawnerArmy
  (params (Unit%20Object :type BP%20Unit%20Object%20Object%20Reference) (WaveNumber :type Integer))
  (bind _returnvalue (Utilities|Array|Add (.army (Utilities|Array|Get(acopy) (Variables|Waves|GetarmyWaves) (- WaveNumber 1))) Unit%20Object))
  (Default|AddUnit (Variables|Default|GetW%20Spawner%20Hover) (Variables|Waves|GetarmyWaves))
  (Default|AddUnitinSpawnerInfo (CallFunction|GetWLevelUI) Unit%20Object _returnvalue (Variables|Waves|GetwaveSpawning))
  (Default|UpdateSelectedUnitsCount (CallFunction|GetGMLevelGameMode) true))

(fn RemoveUnitfromArmy
  (params (unitIndex :type Integer))
  (Utilities|Array|RemoveIndex (.army (Utilities|Array|Get(acopy) (Variables|Waves|GetarmyWaves) (- (Variables|/Game/BluePrint/Player/GM_LevelGameMode.GM_LevelGameMode_C|GetcurrentSelectedSpawnerWave (CallFunction|GetGMLevelGameMode)) 1))) unitIndex)
  (Default|UpdateSelectedUnitsCount (CallFunction|GetGMLevelGameMode) false)
  (Widget|Panel|ClearChildren (Variables|/Game/BluePrint/_Widgets/Level/Spawner/Hover/W_SpawnerHover.W_SpawnerHover_C|GetVerticalBox (Variables|Default|GetW%20Spawner%20Hover))))

(fn SelectSpawner
  (params (select :type Boolean))
  (bind _level_ui (CallFunction|GetWLevelUI))
  (if select
    (if (not (Variables|Default|Getselected))
      (Default|SetClickedSpawner (CallFunction|GetGMLevelGameMode) self true)
      (Default|SetUnhover (Variables|Default|GetW%20Spawner%20Hover))
      (Class|NiagaraComponent|SetAsset (Variables|Default|GetNiagara) "/Game/NiagaraVFX/NS_SPNotSelected.NS_SPNotSelected" true)
      (Rendering|SetVisibility (Variables|Default|GetHoverWidget) false false)
      (Class|NiagaraComponent|SetAsset (Variables|Default|GetNiagara) "/Game/NiagaraVFX/NS_SPClicked-HoveredUnit.NS_SPClicked-HoveredUnit" true)
      (Default|OpenTroopSelection (CallFunction|GetWLevelUI))
      (Variables|Default|Setselected true))
    (elif (Variables|Default|Getselected)
      (Default|SetClickedSpawner (CallFunction|GetGMLevelGameMode) self false)
      (Class|NiagaraComponent|SetAsset (Variables|Default|GetNiagara) "/Game/NiagaraVFX/NS_SPHover.NS_SPHover" true)
      (Class|NiagaraComponent|SetAsset (Variables|Default|GetNiagara) "/Game/NiagaraVFX/NS_SPNotSelected.NS_SPNotSelected" true)
      (Rendering|SetVisibility (Variables|Default|GetHoverWidget) false false)
      (Default|ShowSpawnerInfo _level_ui false)
      (Default|CloseTroopSelection _level_ui)
      (Variables|Default|Setselected false))))

(fn SpawnUnits
  (params (Unit%20Object :type BP%20Unit%20Object%20Object%20Reference))
  (Utilities|Casting|CastToDA_Commander (Variables|/Game/BluePrint/Units/BP_UnitObject.BP_UnitObject_C|GetUnit%20Data Unit%20Object)
    (:then
      (bind _returnvalue (Game|SpawnActorfromClass "/Game/BluePrint/Units/BP_Commander_Unit.BP_Commander_Unit_C" (Transformation|GetWorldTransform (Variables|Default|GetUnitSpawnPoint)) "AlwaysSpawn" "MultiplyWithRoot" 0 0))
      (Default|SetStats _returnvalue Unit%20Object self (Variables|Default|GetnextPathBlock) (Variables|Default|GetCustomTimeDilation))
      (Default|CallOnCommanderSpawned (CallFunction|GetGMLevelGameMode))
      (Default|AddSpawnedUnit (CallFunction|GetGMLevelGameMode) _returnvalue)
      (Default|MovetoNextPathBlock _returnvalue))
    (:CastFailed
      (bind _returnvalue_2 (Game|SpawnActorfromClass "/Game/BluePrint/Units/BP_Troop_Unit.BP_Troop_Unit_C" (Transformation|GetWorldTransform (Variables|Default|GetUnitSpawnPoint)) "AlwaysSpawn" "MultiplyWithRoot" 0 0))
      (Default|SetStats _returnvalue_2 Unit%20Object self (Variables|Default|GetnextPathBlock) (Variables|Default|GetCustomTimeDilation))
      (Default|AddSpawnedUnit (CallFunction|GetGMLevelGameMode) _returnvalue_2)
      (Default|MovetoNextPathBlock _returnvalue_2))))

(fn AreAllWavesEmpty
  (for _array_element (Variables|Waves|GetarmyWaves)
    (if (Utilities|Array|IsEmpty (.army _array_element))
      (Math|Integer|IncrementInt (LocalVariables|GettempEmptyWaves))))
  (return (== (LocalVariables|GettempEmptyWaves) (Utilities|Array|Length (Variables|Waves|GetarmyWaves)))))

(fn AutoSelectWavefromSpawner
  (Default|AutoSelectWave (CallFunction|GetGMLevelGameMode) (Variables|Waves|GetarmyWaves)))