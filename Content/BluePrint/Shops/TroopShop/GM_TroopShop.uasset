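; Game mode for the troop shop, which opens the shop screen and relays item selections to it.
; On BeginPlay it creates the W_TroopShop widget, adds it to the viewport and switches to UI-only input with a visible cursor.
; Troop and gem selections are forwarded to the widget to show stats.
; Selection-border clearing is passed on through CallDisableSelectedShopBorder with shop, army, gem and type arguments.
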(event EventBeginPlay
  (bind _returnvalue (Game|GetPlayerController 0))
  (bind _returnvalue_2 (UserInterface|CreateWidget "/Game/BluePrint/Shops/TroopShop/W_TroopShop.W_TroopShop_C"))
  (bind _output_get (Variables|Default|SettroopShop _returnvalue_2))
  (UserInterface|Viewport|AddtoViewport _output_get 0)
  (Input|SetInputModeUIOnly _returnvalue _output_get "DoNotLock" false)
  (Variables|/Script/Engine.PlayerController|SetbShowMouseCursor _returnvalue true))

(fn ConstructionScript)

(fn DisableSelectedItemBorder
  (params (shop :type W%20Troop%20Shop%20Button%20Object%20Reference) (army :type W%20Troop%20T%20Shop%20Displayer%20Object%20Reference) (gem :type W%20Gem%20T%20Displayer%20Button%20Object%20Reference) (type :type E_ButtonType%20Enum :default "NewEnumerator0"))
  (Default|CallDisableSelectedShopBorder shop army gem type))

(fn SetSelectedTroop
  (params (troop :type DA%20Unit%20Object%20Reference) (type :type E_ButtonType%20Enum :default "NewEnumerator0") (gridIndex :type Integer))
  (Default|ShowTroopStats (Variables|Default|GettroopShop) troop type gridIndex))

(fn SetSelectedGem
  (params (gem :type DA%20Gem%20Object%20Reference) (gridIndex :type Integer))
  (Default|ShowGemStats (Variables|Default|GettroopShop) gem gridIndex))