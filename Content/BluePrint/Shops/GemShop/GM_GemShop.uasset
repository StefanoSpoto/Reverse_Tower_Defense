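; GM_GemShop is the gem shop's game mode, which opens the shop screen and relays selection events to it.
; On BeginPlay it creates and displays the W_GemShop widget, switches input to UI only and shows the mouse cursor.
; SetSelectedTroop and SetSelectedGem forward selections to the widget's stats views.
; DisableSelectedItemBorder fires DisableSelectedGemShopBorder with its shop, army, gem and type arguments to clear selection borders.
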(event EventBeginPlay
  (bind _returnvalue (Game|GetPlayerController 0))
  (bind _returnvalue_2 (UserInterface|CreateWidget "/Game/BluePrint/Shops/GemShop/W_GemShop.W_GemShop_C"))
  (bind _output_get (Variables|Default|SetgemShop _returnvalue_2))
  (UserInterface|Viewport|AddtoViewport _output_get 0)
  (Input|SetInputModeUIOnly _returnvalue _output_get "DoNotLock" false)
  (Variables|/Script/Engine.PlayerController|SetbShowMouseCursor _returnvalue true))

(fn ConstructionScript)

(fn DisableSelectedItemBorder
  (params (shop :type W%20Gem%20Shop%20Button%20Object%20Reference) (army :type W%20Troop%20G%20Shop%20Displayer%20Object%20Reference) (gem :type W%20Gem%20G%20Displayer%20Button%20Object%20Reference) (type :type E_ButtonType%20Enum :default "NewEnumerator0"))
  (Default|CallDisableSelectedGemShopBorder shop army gem type))

(fn SetSelectedTroop
  (params (troop :type BP%20Unit%20Object%20Object%20Reference) (gridIndex :type Integer))
  (Default|ShowTroopStats (Variables|Default|GetgemShop) troop gridIndex))

(fn SetSelectedGem
  (params (gem :type DA%20Gem%20Object%20Reference) (gridIndex :type Integer) (type :type E_ButtonType%20Enum :default "NewEnumerator0"))
  (Default|ShowGemStats (Variables|Default|GetgemShop) gem gridIndex type))