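; Blueprint function library of global accessors for the game's core framework objects in ReverseTD.
; Getters cast the game instance, level and level-selection game modes, player controller and player camera pawn to project classes, returning nothing useful if the cast fails.
; The level UI widget is reached through the level game mode.
; It also includes a utility that rounds floats to a given number of decimal digits.
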(fn GetGIReverseTD
  (bind _asgi_reverse_td (Utilities|Casting|CastToGI_ReverseTD (Game|GetGameInstance)))
  (return _asgi_reverse_td))

(fn GetGMLevelGameMode
  (bind _asgm_level_game_mode (Utilities|Casting|CastToGM_LevelGameMode (Game|GetGameMode)))
  (return _asgm_level_game_mode))

(fn GetPlayerCameraComponent
  (bind _asbp_player_camera (Utilities|Casting|CastToBP_PlayerCamera (Game|Player|GetPlayerPawn 0)))
  (return (Variables|/Game/BluePrint/Player/BP_PlayerCamera.BP_PlayerCamera_C|GetCamera _asbp_player_camera)))

(fn GetWLevelUI
  (return (Variables|/Game/BluePrint/Player/GM_LevelGameMode.GM_LevelGameMode_C|GetW%20Level%20UI (CallFunction|GetGMLevelGameMode))))

(fn GetGMLevelSelectionGameMode
  (bind _asgm_level_selection (Utilities|Casting|CastToGM_LevelSelection (Game|GetGameMode)))
  (return _asgm_level_selection))

(fn RoundFloattoXDigitPrecision
  (params (Value :type Float%20%28double-precision%29) (Decimal%20Digits :type Integer))
  (bind _output_get (LocalVariables|SettruncatedMultiplier (Math|Float|Truncate (Math|Float|Power 1e+01 (Math|Conversions|ToFloat(Integer) Decimal%20Digits)))))
  (return (/ (Math|Float|Round (* _output_get Value)) _output_get)))

(fn GetBPLevelPlayerController
  (bind _asbp_level_player_controller (Utilities|Casting|CastToBP_LevelPlayerController (Game|GetPlayerController 0)))
  (return _asbp_level_player_controller))