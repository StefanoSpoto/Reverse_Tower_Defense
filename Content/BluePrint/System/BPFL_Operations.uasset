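; A Blueprint function library of small shared utilities for numeric rounding and UI button styling.
; RoundFloatToXDigitPrecision rounds a value to a given number of decimals by scaling with a power of ten, rounding and dividing back.
; SetButtonImage keeps each state's tint and applies the new image only to the Normal state, setting Hovered, Pressed and Disabled to the fixed S_SectionButton image.
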(fn RoundFloattoXDigitPrecision
  (params (Value :type Float%20%28double-precision%29) (Decimal%20Digits :type Integer))
  (bind _output_get (LocalVariables|SettruncatedMultiplier (Math|Float|Truncate (Math|Float|Power 1e+01 (Math|Conversions|ToFloat(Integer) Decimal%20Digits)))))
  (return (/ (Math|Float|Round (* _output_get Value)) _output_get)))

(fn SetButtonImage
  (params (Button :type Button%20Object%20Reference) (New%20Image :type Object%20Object%20Reference))
  (bind _widgetstyle (Variables|/Script/UMG.Button|GetWidgetStyle Button))
  (Class|Button|SetStyle Button (Utilities|Struct|MakeButtonStyle (Utilities|Struct|MakeSlateBrush "Image" "NoTile" "NoMirror" "(X=32.000000,Y=32.000000)" "(Left=0.000000,Top=0.000000,Right=0.000000,Bottom=0.000000)" (.tintcolor (.normal _widgetstyle)) "(CornerRadii=(X=0.000000,Y=0.000000,Z=0.000000,W=1.000000),Color=(SpecifiedColor=(R=0.000000,G=0.000000,B=0.000000,A=0.000000),ColorUseRule=UseColor_Specified),Width=0.000000,RoundingType=HalfHeightRadius,bUseBrushTransparency=False)" New%20Image) (Utilities|Struct|MakeSlateBrush "Image" "NoTile" "NoMirror" "(X=32.000000,Y=32.000000)" "(Left=0.000000,Top=0.000000,Right=0.000000,Bottom=0.000000)" (.tintcolor (.hovered _widgetstyle)) "(CornerRadii=(X=0.000000,Y=0.000000,Z=0.000000,W=1.000000),Color=(SpecifiedColor=(R=0.000000,G=0.000000,B=0.000000,A=0.000000),ColorUseRule=UseColor_Specified),Width=0.000000,RoundingType=HalfHeightRadius,bUseBrushTransparency=False)" "/Game/Sprites/UI/S_SectionButton.S_SectionButton") (Utilities|Struct|MakeSlateBrush "Image" "NoTile" "NoMirror" "(X=32.000000,Y=32.000000)" "(Left=0.000000,Top=0.000000,Right=0.000000,Bottom=0.000000)" (.tintcolor (.pressed _widgetstyle)) "(CornerRadii=(X=0.000000,Y=0.000000,Z=0.000000,W=1.000000),Color=(SpecifiedColor=(R=0.000000,G=0.000000,B=0.000000,A=0.000000),ColorUseRule=UseColor_Specified),Width=0.000000,RoundingType=HalfHeightRadius,bUseBrushTransparency=False)" "/Game/Sprites/UI/S_SectionButton.S_SectionButton") (Utilities|Struct|MakeSlateBrush "NoDrawType" "NoTile" "NoMirror" "(X=0.000000,Y=0.000000)" "(Left=0.000000,Top=0.000000,Right=0.000000,Bottom=0.000000)" (.tintcolor (.disabled _widgetstyle)) "(CornerRadii=(X=0.000000,Y=0.000000,Z=0.000000,W=1.000000),Color=(SpecifiedColor=(R=0.000000,G=0.000000,B=0.000000,A=0.000000),ColorUseRule=UseColor_Specified),Width=0.000000,RoundingType=HalfHeightRadius,bUseBrushTransparency=False)" "/Game/Sprites/UI/S_SectionButton.S_SectionButton") "(SpecifiedColor=(R=1.000000,G=0.000000,B=1.000000,A=1.000000),ColorUseRule=UseColor_Foreground)" "(SpecifiedColor=(R=1.000000,G=0.000000,B=1.000000,A=1.000000),ColorUseRule=UseColor_Foreground)" "(SpecifiedColor=(R=1.000000,G=0.000000,B=1.000000,A=1.000000),ColorUseRule=UseColor_Foreground)" "(SpecifiedColor=(R=1.000000,G=0.000000,B=1.000000,A=1.000000),ColorUseRule=UseColor_Foreground)" "(Left=0.000000,Top=0.000000,Right=0.000000,Bottom=0.000000)" "(Left=0.000000,Top=0.000000,Right=0.000000,Bottom=0.000000)" "(ResourceObject=None)" "(ResourceObject=None)")))