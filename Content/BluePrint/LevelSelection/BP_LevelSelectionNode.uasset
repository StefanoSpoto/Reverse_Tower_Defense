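; Selectable node on the level selection map, holding its grid position, floor number, room type and incoming and outgoing edges to other nodes.
; Edge helpers test whether a given node leads into this one and detect crossing connections from a neighboring column.
; Room type sets the sphere outline material, and availability toggles its custom depth rendering.
; While available, cursor hover switches the game mode's highlight actor between light blue and yellow outlines.
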(event OnBeginCursorOver(HoverCollision)
  (params (TouchedComponent :type Primitive%20Component%20Object%20Reference))
  (if (Variables|Default|GetavailableToClick)
    (Default|ActivateLightBlueOutline (Variables|/Game/BluePrint/LevelSelection/GM_LevelSelection.GM_LevelSelection_C|GetHighlightNodes%20Actor (CallFunction|GetGMLevelSelectionGameMode)))))

(event OnEndCursorOver(HoverCollision)
  (params (TouchedComponent :type Primitive%20Component%20Object%20Reference))
  (if (Variables|Default|GetavailableToClick)
    (Default|ActivateYellowOutline (Variables|/Game/BluePrint/LevelSelection/GM_LevelSelection.GM_LevelSelection_C|GetHighlightNodes%20Actor (CallFunction|GetGMLevelSelectionGameMode)))))

(fn ConstructionScript)

(fn Init
  (params (X :type Integer) (Y :type Integer))
  (Variables|Node|SetgridX X)
  (bind _output_get (Variables|Node|SetgridY Y))
  (Variables|Node|SetFloorNumber _output_get))

(fn SetSelectedNode
  (Variables|Node|Setselected true))

(fn CheckforNodeinArrivingEdges
  (params (Node :type BP%20Level%20Selection%20Node%20Object%20Reference))
  (bind _arrivingedges (Variables|Node|GetarrivingEdges))
  (if (> (Utilities|Array|Length _arrivingedges) 0)
    (bind _array_element (Utilities|Array|ForEachLoopwithBreak _arrivingedges :!label _label)
      (:LoopBody
        (if (== (Variables|/Game/BluePrint/LevelSelection/BP_LevelSelectionEdge.BP_LevelSelectionEdge_C|GetStartNode _array_element) Node)
          (LocalVariables|Setexits true)
          (goto _label Break)
          (else
            (LocalVariables|Setexits false))))
      (:Completed
        (return (LocalVariables|Getexits))))
    (else
      (return (LocalVariables|Getexits)))))

(fn AddArrivingEdge
  (params (edge :type BP%20Level%20Selection%20Edge%20Object%20Reference%20%28by%20ref%29))
  (Utilities|Array|Add (Variables|Node|GetarrivingEdges) edge))

(fn SetStartEdge
  (params (edge :type BP%20Level%20Selection%20Edge%20Object%20Reference))
  (Utilities|Array|Add (Variables|Node|GetstartingEdges) edge))

(fn CheckforCrossroad
  (params (isLeftCross :type Boolean) (xIndex :type Integer))
  (if isLeftCross
    (LocalVariables|SetxIndexToCheck (+ xIndex 1))
    (else
      (LocalVariables|SetxIndexToCheck (- xIndex 1))))
  (bind _array_element (Utilities|Array|ForEachLoopwithBreak (Variables|Node|GetarrivingEdges) :!label _label)
    (:LoopBody
      (if (== (Variables|BP_LevelSelectionNode_C|GetgridX (Variables|/Game/BluePrint/LevelSelection/BP_LevelSelectionEdge.BP_LevelSelectionEdge_C|GetStartNode _array_element)) (LocalVariables|GetxIndexToCheck))
        (LocalVariables|SetisCross true)
        (goto _label Break)))
    (:Completed
      (return (LocalVariables|GetisCross)))))

(fn SetRoomType
  (params (roomType :type DA%20Room%20Object%20Reference))
  (bind _output_get (Variables|Node|Settype roomType))
  (Rendering|Material|SetMaterial (Variables|Default|GetSphere%20Outline) 0 (Variables|/Game/BluePrint/LevelSelection/RoomDataAsset/DA_Room.DA_Room_C|Getmateria _output_get)))

(fn SetAvailabletoClick
  (params (available :type Boolean))
  (bind _output_get (Variables|Default|SetavailableToClick available))
  (Rendering|SetRenderCustomDepth (Variables|Default|GetSphere%20Outline) _output_get))

(fn GetHoverDelay
  (return 0.0))