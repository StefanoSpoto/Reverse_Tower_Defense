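; Game mode for the level selection screen that sets up its UI and mouse-driven input.
; On BeginPlay it shows the cursor, adds the level selection widget with game-and-UI input, and creates a collapsed army gem manager widget initialized with units and gems.
; OpenGemManager toggles that menu, switching between UI-only and game-and-UI input, and GetGemManager exposes the widget to other objects.
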(event EventBeginPlay
  (Variables|/Script/Engine.PlayerController|SetbShowMouseCursor (Game|GetPlayerController 0) true)
  ;[1 1 1] HUD
  (bind _returnvalue (UserInterface|CreateWidget "/Game/BluePrint/_Widgets/Level_Selection/W_LevelSelection_UI.W_LevelSelection_UI_C"))
  (bind _output_get (Variables|Default|SetW%20Level%20Selection%20UI _returnvalue))
  (UserInterface|Viewport|AddtoViewport _output_get 0)
  (Input|SetInputModeGameandUI (Game|GetPlayerController 0) _output_get "DoNotLock" false true)
  ;[1 1 1] Gem manager menu
  (bind _returnvalue_2 (UserInterface|CreateWidget "/Game/BluePrint/_Widgets/Menus/Gem_Manager/W_ArmyGemManager.W_ArmyGemManager_C"))
  (bind _output_get_2 (Variables|Default|SetW%20Gems%20Manager _returnvalue_2))
  (UserInterface|Viewport|AddtoViewport _output_get_2 0)
  (Widget|SetVisibility _output_get_2 "Collapsed")
  (Default|SetUpUnitsandGems (Variables|Default|GetW%20Gems%20Manager)))

(fn ConstructionScript)

(fn OpenGemManager
  (params (open :type Boolean))
  (if open
    (Widget|SetVisibility (Variables|Default|GetW%20Gems%20Manager) "Visible")
    (Input|SetInputModeUIOnly (Game|GetPlayerController 0) (Variables|Default|GetW%20Gems%20Manager) "DoNotLock" true)
    (else
      (Widget|SetVisibility (Variables|Default|GetW%20Gems%20Manager) "Collapsed")
      (Input|SetInputModeGameandUI (Game|GetPlayerController 0) (Variables|Default|GetW%20Level%20Selection%20UI) "DoNotLock" false true))))

(fn GetGemManager
  (return (Variables|Default|GetW%20Gems%20Manager)))