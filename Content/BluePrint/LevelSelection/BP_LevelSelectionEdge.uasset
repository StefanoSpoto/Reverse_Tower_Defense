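; BP_LevelSelectionEdge is the visual link between two node actors in level selection, drawn as a cube.
; InitEdge stores both endpoints, then places the actor at their midpoint, rotated to face the end node.
; It stretches the X scale by the distance between them to span the gap.
; The cube always gets a white emissive material, leaving the Material input unused, and the function returns the edge itself.
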(fn ConstructionScript)

(fn InitEdge
  (params (startNode :type BP%20Level%20Selection%20Node%20Object%20Reference) (endNode :type BP%20Level%20Selection%20Node%20Object%20Reference) (material :type Material%20Interface%20Object%20Reference))
  (bind _returnvalue (Transformation|GetActorLocation startNode))
  (bind _returnvalue_2 (Transformation|GetActorLocation endNode))
  (Rendering|Material|SetMaterial (Variables|Default|GetCube) 0 "/Game/Materials/Programmers_Material/Emissive_Colors/MI_White_Emissive.MI_White_Emissive")
  (Variables|Default|SetStartNode startNode)
  (Variables|Default|SetEndNode endNode)
  (Transformation|SetActorLocationAndRotation (/ (+ _returnvalue _returnvalue_2) 2.0) (Math|Rotator|FindLookatRotation _returnvalue _returnvalue_2))
  (Transformation|SetActorScale3D (Math|Vector|MakeVector (/ (Math|Vector|Distance(Vector) _returnvalue _returnvalue_2) 3e+02) 0.75 1.0))
  (return self))