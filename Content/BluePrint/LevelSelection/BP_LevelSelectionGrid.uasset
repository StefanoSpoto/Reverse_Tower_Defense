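; BP_LevelSelectionGrid procedurally generates a branching level-selection map of rooms ending in a boss.
; On BeginPlay it spawns a node grid, then traces paths from random first-row starts through adjacent next-row neighbours, recursively spawning edges and capping crossings.
; Path nodes get room types by weighted probability ranges, with starts fixed as normal stages.
; Unconnected nodes are destroyed, and surviving last-row nodes link to one centred boss node.
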(event EventBeginPlay
  (bind _noderowarray (Variables|Default|GetnodeRowArray))
  (CallFunction|SetRangeforRoomProbability)
  (bind (_current_point _total_points _0_1_phase _poly_center _x_row _y_row) (Utilities|2DGridExecutionMacro (Variables|Default|GetnodeOffset) (Transformation|GetActorLocation) (Variables|Default|GetxSize) (Variables|Default|GetySize))
    (:Per%20Poly%20Execution
      (bind _returnvalue (Game|SpawnActorfromClass "/Game/BluePrint/LevelSelection/BP_LevelSelectionNode.BP_LevelSelectionNode_C" (Math|Conversions|ToTransform(Vector) _poly_center) "AlwaysSpawn" "MultiplyWithRoot" 0 0))
      (Default|Init _returnvalue _x_row _y_row)
      (Utilities|Array|Add _noderowarray _returnvalue)
      (if (== _x_row (- (Variables|Default|GetxSize) 1))
        (Utilities|Array|SetArrayElem (Variables|Default|GetnodeMatrix) _y_row (Utilities|Struct|MakeBS_NodeYArray _noderowarray) true)
        (Utilities|Array|Clear (Variables|Default|GetnodeRowArray))
        (if (== _y_row 0)
          (Utilities|Array|Add (Variables|Default|GetnodeFirstRow) _returnvalue)
          (elif (== (+ _current_point 1) _total_points)
            (CallFunction|SelectStartingNodes)))))))

(fn ConstructionScript)

(fn SelectStartingNodes
  (bind _nodematrix (Variables|Default|GetnodeMatrix))
  (bind _lastrownodes (LocalVariables|GetlastRowNodes))
  (bind _nodematrix_2 (Variables|Default|GetnodeMatrix))
  (bind _output (Utilities|Array|Get(acopy) _nodematrix))
  (while (< (LocalVariables|GetcurrentTotalStartingNodes) (Variables|Default|GetstartingTotalNodes))
    (bind _output_get (LocalVariables|SetrandomIndex (Math|Random|RandomInteger (Utilities|Array|Length (.node _output)))))
    (if (not (Variables|/Game/BluePrint/LevelSelection/BP_LevelSelectionNode.BP_LevelSelectionNode_C|Getselected (Utilities|Array|Get(acopy) (.node _output) _output_get)))
      (Default|SetSelectedNode (Utilities|Array|Get(acopy) (.node _output) _output_get))
      (Default|SetRoomType (Utilities|Array|Get(acopy) (.node _output) _output_get) "/Game/BluePrint/LevelSelection/RoomDataAsset/DAT_NormalStage.DAT_NormalStage")
      (CallFunction|SetNextNode (Utilities|Array|Get(acopy) (.node _output) _output_get))
      (Math|Integer|IncrementInt (LocalVariables|GetcurrentTotalStartingNodes)
        (:%20%20
          (Math|Integer|IncrementInt (Variables|Default|GetcolorIndex))))))
  ;[1 1 1] Destroy Un-used nodes
  (for (_ _array_index) _nodematrix_2
    (if (== _array_index (Utilities|Array|LastIndex _nodematrix_2))
      (LocalVariables|SetnotLastRow false))
    (for _array_element (.node (Utilities|Array|Get(acopy) (Variables|Default|GetnodeMatrix) _array_index))
      (if (LocalVariables|GetnotLastRow)
        (if (== (Utilities|Array|Length (Variables|/Game/BluePrint/LevelSelection/BP_LevelSelectionNode.BP_LevelSelectionNode_C|GetstartingEdge _array_element)) 0)
          (Actor|DestroyActor _array_element))
        (elif (== (Utilities|Array|Length (Variables|/Game/BluePrint/LevelSelection/BP_LevelSelectionNode.BP_LevelSelectionNode_C|GetarrivingEdges _array_element)) 0)
          (Actor|DestroyActor _array_element)
          (else
            (Utilities|Array|Add (LocalVariables|GetlastRowNodes) _array_element))))))
  ;[1 0.2419 0.4023] Spawn Boss Room
  (for _array_element_2 (LocalVariables|GetlastRowNodes)
    (LocalVariables|SetxMedium (+ (LocalVariables|GetxMedium) (.x (Transformation|GetActorLocation _array_element_2)))))
  (bind _returnvalue (Game|SpawnActorfromClass "/Game/BluePrint/LevelSelection/BP_LevelSelectionNode.BP_LevelSelectionNode_C" (Math|Transform|MakeTransform (Math|Vector|MakeVector (/ (LocalVariables|GetxMedium) (Utilities|Array|Length (LocalVariables|GetlastRowNodes))) (+ (.y (Transformation|GetActorLocation (Utilities|Array|Get(acopy) _lastrownodes (Utilities|Array|LastIndex _lastrownodes)))) (Variables|Default|GetnodeOffset)) 0.0) "0, 0, 0" "1.500000,1.500000,1.500000") "Undefined" "MultiplyWithRoot" 0 0))
  (Variables|/Game/BluePrint/LevelSelection/BP_LevelSelectionNode.BP_LevelSelectionNode_C|SetgridY _returnvalue (Variables|Default|GetySize))
  (Default|SetRoomType _returnvalue "/Game/BluePrint/LevelSelection/RoomDataAsset/DAT_Boss.DAT_Boss")
  (for _array_element_3 (LocalVariables|GetlastRowNodes)
    (bind _returnvalue_2 (Game|SpawnActorfromClass "/Game/BluePrint/LevelSelection/BP_LevelSelectionEdge.BP_LevelSelectionEdge_C" (Math|Transform|MakeTransform "0, 0, 0" "0, 0, 0" "1.000000,1.000000,1.000000") "Undefined" "MultiplyWithRoot" 0 0))
    (bind _selfedge (Default|Init _returnvalue_2 _array_element_3 _returnvalue (Utilities|Array|Get(acopy) (Variables|Default|Getcolors) (Variables|Default|GetcolorIndex))))
    (Default|SetStartEdge _array_element_3 _selfedge)
    (Default|AddArrivingEdge _returnvalue _selfedge)))

(fn GetNeighbours
  (params (xMatrixIndex :type Integer) (yMatrixIndex :type Integer))
  (bind _result (Math|Integer|IncrementInt yMatrixIndex)
    (:%20%20
      (LocalVariables|SetyIndex _result)
      (bind _output_get (LocalVariables|SetxIndex xMatrixIndex))
      (if (<= (+ yMatrixIndex 1) (Variables|Default|GetySize))
        (Utilities|Array|Add (LocalVariables|Getneighbours) (Utilities|Array|Get(acopy) (.node (Utilities|Array|Get(acopy) (Variables|Default|GetnodeMatrix) (LocalVariables|GetyIndex))) _output_get))
        (Utilities|FlowControl|Sequence
          (:then_0
            (if (< (+ (LocalVariables|GetxIndex) 1) (Variables|Default|GetxSize))
              (Utilities|Array|Add (LocalVariables|Getneighbours) (Utilities|Array|Get(acopy) (.node (Utilities|Array|Get(acopy) (Variables|Default|GetnodeMatrix) (LocalVariables|GetyIndex))) (+ (LocalVariables|GetxIndex) 1)))))
          (:then_1
            (if (>= (- (LocalVariables|GetxIndex) 1) 0)
              (Utilities|Array|Add (LocalVariables|Getneighbours) (Utilities|Array|Get(acopy) (.node (Utilities|Array|Get(acopy) (Variables|Default|GetnodeMatrix) (LocalVariables|GetyIndex))) (- (LocalVariables|GetxIndex) 1)))))
          (:then_2
            (return (LocalVariables|Getneighbours))))
        (else
          (return (LocalVariables|Getneighbours)))))))

(fn SetNextNode
  (params (StartNode :type BP%20Level%20Selection%20Node%20Object%20Reference))
  (LocalVariables|SetcurrentStartNode StartNode)
  (bind _nodeneighbours (CallFunction|GetNeighbours (Variables|/Game/BluePrint/LevelSelection/BP_LevelSelectionNode.BP_LevelSelectionNode_C|GetgridX StartNode) (Variables|/Game/BluePrint/LevelSelection/BP_LevelSelectionNode.BP_LevelSelectionNode_C|GetgridY StartNode)))
  (if (not (== (Utilities|Array|Length _nodeneighbours) 0))
    (bind _output_get (LocalVariables|SetrandomIndex (Math|Random|RandomInteger (Utilities|Array|Length _nodeneighbours))))
    (Utilities|FlowControl|ForLoopwithBreak 0 (Utilities|Array|Length _nodeneighbours) :!label _label
      (:LoopBody
        (bind _existsinarrivingedges (Default|CheckforNodeinArrivingEdges (Utilities|Array|Get(acopy) _nodeneighbours _output_get) (LocalVariables|GetcurrentStartNode)))
        (if _existsinarrivingedges
          (bind _result (Math|Integer|IncrementInt (LocalVariables|GetrandomIndex))
            (:%20%20
              (if (== (Utilities|Array|Length _nodeneighbours) _result)
                (LocalVariables|SetrandomIndex 0))))
          (elif (== (Variables|/Game/BluePrint/LevelSelection/BP_LevelSelectionNode.BP_LevelSelectionNode_C|GetgridX (Utilities|Array|Get(acopy) _nodeneighbours (LocalVariables|GetrandomIndex))) (Variables|/Game/BluePrint/LevelSelection/BP_LevelSelectionNode.BP_LevelSelectionNode_C|GetgridX (LocalVariables|GetcurrentStartNode)))
            (bind _output_get_2 (LocalVariables|SetnewNode (Utilities|Array|Get(acopy) _nodeneighbours _output_get) :!label _label_2))
            (bind _returnvalue (Game|SpawnActorfromClass "/Game/BluePrint/LevelSelection/BP_LevelSelectionEdge.BP_LevelSelectionEdge_C" (Math|Transform|MakeTransform "0, 0, 0" "0, 0, 0" "1.000000,1.000000,1.000000") "Undefined" "MultiplyWithRoot" 0 0))
            (bind _selfedge (Default|Init _returnvalue (LocalVariables|GetcurrentStartNode) _output_get_2 (Utilities|Array|Get(acopy) (Variables|Default|Getcolors) (Variables|Default|GetcolorIndex))))
            (Default|SetStartEdge (LocalVariables|GetcurrentStartNode) _selfedge)
            (Default|AddArrivingEdge (LocalVariables|GetnewNode) _selfedge)
            (bind _roomtype (CallFunction|GetRandomRoomType))
            (Default|SetRoomType (LocalVariables|GetnewNode) _roomtype)
            (goto _label Break)
            (else
              (bind _cross (Default|CheckforCrossroad (Utilities|Array|Get(acopy) (.node (Utilities|Array|Get(acopy) (Variables|Default|GetnodeMatrix) (+ (Variables|/Game/BluePrint/LevelSelection/BP_LevelSelectionNode.BP_LevelSelectionNode_C|GetgridY (LocalVariables|GetcurrentStartNode)) 1))) (Variables|/Game/BluePrint/LevelSelection/BP_LevelSelectionNode.BP_LevelSelectionNode_C|GetgridX (LocalVariables|GetcurrentStartNode))) (> (Variables|/Game/BluePrint/LevelSelection/BP_LevelSelectionNode.BP_LevelSelectionNode_C|GetgridX (Utilities|Array|Get(acopy) _nodeneighbours (LocalVariables|GetrandomIndex))) (Variables|/Game/BluePrint/LevelSelection/BP_LevelSelectionNode.BP_LevelSelectionNode_C|GetgridX (LocalVariables|GetcurrentStartNode))) (Variables|/Game/BluePrint/LevelSelection/BP_LevelSelectionNode.BP_LevelSelectionNode_C|GetgridX (LocalVariables|GetcurrentStartNode))))
              (if _cross
                (if (< (Variables|Default|GetcurrentCrossroads) (Variables|Default|GetmaxCrossroads))
                  (Math|Integer|IncrementInt (Variables|Default|GetcurrentCrossroads)
                    (:%20%20
                      (goto _label_2)))
                  (else
                    (bind _result_2 (Math|Integer|IncrementInt (LocalVariables|GetrandomIndex))
                      (:%20%20
                        (if (== (Utilities|Array|Length _nodeneighbours) _result_2)
                          (LocalVariables|SetrandomIndex 0))))))
                (else
                  (goto _label_2)))))))
      (:Completed
        (CallFunction|SetNextNode _output_get_2)))))

(fn GetRandomRoomType
  (LocalVariables|SetrandomNum (Math|Random|RandomIntegerinRange 1 100))
  (bind _array_element (Utilities|Array|ForEachLoopwithBreak (Variables|RoomType|GetroomTypes))
    (:LoopBody
      (if (and (<= (Variables|/Game/BluePrint/LevelSelection/RoomDataAsset/DA_Room.DA_Room_C|GetlowRange _array_element) (LocalVariables|GetrandomNum)) (>= (Variables|/Game/BluePrint/LevelSelection/RoomDataAsset/DA_Room.DA_Room_C|GethighRange _array_element) (LocalVariables|GetrandomNum)))
        (return _array_element)))))

(fn SetRangeforRoomProbability
  (for _array_element (Variables|RoomType|GetroomTypes)
    (Variables|/Game/BluePrint/LevelSelection/RoomDataAsset/DA_Room.DA_Room_C|SetlowRange _array_element (+ (LocalVariables|Getlow) 1))
    (bind _output_get (Variables|/Game/BluePrint/LevelSelection/RoomDataAsset/DA_Room.DA_Room_C|SethighRange _array_element (Math|Float|Truncate (+ (LocalVariables|Getlow) (Variables|/Game/BluePrint/LevelSelection/RoomDataAsset/DA_Room.DA_Room_C|GetspawnProbability _array_element)))))
    (LocalVariables|Setlow _output_get)))