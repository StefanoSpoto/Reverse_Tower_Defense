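; Stage selector Blueprint meant to load a random level for a chosen node type, such as combat, boss, shop or special room.
; On BeginPlay it binds SelectLevel to the player's load-level event, which forwards the node type to LoadRandomLevel.
; LoadRandomLevel currently only prints the type.
; Its switch, which would stream a random level instance from per-type soft-reference arrays, is disconnected and never runs.
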(event Custom|SelectLevel
  (params (NodeType :type E_NodeType%20Enum :default "NewEnumerator0"))
  (CallFunction|LoadRandomLevel NodeType))

(event EventBeginPlay
  (EventDispatchers|BindEventtoLoadLevel (Variables|Default|Getplayer) (delegate Custom|SelectLevel)))

(fn ConstructionScript)

(fn LoadRandomLevel
  (params (type :type E_NodeType%20Enum :default "NewEnumerator0"))
  (Development|PrintString (Utilities|String|EnumtoString type) true true "(R=0.017737,G=0.000000,B=1.000000,A=1.000000)"))