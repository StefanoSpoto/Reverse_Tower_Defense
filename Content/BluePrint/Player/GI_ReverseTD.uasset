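; GI_ReverseTD is the game instance for a reverse tower defense game, holding the player's army, commander, gold and gems across levels.
; Units and the commander are BP_UnitObjects built from data assets, with the commander's data setting army gem socket limits and starting coins.
; Level loading can optionally clear the army and commander, alongside helpers for restarting, clamped gold spending, and test gems and units.
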(fn RestartLevel
  (bind _returnvalue (Game|GetCurrentLevelName true))
  (Game|OpenLevel(byName) (Utilities|String|StringToName _returnvalue)))

(fn LoadLevel
  (params (Level :type World%20Soft%20Object%20Reference) (Reset%20Army :type Boolean))
  (if Reset%20Army
    (Utilities|Array|Clear (Variables|Army|GetunitArmy))
    (Variables|Commander|Setcommander 0))
  (Game|OpenLevel(byObjectReference) Level))

(fn AddUnittoArmy
  (params (unitData :type DA%20Unit%20Object%20Reference))
  (bind _returnvalue (Game|ConstructObjectfromClass "/Game/BluePrint/Units/BP_UnitObject.BP_UnitObject_C"))
  (Variables|/Game/BluePrint/Units/BP_UnitObject.BP_UnitObject_C|SetUnit%20Data _returnvalue unitData)
  (Default|SetGemSockets _returnvalue (Units|GetCommanderMaxGemSockets))
  (Default|Init _returnvalue)
  (Utilities|Array|Add (Variables|Army|GetunitArmy) _returnvalue))

(fn GetCommanderStartingCoins
  (return (Math|Float|Truncate (Variables|/Game/BluePrint/Units/DataAssets/Commanders/DA_Commander.DA_Commander_C|GetstartingCoins (Variables|Commander|GetcommanderData)))))

(fn SetCommander
  (params (Commander%20Data :type DA%20Commander%20Object%20Reference))
  (bind _output_get (Variables|Commander|SetcommanderData Commander%20Data))
  (bind _returnvalue (Game|ConstructObjectfromClass "/Game/BluePrint/Units/BP_UnitObject.BP_UnitObject_C"))
  (bind _output_get_2 (Variables|Commander|Setcommander _returnvalue))
  (Variables|/Game/BluePrint/Units/BP_UnitObject.BP_UnitObject_C|SetUnit%20Data _output_get_2 _output_get))

(fn GetTestGems
  (return (Variables|Gems|GetGems)))

(fn RemoveTestGem
  (params (indexToRemove :type Integer))
  (Utilities|Array|RemoveIndex (Variables|Gems|GetGems) indexToRemove))

(fn AddTestGem
  (params (gem :type DA%20Gem%20Object%20Reference))
  (Utilities|Array|Add (Variables|Gems|GetGems) gem))

(fn GetCommanderMaxGemSockets
  (return (Variables|/Game/BluePrint/Units/DataAssets/Commanders/DA_Commander.DA_Commander_C|GetmaxAviableGemSockets (Variables|Commander|GetcommanderData))))

(fn SetMaxGemSocketsinArmy
  (for _array_element (Variables|Army|GetunitArmy)
    (Default|SetGemSockets _array_element (Units|GetCommanderMaxGemSockets))))

(fn GainGold
  (params (gold :type Integer))
  (Variables|Gold|SettotalGold (+ gold (Variables|Gold|GettotalGold))))

(fn SpendGold
  (params (gold :type Integer))
  (bind _output_get (Variables|Gold|SettotalGold (- (Variables|Gold|GettotalGold) gold)))
  (if (< _output_get 0)
    (Variables|Gold|SettotalGold 0)))

(fn TestAddUnittoArmy
  (for _index (range 0 12)
    (bind _returnvalue (Game|ConstructObjectfromClass "/Game/BluePrint/Units/BP_UnitObject.BP_UnitObject_C"))
    (Variables|/Game/BluePrint/Units/BP_UnitObject.BP_UnitObject_C|SetUnit%20Data _returnvalue "/Game/BluePrint/Units/DataAssets/Troops/DAT_Chonki.DAT_Chonki")
    (Utilities|Array|Add (Variables|Army|GetunitArmy) _returnvalue)))