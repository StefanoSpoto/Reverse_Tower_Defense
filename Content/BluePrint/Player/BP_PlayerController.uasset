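; Player controller that lets the player click path blocks in the world to switch their orientation.
; On BeginPlay it adds the player input mapping context through Enhanced Input.
; The click action converts the DPI-scaled mouse position to pixels, deprojects it and runs a long Visibility line trace.
; If the hit actor is a BP_PathBlock, it calls SwitchOrientation on it.
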(event Input|EnhancedActionEvents|EnhancedInputActionIA_Click
  (params (ActionValue :type Boolean) (ElapsedSeconds :type Float%20%28double-precision%29) (TriggeredSeconds :type Float%20%28double-precision%29) (InputAction :type Input%20Action%20Object%20Reference :default "/Game/Inputs/IA_Click.IA_Click"))
  (:Started
    (bind _returnvalue (Class|WidgetLayoutLibrary|GetMousePositiononViewport))
    (bind _outhit (Collision|LineTraceByChannel (.WorldPosition (Class|GameplayStatics|DeprojectScreentoWorld (Game|GetPlayerController 0) (* _returnvalue (Class|WidgetLayoutLibrary|GetViewportScale)))) (+ (.WorldPosition (Class|GameplayStatics|DeprojectScreentoWorld (Game|GetPlayerController 0) (* _returnvalue (Class|WidgetLayoutLibrary|GetViewportScale)))) (* (.WorldDirection (Class|GameplayStatics|DeprojectScreentoWorld (Game|GetPlayerController 0) (* _returnvalue (Class|WidgetLayoutLibrary|GetViewportScale)))) 9999.0)) "TraceTypeQuery1" false 0 "None"))
    (Utilities|IsValid (.hitactor _outhit)
      (:Is%20Valid
        (bind _asbp_path_block (Utilities|Casting|CastToBP_PathBlock (.hitactor _outhit)))
        (Default|SwitchOrientation _asbp_path_block)))))

(event EventBeginPlay
  (bind _returnvalue (PlayerController|LocalPlayerSubsystems|GetEnhancedInputLocalPlayerSubsystem))
  (Utilities|IsValid _returnvalue
    (:Is%20Valid
      (Input|AddMappingContext _returnvalue "/Game/Inputs/IMC_PlayerInputs.IMC_PlayerInputs" 0 "(bIgnoreAllPressedKeysUntilRelease=True,bForceImmediately=False,bNotifyUserSettings=False)"))))

(fn ConstructionScript)