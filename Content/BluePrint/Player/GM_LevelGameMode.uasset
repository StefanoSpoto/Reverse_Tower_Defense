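; Game mode for a reverse tower defense level, coordinating UI, spawners, waves, the commander and win/lose flow.
; BeginPlay shows the tutorial and prebuilds HUD, gem manager and result screens, which join the viewport when the tutorial finishes.
; It tracks selected spawner, wave and spawned units, broadcasting selection and game-speed changes through dispatchers.
; Unit deaths trigger loss once none remain; winning freezes time and tallies gold from units and strongholds.
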(event Custom|CheckLoseCondition
  (if (Utilities|Array|IsEmpty (Variables|Units|GetspawnedUnits))
    (UI|OpenLoseScreen true)))

(event EventBeginPlay
  (bind _asgi_reverse_td (CallFunction|GetGIReverseTD))
  (bind _returnvalue (UserInterface|CreateWidget "/Game/BluePrint/_Widgets/Tutorial/WB_Tutorial.WB_Tutorial_C"))
  (UserInterface|Viewport|AddtoViewport _returnvalue 0)
  (Input|SetInputModeUIOnly (CallFunction|GetBPLevelPlayerController) _returnvalue "DoNotLock" true)
  ;[1 1 1] HUD
  (bind _returnvalue_2 (UserInterface|CreateWidget "/Game/BluePrint/_Widgets/Level/W_LevelUI.W_LevelUI_C"))
  (bind _output_get (Variables|UI|SetW%20Level%20UI _returnvalue_2))
  (Default|SetUpArmyButtonsandCommanderAbility _output_get (Variables|/Game/BluePrint/Player/GI_ReverseTD.GI_ReverseTD_C|GetunitArmy _asgi_reverse_td) (Variables|/Game/BluePrint/Player/GI_ReverseTD.GI_ReverseTD_C|Getcommander _asgi_reverse_td))
  (Default|EnableTroopButtons _output_get false)
  ;[1 1 1] Gem Manager Menu
  (bind _returnvalue_3 (UserInterface|CreateWidget "/Game/BluePrint/_Widgets/Menus/Gem_Manager/W_ArmyGemManager.W_ArmyGemManager_C"))
  (bind _output_get_2 (Variables|UI|SetW%20Gems%20Manager _returnvalue_3))
  (Widget|SetVisibility _output_get_2 "Collapsed")
  (Default|SetUpUnitsandGems (Variables|UI|GetW%20Gems%20Manager))
  ;[1 1 1] Win screen
  (bind _returnvalue_4 (UserInterface|CreateWidget "/Game/BluePrint/_Widgets/Level/W_WinScreen.W_WinScreen_C"))
  (bind _output_get_3 (Variables|UI|SetW%20Win%20Screen _returnvalue_4))
  (Widget|SetVisibility _output_get_3 "Collapsed")
  ;[1 1 1] Lose screen
  (bind _returnvalue_5 (UserInterface|CreateWidget "/Game/BluePrint/_Widgets/Level/W_LoseScreen.W_LoseScreen_C"))
  (bind _output_get_4 (Variables|UI|SetW%20Lose%20Screen _returnvalue_5))
  (Widget|SetVisibility _output_get_4 "Collapsed")
  ;[1 1 1] Get all spawners in level
  (bind _outactors (Actor|GetAllActorsOfClass "/Game/BluePrint/Path/Spawner/BP_UnitSpawner_PathBlock.BP_UnitSpawner_PathBlock_C"))
  (bind _output_get_5 (Variables|Spawner|SetspawnersInLevel _outactors))
  (for _array_element _output_get_5
    (Default|AddSpawnerTabButton (Variables|UI|GetW%20Level%20UI) (Variables|/Game/BluePrint/Path/Spawner/BP_UnitSpawner_PathBlock.BP_UnitSpawner_PathBlock_C|GetspawnerIndex _array_element))
    (EventDispatchers|BindEventtoOnUnitDeath (delegate Custom|CheckLoseCondition))))

(fn ConstructionScript)

(fn SetClickedSpawner
  (params (newSpawner :type BP%20Unit%20Spawner%20Path%20Block%20Object%20Reference) (select :type Boolean))
  ;[1 1 1] Si Setta come variabile
  (if select
    (bind _output_get (Variables|Spawner|SetselectedSpawnerReference newSpawner))
    (Default|CallOnSelectSpawner _output_get)
    (Default|ChangeSpawnerAspect _output_get true)
    (else
      (bind _output_get_2 (Variables|Spawner|SetselectedSpawnerReference 0))
      (Default|CallOnSelectSpawner _output_get_2)
      (Default|ChangeSpawnerAspect newSpawner false))))

(fn SetTurretUI
  (params (isVisible :type Boolean) (name :type String) (damage :type Float%20%28double-precision%29) (fireRate :type Float%20%28double-precision%29) (range :type Float%20%28double-precision%29) (specialTrait :type String) (damageType :type E_DamageType%20Enum :default "NewEnumerator0"))
  (bind _w_level_ui (Variables|UI|GetW%20Level%20UI))
  (bind _turretinfo (Variables|/Game/BluePrint/_Widgets/Level/W_LevelUI.W_LevelUI_C|GetTurretInfo _w_level_ui))
  (if isVisible
    (Widget|SetVisibility _turretinfo "Visible")
    (else
      (Widget|SetVisibility _turretinfo "Collapsed")))
  (Default|UpdateTurretInfo (Variables|UI|GetW%20Level%20UI) name damage fireRate range specialTrait damageType))

(fn UpdateSelectedUnitsCount
  (params (Is%20Increment :type Boolean))
  (Utilities|FlowControl|Sequence
    (:then_0
      (if Is%20Increment
        (Math|Integer|IncrementInt (Variables|Spawner|GetselectedUnitsCount)
          (:%20%20
            (Default|CallOnArmyIncrease)))
        (else
          (bind _result (Math|Integer|DecrementInt (Variables|Spawner|GetselectedUnitsCount))
            (:%20%20
              (if (<= _result 0)
                (Default|CallOnArmyDecrease)))))))
    (:then_1
      (if (> (Variables|Spawner|GetcurrentSelectedSpawnerWave) (Variables|Spawner|GetmaxUsedWave))
        (Variables|Spawner|SetmaxUsedWave (Variables|Spawner|GetcurrentSelectedSpawnerWave))))))

(fn SelectSpawnerfromTab
  (params (SpawnerIndex :type Integer))
  (Default|CallOnSelectSpawner (Variables|Spawner|GetselectedSpawnerReference))
  (for _array_element (Variables|Spawner|GetspawnersInLevel)
    (if (== (Variables|/Game/BluePrint/Path/Spawner/BP_UnitSpawner_PathBlock.BP_UnitSpawner_PathBlock_C|GetspawnerIndex _array_element) SpawnerIndex)
      (Default|SelectSpawner _array_element true))))

(fn AddSpawnedUnit
  (params (unit :type BP%20Unit%20Object%20Reference))
  (Utilities|Array|Add (Variables|Units|GetspawnedUnits) unit)
  (bind _asbp_commander_unit (Utilities|Casting|CastToBP_Commander_Unit unit))
  (Variables|Units|SetcommanderUnit _asbp_commander_unit))

(fn RemoveSpawnedUnit
  (params (unit :type BP%20Unit%20Object%20Reference))
  (Utilities|Array|RemoveItem (Variables|Units|GetspawnedUnits) unit))

(fn UseCommanderActiveAbility
  (Default|ActivateActiveAbility (Variables|Units|GetcommanderUnit)))

(fn IsCommanderAviable
  (return (Utilities|Array|ContainsItem (Variables|Units|GetspawnedUnits) (Variables|Units|GetcommanderUnit))))

(fn IsSpawnerAviable
  (Utilities|IsValid (Variables|Spawner|GetselectedSpawnerReference)
    (:Is%20Valid
      (return (not (Variables|/Game/BluePrint/Path/Spawner/BP_UnitSpawner_PathBlock.BP_UnitSpawner_PathBlock_C|GetisSpawning (Variables|Spawner|GetselectedSpawnerReference)))))
    (:Is%20Not%20Valid
      (return false))))

(fn IsCurrentSpawner
  (params (spawner :type BP%20Unit%20Spawner%20Path%20Block%20Object%20Reference))
  (return (== spawner (Variables|Spawner|GetselectedSpawnerReference))))

(fn GetCurrentWaveArmy
  (bind _currentselectedspawnerwave (Variables|Spawner|GetcurrentSelectedSpawnerWave))
  (Development|PrintString (Utilities|String|ToString(Integer) _currentselectedspawnerwave))
  (return (.army (Utilities|Array|Get(acopy) (Variables|/Game/BluePrint/Path/Spawner/BP_UnitSpawner_PathBlock.BP_UnitSpawner_PathBlock_C|GetarmyWaves (Variables|Spawner|GetselectedSpawnerReference)) _currentselectedspawnerwave))))

(fn SelectWave
  (params (SelectedWave :type Integer) (ManualSelection :type Boolean) (Army%20Waves :type Array%20of%20BS%20Spawner%20Army%20Wave%20Structures))
  (bind _w_level_ui (Variables|UI|GetW%20Level%20UI))
  (Variables|Spawner|SetcurrentSelectedSpawnerWave SelectedWave)
  (if ManualSelection
    (Default|CallOnClickWaveButton _w_level_ui (Variables|Spawner|GetcurrentSelectedSpawnerWave) :!label _label)
    (Default|ShowSpawnerInfo _w_level_ui true (Utilities|Array|Get(acopy) Army%20Waves (- (Variables|Spawner|GetcurrentSelectedSpawnerWave) 1)))
    (else
      (bind _array_element (Utilities|Array|ForEachLoopwithBreak Army%20Waves :!label _label_2)
        (:LoopBody
          (if (Utilities|Array|IsNotEmpty (.Army (Utilities|Struct|BreakBS_SpawnerArmyWave _array_element)))
            (Variables|Spawner|SetcurrentSelectedSpawnerWave (.WaveNumber (Utilities|Struct|BreakBS_SpawnerArmyWave _array_element)))
            (goto _label_2 Break)))
        (:Completed
          (goto _label))))))

(fn AutoSelectWave
  (params (Army%20Waves :type Array%20of%20BS%20Spawner%20Army%20Wave%20Structures))
  (bind _w_level_ui (Variables|UI|GetW%20Level%20UI))
  (bind _array_element (Utilities|Array|ForEachLoopwithBreak Army%20Waves :!label _label)
    (:LoopBody
      (if (not (.HasBeenSpawned (Utilities|Struct|BreakBS_SpawnerArmyWave _array_element)))
        (Variables|Spawner|SetcurrentSelectedSpawnerWave (.WaveNumber (Utilities|Struct|BreakBS_SpawnerArmyWave _array_element)))
        (goto _label Break)))
    (:Completed
      (Default|CallOnClickWaveButton _w_level_ui (Variables|Spawner|GetcurrentSelectedSpawnerWave))
      (Default|ShowSpawnerInfo _w_level_ui true (Utilities|Array|Get(acopy) Army%20Waves (- (Variables|Spawner|GetcurrentSelectedSpawnerWave) 1))))))

(fn IsNoSpawnerSelected
  (for _array_element (Variables|Spawner|GetspawnersInLevel)
    (if (not (Variables|/Game/BluePrint/Path/Spawner/BP_UnitSpawner_PathBlock.BP_UnitSpawner_PathBlock_C|Getselected _array_element))
      (Math|Integer|IncrementInt (LocalVariables|Getcount))))
  (return (== (LocalVariables|Getcount) (Utilities|Array|Length (Variables|Spawner|GetspawnersInLevel)))))

(fn OpenGemManager
  (params (open :type Boolean))
  (if open
    (Widget|SetVisibility (Variables|UI|GetW%20Gems%20Manager) "Visible")
    (Input|SetInputModeUIOnly (Game|GetPlayerController 0) (Variables|UI|GetW%20Gems%20Manager) "DoNotLock" true)
    (else
      (Widget|SetVisibility (Variables|UI|GetW%20Gems%20Manager) "Collapsed")
      (Input|SetInputModeGameandUI (Game|GetPlayerController 0) (Variables|UI|GetW%20Level%20UI) "DoNotLock" true true))))

(fn GetGemManager
  (return (Variables|UI|GetW%20Gems%20Manager)))

(fn OpenWinScreen
  (params (open :type Boolean) (UnitsThatReachedTheEnd :type Array%20of%20BP%20Unit%20Object%20References) (EndStrongholdGold :type Integer))
  (if open
    (Utilities|Time|SetGlobalTimeDilation 0.0)
    (for _array_element UnitsThatReachedTheEnd
      (LocalVariables|SettotalCoinGold (+ (Variables|/Game/BluePrint/Units/BP_Unit.BP_Unit_C|Getgold _array_element) (LocalVariables|GettotalCoinGold)))
      (LocalVariables|SettotalGemBonusGold (+ (Variables|/Game/BluePrint/Units/BP_UnitObject.BP_UnitObject_C|GetEnd%20Level%20Gold%20Bonus (Variables|/Game/BluePrint/Units/BP_Unit.BP_Unit_C|GetUnit%20Object _array_element)) (LocalVariables|GettotalGemBonusGold))))
    (for _array_element_2 (Variables|Units|GetspawnedUnits)
      (LocalVariables|SettotalGoldOfSurvivedUnits (+ 1 (LocalVariables|GettotalGoldOfSurvivedUnits))))
    (Default|SetResults (Variables|UI|GetW%20Win%20Screen) (LocalVariables|GettotalCoinGold) (LocalVariables|GettotalGoldOfSurvivedUnits) (LocalVariables|GettotalGemBonusGold) (Variables|Gold|GettotalStrongholdGold) EndStrongholdGold)
    (Widget|SetVisibility (Variables|UI|GetW%20Win%20Screen) "Visible")
    (Widget|SetVisibility (Variables|UI|GetW%20Level%20UI) "Collapsed")
    (Input|SetInputModeUIOnly (Game|GetPlayerController 0) (Variables|UI|GetW%20Win%20Screen) "DoNotLock" true)
    (else
      (Widget|SetVisibility (Variables|UI|GetW%20Win%20Screen) "Collapsed")
      (Widget|SetVisibility (Variables|UI|GetW%20Level%20UI) "Visible")
      (Input|SetInputModeGameandUI (Game|GetPlayerController 0) (Variables|UI|GetW%20Level%20UI) "DoNotLock" true true))))

(fn IncrementTotalStrongholdGold
  (params (Stronghold%20Gold :type Integer))
  (Variables|Gold|SettotalStrongholdGold (+ Stronghold%20Gold (Variables|Gold|GettotalStrongholdGold))))

(fn OpenLoseScreen
  (params (open :type Boolean))
  (if open
    (Utilities|Time|SetGlobalTimeDilation 0.0)
    (Widget|SetVisibility (Variables|UI|GetW%20Lose%20Screen) "Visible")
    (Widget|SetVisibility (Variables|UI|GetW%20Level%20UI) "Collapsed")
    (Input|SetInputModeUIOnly (Game|GetPlayerController 0) (Variables|UI|GetW%20Gems%20Manager) "DoNotLock" true)
    (else
      (Widget|SetVisibility (Variables|UI|GetW%20Lose%20Screen) "Collapsed")
      (Widget|SetVisibility (Variables|UI|GetW%20Level%20UI) "Visible")
      (Input|SetInputModeGameandUI (Game|GetPlayerController 0) (Variables|UI|GetW%20Level%20UI) "DoNotLock" true true))))

(fn SpeedUp
  (bind _result (Math|Integer|IncrementInt (Variables|Speed|GetglobalSpeedsIndex))
    (:%20%20
      (if (> _result (Utilities|Array|LastIndex (Variables|Speed|GetglobalSpeeds)))
        (Variables|Speed|SetglobalSpeedsIndex 0))
      (Default|CallOnChangeTimeDilation (Utilities|Array|Get(acopy) (Variables|Speed|GetglobalSpeeds) (Variables|Speed|GetglobalSpeedsIndex)))
      (Default|ChangeSpeedUpText (CallFunction|GetWLevelUI) (Utilities|Array|Get(acopy) (Variables|Speed|GetglobalSpeeds) (Variables|Speed|GetglobalSpeedsIndex))))))

(fn PauseSpeed
  (params (Pause :type Boolean))
  (bind _globalspeeds (Variables|Speed|GetglobalSpeeds))
  (bind _globalspeedsindex (Variables|Speed|GetglobalSpeedsIndex))
  (bind _output (Utilities|Array|Get(acopy) _globalspeeds _globalspeedsindex))
  (if Pause
    (Default|CallOnChangeTimeDilation 0.0)
    (Default|ChangeSpeedUpText (CallFunction|GetWLevelUI) 0.0)
    (else
      (Default|CallOnChangeTimeDilation _output)
      (Default|ChangeSpeedUpText (CallFunction|GetWLevelUI) _output))))

(fn AddSpawnedWaves
  (params (Wave :type Integer%20%28by%20ref%29))
  (Utilities|Array|Add (Variables|Spawner|GetspawnedWaves) Wave))

(fn HasWaveAlreadyBeenSpawned
  (params (wave :type Integer))
  (return (Utilities|Array|ContainsItem (Variables|Spawner|GetspawnedWaves) wave)))

(fn FinishTutorial
  (UserInterface|Viewport|AddtoViewport (Variables|UI|GetW%20Level%20UI) 0)
  (UserInterface|Viewport|AddtoViewport (Variables|UI|GetW%20Gems%20Manager) 0)
  (UserInterface|Viewport|AddtoViewport (Variables|UI|GetW%20Win%20Screen) 0)
  (UserInterface|Viewport|AddtoViewport (Variables|UI|GetW%20Lose%20Screen) 0)
  (Input|SetInputModeGameandUI (Game|GetPlayerController 0) (Variables|UI|GetW%20Level%20UI) "DoNotLock" true true))