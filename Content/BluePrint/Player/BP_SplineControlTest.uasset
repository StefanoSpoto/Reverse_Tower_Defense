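; Test orbit camera that makes itself the view target of player controller 0 on BeginPlay.
; Enhanced Input rotate and zoom actions drive the CameraBoom's yaw, pitch and arm length, scaled by delta time and per-axis speeds.
; Pitch and zoom clamp to configurable limits, with roll held at zero.
; The construction script applies the starting Length to the boom; despite the asset name, the graphs use no spline.
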(event Input|EnhancedActionEvents|EnhancedInputActionIA_RotateCamera
  (params (ActionValue :type Vector%202D%20Structure) (ElapsedSeconds :type Float%20%28double-precision%29) (TriggeredSeconds :type Float%20%28double-precision%29) (InputAction :type Input%20Action%20Object%20Reference :default "/Game/Inputs/IA_RotateCamera.IA_RotateCamera"))
  (CallFunction|SetOrbitMovement (.x ActionValue))
  (CallFunction|SetUpwardsRotation (.y ActionValue)))

(event Input|EnhancedActionEvents|EnhancedInputActionIA_ZoomCamera
  (params (ActionValue :type Float%20%28double-precision%29) (ElapsedSeconds :type Float%20%28double-precision%29) (TriggeredSeconds :type Float%20%28double-precision%29) (InputAction :type Input%20Action%20Object%20Reference :default "/Game/Inputs/IA_ZoomCamera.IA_ZoomCamera"))
  (CallFunction|SetZoom ActionValue))

(event EventBeginPlay
  (Game|Player|SetViewTargetwithBlend (Game|GetPlayerController 0) self 0.0 "VTBlend_Linear" 0.0 false))

(fn ConstructionScript
  (Variables|/Script/Engine.SpringArmComponent|SetTargetArmLength (Variables|Default|GetCameraBoom) (Variables|Zoom|Getlength)))

(fn SetUpwardsRotation
  (params (Action%20Value%20Y :type Float%20%28double-precision%29))
  (bind _cameraboom (Variables|Default|GetCameraBoom))
  (bind _minrotation (Variables|UpwardsRotation|GetminRotation))
  (bind _cameraboom_2 (Variables|Default|GetCameraBoom))
  (bind _maxrotation (Variables|UpwardsRotation|GetmaxRotation))
  (bind _returnvalue (Transformation|GetWorldRotation _cameraboom_2))
  (bind _returnvalue_2 (Transformation|GetWorldRotation _cameraboom))
  (Transformation|SetWorldRotation _cameraboom_2 (Math|Rotator|MakeRotator 0.0 (+ (* (* Action%20Value%20Y (* (Utilities|Time|GetWorldDeltaSeconds) (Variables|UpwardsRotation|GetrotationSpeed))) -1.0) (.pitch _returnvalue_2)) (.yaw _returnvalue_2)) false false)
  (if (> (.pitch _returnvalue) _minrotation)
    (Transformation|SetWorldRotation (Variables|Default|GetCameraBoom) (Math|Rotator|MakeRotator 0.0 _minrotation (.yaw _returnvalue)) false false)
    (elif (< (.pitch _returnvalue) _maxrotation)
      (Transformation|SetWorldRotation (Variables|Default|GetCameraBoom) (Math|Rotator|MakeRotator 0.0 _maxrotation (.yaw _returnvalue)) false false))))

(fn SetOrbitMovement
  (params (Action%20Value%20X :type Float%20%28double-precision%29))
  (bind _cameraboom (Variables|Default|GetCameraBoom))
  (Transformation|SetWorldRotation _cameraboom (Math|Rotator|MakeRotator 0.0 (.pitch (Transformation|GetWorldRotation _cameraboom)) (+ (.yaw (Transformation|GetWorldRotation _cameraboom)) (* (* (Utilities|Time|GetWorldDeltaSeconds) (Variables|OrbitMovement|GetmoveSpeed)) (* Action%20Value%20X -1.0)))) false false))

(fn SetZoom
  (params (Action%20Value%20Y :type Float%20%28double-precision%29))
  (bind _maxlength (Variables|Zoom|GetmaxLength))
  (bind _minlength (Variables|Zoom|GetminLength))
  (bind _output_get (Variables|Zoom|Setlength (- (Variables|Zoom|Getlength) (* Action%20Value%20Y (* (Utilities|Time|GetWorldDeltaSeconds) (Variables|Zoom|GetzoomSpeed))))))
  (bind _output_get_2 (Variables|/Script/Engine.SpringArmComponent|SetTargetArmLength (Variables|Default|GetCameraBoom) _output_get))
  (if (> _output_get_2 _maxlength)
    (bind _output_get_3 (Variables|Zoom|Setlength _maxlength))
    (Variables|/Script/Engine.SpringArmComponent|SetTargetArmLength (Variables|Default|GetCameraBoom) _output_get_3)
    (elif (< _output_get_2 _minlength)
      (bind _output_get_4 (Variables|Zoom|Setlength _minlength))
      (Variables|/Script/Engine.SpringArmComponent|SetTargetArmLength (Variables|Default|GetCameraBoom) _output_get_4))))