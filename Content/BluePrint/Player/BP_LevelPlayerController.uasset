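; Player controller for levels that handles mouse interaction with path blocks and hoverable actors such as strongholds.
; On begin play it adds the input mapping context, and clicks trace under the cursor to switch a path block's orientation.
; Each tick, an object trace broadcasts an unhover-all call, then outlines any BPI_Hoverable hit and sets it hovered after that actor's own delay.
; The UnhoverActor call in the event graph is disconnected.
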(event Custom|Hover%20Actor
  (params (Hit%20Actor :type Actor%20Object%20Reference))
  (bind _asbpi_hoverable (Utilities|Casting|CastToBPI_Hoverable Hit%20Actor))
  (Default|ShowOutline _asbpi_hoverable true)
  (bind _delay (Default|GetHoverDelay _asbpi_hoverable))
  (Utilities|FlowControl|Delay _delay)
  (Default|SetHover _asbpi_hoverable)
  (Variables|Default|SethoveredActor Hit%20Actor)
  (Variables|Default|SetisHovering true))

(event Input|EnhancedActionEvents|EnhancedInputActionIA_ClickPathBlock
  (params (ActionValue :type Boolean) (ElapsedSeconds :type Float%20%28double-precision%29) (TriggeredSeconds :type Float%20%28double-precision%29) (InputAction :type Input%20Action%20Object%20Reference :default "/Game/Inputs/IA_ClickPathBlock.IA_ClickPathBlock"))
  (bind (_locationx _locationy) (Game|Player|GetMousePosition))
  (bind _self self)
  (bind (_worldposition _worlddirection) (Class|GameplayStatics|DeprojectScreentoWorld _self (Math|Vector2D|MakeVector2D _locationx _locationy)))
  ;[1 1 1] Switch Path Block click detection
  (:Started
    (bind _outhit (Collision|LineTraceByChannel _worldposition (+ _worldposition (* _worlddirection 9999.0)) "TraceTypeQuery1" false 0 "None"))
    (if (.bblockinghit _outhit)
      (bind _asbp_path_block (Utilities|Casting|CastToBP_PathBlock (.hitactor _outhit)))
      (Default|SwitchOrientation _asbp_path_block))))

(event EventTick
  (params (DeltaSeconds :type Float%20%28single-precision%29))
  (bind (_locationx _locationy) (Game|Player|GetMousePosition))
  (bind _self self)
  (bind (_worldposition _worlddirection) (Class|GameplayStatics|DeprojectScreentoWorld _self (Math|Vector2D|MakeVector2D _locationx _locationy)))
  ;[1 1 1] Stronghold hover detection
  (bind _outhit (Collision|LineTraceForObjects _worldposition (+ _worldposition (* _worlddirection 9999.0)) (Utilities|Array|MakeArray "ObjectTypeQuery8" "ObjectTypeQuery9") false 0 "None"))
  (if (.bblockinghit _outhit)
    (Default|CallOnUnhoverAllHoverableActors (.hitactor _outhit))
    (CallFunction|HoverActor (.hitactor _outhit))
    (else
      (Default|CallOnUnhoverAllHoverableActors))))

(event EventBeginPlay
  (bind _returnvalue (PlayerController|LocalPlayerSubsystems|GetEnhancedInputLocalPlayerSubsystem))
  (Utilities|IsValid _returnvalue
    (:Is%20Valid
      (Input|AddMappingContext _returnvalue "/Game/Inputs/IMC_PlayerInputs.IMC_PlayerInputs" 0 "(bIgnoreAllPressedKeysUntilRelease=True,bForceImmediately=False,bNotifyUserSettings=False)"))))

(fn ConstructionScript)

(fn MouseHoverLineTrace
  (params (ObjectTypes :type Array%20of%20EObjectTypeQuery%20Enums :default "ObjectTypeQuery1"))
  (bind (_locationx _locationy) (Game|Player|GetMousePosition))
  (bind _self self)
  (bind (_worldposition _worlddirection) (Class|GameplayStatics|DeprojectScreentoWorld _self (Math|Vector2D|MakeVector2D _locationx _locationy)))
  (bind _outhit (Collision|LineTraceForObjects _worldposition (+ _worldposition (* _worlddirection 9999.0)) ObjectTypes false 0 "None"))
  (return (.hitactor _outhit)))

(fn UnhoverActor
  (bind _hoveredactor (Variables|Default|GethoveredActor))
  (Utilities|IsValid _hoveredactor
    (:Is%20Valid
      (bind _asbpi_hoverable (Utilities|Casting|CastToBPI_Hoverable _hoveredactor))
      (Default|SetUnhover _asbpi_hoverable))))