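; GI_Test_ReverseTD is a game instance, apparently for a reverse tower defense test, that holds the player's unit army and chosen commander.
; It restarts the current level by name or opens another, optionally clearing the army and commander.
; Units added to the army receive the commander's gem sockets if they are troop data assets.
; It also exposes the commander's starting coins as a truncated integer.
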(fn RestartLevel
  (bind _returnvalue (Game|GetCurrentLevelName true))
  (Game|OpenLevel(byName) (Utilities|String|StringToName _returnvalue)))

(fn OpenLevel
  (params (Level :type World%20Soft%20Object%20Reference) (resetArmy :type Boolean))
  (if resetArmy
    (Utilities|Array|Clear (Variables|Units|GetunitArmy))
    (Variables|Units|Setcommander "/Game/BluePrint/Units/DataAssets/Commanders/DAC_None.DAC_None"))
  (Game|OpenLevel(byObjectReference) Level))

(fn AddUnittoArmy
  (params (unit :type DA%20Unit%20Object%20Reference))
  (bind _commander (Variables|Units|Getcommander))
  (Utilities|FlowControl|Sequence
    (:then_0
      (bind _asda_troop (Utilities|Casting|CastToDA_Troop unit))
      (Utilities|IsValid _commander
        (:Is%20Valid
          (Default|SetGemSockets _asda_troop (Variables|/Game/BluePrint/Units/DataAssets/Commanders/DA_Commander.DA_Commander_C|GetgemSockets _commander)))))
    (:then_1
      (Utilities|Array|Add (Variables|Units|GetunitArmy) unit))))

(fn GetCommanderStartingCoins
  (return (Math|Float|Truncate (Variables|/Game/BluePrint/Units/DataAssets/Commanders/DA_Commander.DA_Commander_C|GetstartingCoins (Variables|Units|Getcommander)))))