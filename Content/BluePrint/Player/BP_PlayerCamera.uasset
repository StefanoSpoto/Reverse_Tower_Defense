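; Player camera pawn with a spring arm that pans, rotates and zooms over the level and also forwards a game speed-up input to the level game mode.
; Enhanced Input sets a desired location and zoom, which Tick interpolates toward; mouse drag moves the actor directly and click-held rotation applies yaw.
; When the game mode reports a selected spawner, the camera glides to its ground position, blocking camera input until a timeline finishes.
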(event Custom|OnSpawnerSelected
  (params (Spawner%20Actor :type BP%20Unit%20Spawner%20Path%20Block%20Object%20Reference))
  (Utilities|IsValid Spawner%20Actor
    (:Is%20Valid
      (CallFunction|LookatSpawner (Transformation|GetActorLocation Spawner%20Actor)))))

(event Custom|LookAtSpawner
  (params (Spawner%20Position :type Vector))
  (bind (_x _y) (Math|Vector|BreakVector Spawner%20Position))
  (Variables|LookatSpawner|SetcanReadInput false)
  (Variables|Movement|SetdesiredLocation (Math|Vector|MakeVector _x _y 0.0))
  (Timeline|LookAtSpawner%20Timeline PlayFromStart
    (:Finished
      (Variables|LookatSpawner|SetcanReadInput true))))

(event Input|EnhancedActionEvents|EnhancedInputActionIA_MoveCamera_Keyboard
  (params (ActionValue :type Vector%202D%20Structure) (ElapsedSeconds :type Float%20%28double-precision%29) (TriggeredSeconds :type Float%20%28double-precision%29) (InputAction :type Input%20Action%20Object%20Reference :default "/Game/Inputs/Camera_Movement/IA_MoveCamera_Keyboard.IA_MoveCamera_Keyboard"))
  ;[1 1 1] Movement keyboard
  (if (Variables|LookatSpawner|GetcanReadInput)
    (if (not (Variables|Movement|GetisClickedMovement))
      (Variables|Movement|SetdesiredLocation (+ (* (Transformation|GetActorRightVector) (* (Variables|Movement|GetmoveSpeed) (.x ActionValue))) (Variables|Movement|GetdesiredLocation)))
      (Variables|Movement|SetdesiredLocation (+ (Variables|Movement|GetdesiredLocation) (* (* (.y ActionValue) (Variables|Movement|GetmoveSpeed)) (Transformation|GetActorForwardVector)))))))

(event Input|EnhancedActionEvents|EnhancedInputActionIA_ZoomCamera
  (params (ActionValue :type Float%20%28double-precision%29) (ElapsedSeconds :type Float%20%28double-precision%29) (TriggeredSeconds :type Float%20%28double-precision%29) (InputAction :type Input%20Action%20Object%20Reference :default "/Game/Inputs/IA_ZoomCamera.IA_ZoomCamera"))
  ;[1 1 1] Zoom input
  (if (Variables|LookatSpawner|GetcanReadInput)
    (Variables|Zoom|SetdesiredZoomLength (Math|Float|Clamp(Float) (+ (Variables|Zoom|GetdesiredZoomLength) (* (* ActionValue -1.0) (Variables|Zoom|GetzoomSpeed))) (Variables|Zoom|GetminZoomLength) (Variables|Zoom|GetmaxZoomLength)))))

(event Input|EnhancedActionEvents|EnhancedInputActionIA_RotateCamera
  (params (ActionValue :type Float%20%28double-precision%29) (ElapsedSeconds :type Float%20%28double-precision%29) (TriggeredSeconds :type Float%20%28double-precision%29) (InputAction :type Input%20Action%20Object%20Reference :default "/Game/Inputs/IA_RotateCamera.IA_RotateCamera"))
  ;[1 1 1] Rotation inputs
  (if (Variables|LookatSpawner|GetcanReadInput)
    (if (Variables|Rotation|GetisClickedRotation)
      (Transformation|SetActorRotation (Math|Rotator|CombineRotators (Transformation|GetActorRotation) (Math|Rotator|MakeRotator 0.0 0.0 (* ActionValue (Variables|Rotation|GetrotationSpeed))))))))

(event Input|EnhancedActionEvents|EnhancedInputActionIA_ClickRotateCamera
  (params (ActionValue :type Boolean) (ElapsedSeconds :type Float%20%28double-precision%29) (TriggeredSeconds :type Float%20%28double-precision%29) (InputAction :type Input%20Action%20Object%20Reference :default "/Game/Inputs/IA_ClickRotateCamera.IA_ClickRotateCamera"))
  ;[1 1 1] Rotation inputs
  (if (Variables|LookatSpawner|GetcanReadInput)
    (Variables|Rotation|SetisClickedRotation ActionValue)))

(event Input|EnhancedActionEvents|EnhancedInputActionIA_MoveCamera_Mouse
  (params (ActionValue :type Vector%202D%20Structure) (ElapsedSeconds :type Float%20%28double-precision%29) (TriggeredSeconds :type Float%20%28double-precision%29) (InputAction :type Input%20Action%20Object%20Reference :default "/Game/Inputs/Camera_Movement/IA_MoveCamera_Mouse.IA_MoveCamera_Mouse"))
  (bind _returnvalue (Transformation|GetActorLocation))
  (bind _returnvalue_2 (Transformation|GetActorForwardVector))
  (bind _returnvalue_3 (Transformation|GetActorRightVector))
  (bind _returnvalue_4 (* (.y ActionValue) -1.0))
  (bind _returnvalue_5 (* (.x ActionValue) -1.0))
  (bind _movespeed (Variables|Movement|GetmoveSpeed))
  (bind _movespeed_2 (Variables|Movement|GetmoveSpeed))
  (bind _returnvalue_6 (* _returnvalue_4 _movespeed))
  (bind _returnvalue_7 (* _movespeed_2 _returnvalue_5))
  (bind _returnvalue_8 (* _returnvalue_2 _returnvalue_6))
  (bind _returnvalue_9 (* _returnvalue_3 _returnvalue_7))
  (bind _returnvalue_10 (+ _returnvalue_9 _returnvalue_8 _returnvalue))
  ;[1 1 1] Movement click
  (if (Variables|LookatSpawner|GetcanReadInput)
    (if (Variables|Movement|GetisClickedMovement)
      (Variables|Movement|SetdesiredLocation _returnvalue_10)
      (Transformation|SetActorLocation _returnvalue_10 false false))))

(event Input|EnhancedActionEvents|EnhancedInputActionIA_ClickMoveCamera
  (params (ActionValue :type Boolean) (ElapsedSeconds :type Float%20%28double-precision%29) (TriggeredSeconds :type Float%20%28double-precision%29) (InputAction :type Input%20Action%20Object%20Reference :default "/Game/Inputs/Camera_Movement/Mouse/IA_ClickMoveCamera.IA_ClickMoveCamera"))
  ;[1 1 1] Movement click
  (if (Variables|LookatSpawner|GetcanReadInput)
    (Variables|Movement|SetisClickedMovement ActionValue)))

(event Input|EnhancedActionEvents|EnhancedInputActionIA_SpeedUp
  (params (ActionValue :type Boolean) (ElapsedSeconds :type Float%20%28double-precision%29) (TriggeredSeconds :type Float%20%28double-precision%29) (InputAction :type Input%20Action%20Object%20Reference :default "/Game/Inputs/IA_SpeedUp.IA_SpeedUp"))
  ;[1 1 1] Change game speed
  (Default|SpeedUp (CallFunction|GetGMLevelGameMode)))

(event EventTick
  (params (DeltaSeconds :type Float%20%28single-precision%29))
  (bind _springarm (Variables|Default|GetSpringArm))
  ;[1 1 1] Interpolate spring arm length (zoom)
  (Variables|/Script/Engine.SpringArmComponent|SetTargetArmLength _springarm (Math|Interpolation|FInterpTo (Variables|/Script/Engine.SpringArmComponent|GetTargetArmLength _springarm) (Variables|Zoom|GetdesiredZoomLength) DeltaSeconds 5.0))
  ;[1 1 1] Interpolate position
  (Transformation|SetActorLocation (Math|Interpolation|VInterpTo (Transformation|GetActorLocation) (Variables|Movement|GetdesiredLocation) (Utilities|Time|GetWorldDeltaSeconds) 5.0) false false))

(event EventBeginPlay
  (EventDispatchers|BindEventtoOnSelectSpawner (CallFunction|GetGMLevelGameMode) (delegate Custom|OnSpawnerSelected))
  (Variables|Movement|SetdesiredLocation (Transformation|GetActorLocation))
  (Variables|Zoom|SetdesiredZoomLength (Variables|/Script/Engine.SpringArmComponent|GetTargetArmLength (Variables|Default|GetSpringArm))))

(fn ConstructionScript)