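; Troop ability actor for the Tamer Goblin that spawns a replacement unit when the ability actor is destroyed.
; It follows the game mode's time dilation changes through its own CustomTimeDilation.
; On Destroyed it spawns a BP_Unit at its transform and registers it with the game mode.
; The new unit takes the Troop's UnitObject, path blocks and the ability's time dilation, then moves to the next path block.
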(event Custom|Change%20Custom%20Time%20Dilation
  (params (newTimeDilation :type Float%20%28double-precision%29))
  (Variables|Default|SetCustomTimeDilation newTimeDilation))

(event EventBeginPlay
  (|CallParentFunction)
  (EventDispatchers|BindEventtoOnChangeTimeDilation (CallFunction|GetGMLevelGameMode) (delegate Custom|Change%20Custom%20Time%20Dilation)))

(event EventDestroyed
  (bind _troop (Variables|Default|GetTroop))
  (bind _returnvalue (Game|SpawnActorfromClass "/Game/BluePrint/Units/BP_Unit.BP_Unit_C" (Math|Transform|MakeTransform (Transformation|GetActorLocation) (Transformation|GetActorRotation) "1.000000,1.000000,1.000000") "Undefined" "MultiplyWithRoot" 0 0))
  (Default|AddSpawnedUnit (CallFunction|GetGMLevelGameMode) _returnvalue)
  (Utilities|IsValid _returnvalue
    (:Is%20Valid
      (Default|SetStats _returnvalue (Variables|/Game/BluePrint/Units/BP_Unit.BP_Unit_C|GetUnit%20Object _troop) (Variables|/Game/BluePrint/Units/BP_Unit.BP_Unit_C|GetpreviousPath _troop) (Variables|/Game/BluePrint/Units/BP_Unit.BP_Unit_C|GetnextPath _troop) (Variables|Default|GetCustomTimeDilation))
      (Default|MovetoNextPathBlock _returnvalue))))

(fn ConstructionScript
  (|CallParentFunction))