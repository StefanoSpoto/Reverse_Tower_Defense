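; Troop ability for the Barrel Goblin that spawns three goblin units along the path when destroyed, provided its troop can move.
; Each BP_Unit starts on consecutive path blocks from the troop's previous one onward, takes the troop's UnitObject stats and begins moving.
; The ability follows the level game mode's time dilation changes and passes its custom dilation to the spawned units.
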(event Custom|Change%20Custom%20Time%20Dilation
  (params (newTimeDilation :type Float%20%28double-precision%29))
  (Variables|Default|SetCustomTimeDilation newTimeDilation))

(event EventBeginPlay
  (|CallParentFunction)
  (EventDispatchers|BindEventtoOnChangeTimeDilation (CallFunction|GetGMLevelGameMode) (delegate Custom|Change%20Custom%20Time%20Dilation)))

(event EventDestroyed
  (if (Variables|/Game/BluePrint/Units/BP_Unit.BP_Unit_C|GetcanMove (Variables|Default|GetTroop))
    (Utilities|FlowControl|Sequence
      (:then_0
        (CallFunction|SpawnGoblin (Variables|/Game/BluePrint/Units/BP_Unit.BP_Unit_C|GetpreviousPath (Variables|Default|GetTroop)) (Variables|/Game/BluePrint/Units/BP_Unit.BP_Unit_C|GetnextPath (Variables|Default|GetTroop))))
      (:then_1
        (CallFunction|SpawnGoblin (Variables|/Game/BluePrint/Units/BP_Unit.BP_Unit_C|GetnextPath (Variables|Default|GetTroop)) (Variables|/Game/BluePrint/Path/BP_PathBlock.BP_PathBlock_C|GetnextPathBlock (Variables|/Game/BluePrint/Units/BP_Unit.BP_Unit_C|GetnextPath (Variables|Default|GetTroop)))))
      (:then_2
        (CallFunction|SpawnGoblin (Variables|/Game/BluePrint/Path/BP_PathBlock.BP_PathBlock_C|GetnextPathBlock (Variables|/Game/BluePrint/Units/BP_Unit.BP_Unit_C|GetnextPath (Variables|Default|GetTroop))) (Variables|/Game/BluePrint/Path/BP_PathBlock.BP_PathBlock_C|GetnextPathBlock (Variables|/Game/BluePrint/Path/BP_PathBlock.BP_PathBlock_C|GetnextPathBlock (Variables|/Game/BluePrint/Units/BP_Unit.BP_Unit_C|GetnextPath (Variables|Default|GetTroop)))))))))

(fn ConstructionScript
  (|CallParentFunction))

(fn SpawnGoblin
  (params (startingPathBlock :type BP%20Path%20Block%20Object%20Reference) (nextPathBlock :type BP%20Path%20Block%20Object%20Reference))
  (bind _returnvalue (Game|SpawnActorfromClass "/Game/BluePrint/Units/BP_Unit.BP_Unit_C" (Math|Transform|MakeTransform (.location (Default|GetUnitPathTransform startingPathBlock)) (Transformation|GetActorRotation) "1.000000,1.000000,1.000000") "Undefined" "MultiplyWithRoot" 0 0))
  (Utilities|IsValid _returnvalue
    (:Is%20Valid
      (Default|SetStats _returnvalue (Variables|/Game/BluePrint/Units/BP_Unit.BP_Unit_C|GetUnit%20Object (Variables|Default|GetTroop)) startingPathBlock nextPathBlock (Variables|Default|GetCustomTimeDilation))
      (Default|MovetoNextPathBlock _returnvalue))))