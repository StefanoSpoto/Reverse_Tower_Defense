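; Gold Goblin troop ability Blueprint that sets the gold multiplier on its troop.
; On BeginPlay it runs the parent logic, waits half a second, then copies its GoldGoblinCoinMultiplier value into the Troop's GoldMultiplier.
; The value is set once; overlap and tick events are disabled.
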(event EventBeginPlay
  (|CallParentFunction)
  (Utilities|FlowControl|Delay 0.5)
  (Variables|/Game/BluePrint/Units/BP_Unit.BP_Unit_C|SetgoldMultiplier (Variables|Default|GetTroop) (Variables|Default|GetgoldGoblinCoinMultiplier)))

(event Collision|EventActorBeginOverlap
  (params (OtherActor :type Actor%20Object%20Reference))
  (|CallParentFunction OtherActor) ; This node is disabled and will not be called.\nDrag off pins to build functionality.
)

(event EventTick
  (params (DeltaSeconds :type Float%20%28single-precision%29))
  (|CallParentFunction DeltaSeconds) ; This node is disabled and will not be called.\nDrag off pins to build functionality.
)

(fn ConstructionScript
  (|CallParentFunction))