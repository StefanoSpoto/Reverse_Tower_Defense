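; Troop ability for the Shadow Goblin that periodically makes its troop untargetable for aggro.
; A self-retriggering ShadowStep event starts on BeginPlay and alternates two phases using the same delay.
; If the troop is not aggroed after the first delay, it turns white and cannot be aggroed.
; After the second delay, it always becomes targetable again with a black material and the cycle repeats.
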(event Custom|ShadowStep
  (Utilities|FlowControl|Delay (Variables|Default|GetshadowStepDelay))
  (if (Variables|/Game/BluePrint/Units/BP_Unit.BP_Unit_C|GetisAggroed (Variables|Default|GetTroop))
    _
    (else
      (Rendering|Material|SetMaterial (Variables|/Game/BluePrint/Units/BP_Unit.BP_Unit_C|GetSkeletalMesh (Variables|Default|GetTroop)) 0 "/Game/Materials/Programmers_Material/Solid_Color/MI_White.MI_White")
      (Variables|/Game/BluePrint/Units/BP_Unit.BP_Unit_C|SetcanBeAggro (Variables|Default|GetTroop) false)))
  (Utilities|FlowControl|Delay (Variables|Default|GetshadowStepDelay))
  (Variables|/Game/BluePrint/Units/BP_Unit.BP_Unit_C|SetcanBeAggro (Variables|Default|GetTroop) true)
  (Rendering|Material|SetMaterial (Variables|/Game/BluePrint/Units/BP_Unit.BP_Unit_C|GetSkeletalMesh (Variables|Default|GetTroop)) 0 "/Game/Materials/Programmers_Material/Solid_Color/MI_Black.MI_Black")
  (CallFunction|ShadowStep))

(event EventBeginPlay
  (|CallParentFunction)
  (CallFunction|ShadowStep))

(fn ConstructionScript
  (|CallParentFunction))