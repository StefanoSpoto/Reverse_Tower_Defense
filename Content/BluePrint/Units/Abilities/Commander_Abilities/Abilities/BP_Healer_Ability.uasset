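; Healer commander ability that restores health to units through an active and a passive effect.
; The active effect heals every unit in the game mode's SpawnedUnits list.
; After a cooldown delay, the passive effect runs a sphere overlap around itself and heals the units found, excluding its parent actor.
; The passive radius is drawn as a brief debug sphere on each pulse.
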(event EventActiveAbility
  (for _array_element (Variables|/Game/BluePrint/Player/GM_LevelGameMode.GM_LevelGameMode_C|GetspawnedUnits (CallFunction|GetGMLevelGameMode))
    (Default|Heal _array_element (Variables|Active|GetactiveHealAmount))))

(event EventPassiveAbility
  (Utilities|FlowControl|Delay (Variables|Passive|GetpassiveCooldown))
  (Rendering|Debug|DrawDebugSphere (Transformation|GetActorLocation) (Variables|Passive|GetpassiveRadius) 12 "(R=0.000000,G=1.000000,B=1.000000,A=1.000000)" 0.2 1.0)
  (bind (_outactors _returnvalue) (Collision|SphereOverlapActors (Transformation|GetActorLocation) (Variables|Passive|GetpassiveRadius) (Utilities|Array|MakeArray "ObjectTypeQuery7") 0))
  (if _returnvalue
    (for _array_element _outactors
      (bind _asbp_unit (Utilities|Casting|CastToBP_Unit _array_element))
      (if (!= _asbp_unit (Actor|GetParentActor))
        (Default|Heal _asbp_unit (Variables|Passive|GetpassiveHealAmount))))))

(fn ConstructionScript
  (|CallParentFunction))