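; BP_Troop is a unit Blueprint for troops whose special ability is supplied by its DA_Troop data asset.
; SetStats passes the data and starting and next path blocks to the parent, then sets the ChildActor component's class to the data's Ability.
; The spawned BP_Troop_Ability receives a reference back to the troop, keeping ability logic in a separate actor.
; The event graph and construction script add no logic of their own.
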(event EventBeginPlay
  (|CallParentFunction) ; This node is disabled and will not be called.\nDrag off pins to build functionality.
)

(event Collision|EventActorBeginOverlap
  (params (OtherActor :type Actor%20Object%20Reference)))

(event EventTick
  (params (DeltaSeconds :type Float%20%28single-precision%29)))

(fn ConstructionScript
  (|CallParentFunction))

(fn SetStats
  (params (data :type DA%20Unit%20Object%20Reference) (startingPathBlock :type BP%20Path%20Block%20Object%20Reference) (nextPathBlock :type BP%20Path%20Block%20Object%20Reference))
  (|CallParentFunction data startingPathBlock nextPathBlock)
  (bind _asda_troop (Utilities|Casting|CastToDA_Troop data))
  (ChildActorComponent|SetChildActorClass (Variables|Default|GetChildActor) (Variables|/Game/BluePrint/Units/DataAssets/Troops/DA_Troop.DA_Troop_C|Getability _asda_troop))
  (bind _asbp_troop_ability (Utilities|Casting|CastToBP_Troop_Ability (Variables|/Script/Engine.ChildActorComponent|GetChildActor (Variables|Default|GetChildActor))))
  (Variables|/Game/BluePrint/Units/Troop_Abilities/BP_Troop_Ability.BP_Troop_Ability_C|SetTroop _asbp_troop_ability self))