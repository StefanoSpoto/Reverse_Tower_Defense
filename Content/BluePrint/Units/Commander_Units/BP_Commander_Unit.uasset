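; BP_Commander_Unit is the commander unit Blueprint, extending a parent unit with a data-driven ability.
; SetStats runs the parent setup with the path blocks, casts the data asset to DA_Commander and constructs the Ability object from its AbilityClass.
; ActivateActiveAbility forwards UnitsSpawned to that object, so ability logic lives outside the unit.
; ActivatePassiveAbility is an empty stub.
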(event Custom|ActivateActiveAbility
  (params (units%20spawned :type Array%20of%20BP%20Unit%20Object%20References))
  (Default|ActiveAbility (Variables|Default|GetAbility) units%20spawned))

(event Custom|ActivatePassiveAbility)

(event EventBeginPlay
  (|CallParentFunction) ; This node is disabled and will not be called.\nDrag off pins to build functionality.
)

(event Collision|EventActorBeginOverlap
  (params (OtherActor :type Actor%20Object%20Reference)))

(event EventTick
  (params (DeltaSeconds :type Float%20%28single-precision%29)))

(fn ConstructionScript
  (|CallParentFunction))

(fn SetStats
  (params (data :type DA%20Unit%20Object%20Reference) (startingPathBlock :type BP%20Path%20Block%20Object%20Reference) (nextPathBlock :type BP%20Path%20Block%20Object%20Reference))
  (|CallParentFunction data startingPathBlock nextPathBlock)
  (bind _asda_commander (Utilities|Casting|CastToDA_Commander data))
  (bind _returnvalue (Game|ConstructObjectfromClass (Variables|/Game/BluePrint/Units/DataAssets/Commanders/DA_Commander.DA_Commander_C|GetabilityClass _asda_commander)))
  (Variables|Default|SetAbility _returnvalue))