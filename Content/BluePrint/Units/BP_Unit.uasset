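; Base unit actor for a reverse tower defense game, walking linked path blocks via a timeline whose play rate follows its speed.
; SetStats loads data-asset stats and applies gem modifiers and child-actor abilities.
; It handles healing, damage multipliers and recursive damage over time, dropping carried gold on death and notifying the game mode.
; Overlapping units trigger a randomized sideways shift of mesh and health bar, timed by their speed difference.
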(event OnComponentBeginOverlap(UnitToUnitCollision)
  (params (OverlappedComponent :type Primitive%20Component%20Object%20Reference) (OtherActor :type Actor%20Object%20Reference) (OtherComp :type Primitive%20Component%20Object%20Reference) (OtherBodyIndex :type Integer) (bFromSweep :type Boolean) (SweepResult :type Hit%20Result%20Structure%20%28by%20ref%29))
  (bind _speed (Variables|Unit|Getspeed))
  ;[1 1 1] Check for unit collision
  (bind _asbp_unit (Utilities|Casting|CastToBP_Unit OtherActor))
  (if (>= (Variables|BP_Unit_C|Getspeed _asbp_unit) _speed)
    (Variables|Shift|SetcollisionUnit self)
    (else
      (Variables|Shift|SetcollisionUnit _asbp_unit)))
  (if (not (Variables|BP_Unit_C|GetisAlreadyShifting (Variables|Shift|GetcollisionUnit)))
    (Movement|SetUpShift (Variables|Shift|GetcollisionUnit) (Variables|BP_Unit_C|Getspeed _asbp_unit) _speed)
    (CallFunction|SetHealthBarOpacity (Variables|Shift|GetcollisionUnit) false)))

(event Custom|Change%20Custom%20Time%20Dilation
  (params (newTimeDilation :type Float%20%28double-precision%29))
  (Variables|Default|SetCustomTimeDilation newTimeDilation))

(event Custom|KillUnit
  (params (killed :type Boolean))
  (bind _returnvalue (Transformation|GetActorLocation))
  ;[1 1 1] Kill Unit
  (if killed
    (Default|CallOnRemoveUnitfromTurretTargets (CallFunction|GetGMLevelGameMode) self)
    (Utilities|Casting|CastToDA_Commander (Variables|Unit|GetData)
      (:then
        (Default|CallOnCommanderDied (CallFunction|GetGMLevelGameMode)))
      (:CastFailed
        _))
    (if (> (Variables|Unit|Getgold) 0)
      ;[0.1939 1 0.2324] Spawn Collected Coins
      (if (== (Variables|Unit|Getgold) 1)
        (Game|SpawnActorfromClass "/Game/BluePrint/Coins/BP_Coin.BP_Coin_C" (Math|Transform|MakeTransform _returnvalue "0, 0, 0" "1.000000,1.000000,1.000000") "Undefined" "MultiplyWithRoot" 0 0)
        (Actor|DestroyActor)
        (else
          (bind _returnvalue_2 (Game|SpawnActorfromClass "/Game/BluePrint/Coins/BP_CoinBag.BP_CoinBag_C" (Math|Transform|MakeTransform _returnvalue "0, 0, 0" "1.000000,1.000000,1.000000") "Undefined" "MultiplyWithRoot" 0 0))
          (Default|SetCoinsAmount _returnvalue_2 (Variables|Unit|Getgold))
          (Actor|DestroyActor)))
      (else
        (Actor|DestroyActor)))))

(event Custom|SetHealthBarOpacity
  (params (isReturningOpaque :type Boolean))
  ;[0.1823 1 0.9716] Set health bar opacity when unit shifting to side
  (if isReturningOpaque
    (bind _alpha (Timeline|Timeline_HealthBarOpacity Reverse)
      (:Update
        (Default|SetOpacity (Variables|Unit|GethealthBarWidget) _alpha)))
    (else
      (Timeline|Timeline_HealthBarOpacity PlayFromStart))))

(event Custom|MoveToNextPathBlock
  ;[1 0.7863 0.3424] Move to next path block
  (if (Variables|Movement|GetcanMove)
    (if (Variables|/Game/BluePrint/Path/BP_PathBlock.BP_PathBlock_C|GetisSwitching (Variables|Movement|GetpreviousPath))
      (Variables|Movement|SetpreviousPathRotation (Variables|/Game/BluePrint/Path/BP_PathBlock.BP_PathBlock_C|GetoldRotation (Variables|Movement|GetpreviousPath)))
      (bind _locationalpha (Timeline|Timeline_UnitMovement PlayFromStart)
        (:Update
          (if (Variables|Movement|GetcanMove)
            (Transformation|SetActorLocationAndRotation (Math|Vector|Lerp(Vector) (.location (Default|GetUnitPathTransform (Variables|Movement|GetpreviousPath))) (.location (Default|GetUnitPathTransform (Variables|Movement|GetnextPath))) _locationalpha) (Math|Rotator|Lerp(Rotator) (Transformation|GetActorRotation) (Variables|Movement|GetpreviousPathRotation) _locationalpha true))))
        (:Finished
          (Variables|Movement|SetpreviousPath (Variables|Movement|GetnextPath))
          (bind _output_get (Variables|Movement|SetnextPath (Variables|/Game/BluePrint/Path/BP_PathBlock.BP_PathBlock_C|GetnextPathBlock (Variables|Movement|GetpreviousPath))))
          (Utilities|IsValid _output_get
            (:Is%20Valid
              (CallFunction|MovetoNextPathBlock)))))
      (else
        (Variables|Movement|SetpreviousPathRotation (.rotation (Default|GetUnitPathTransform (Variables|Movement|GetpreviousPath))))
        (Timeline|Timeline_UnitMovement PlayFromStart)))))

(event Custom|StartShiftUnit
  (params (Starting%20Shift%20Location :type Vector) (Destination%20Shift%20Location :type Vector))
  (bind _skeletalmesh (Variables|Default|GetSkeletalMesh))
  (bind _healthbar (Variables|Default|GetHealthbar))
  (bind _skeletalmesh_2 (Variables|Default|GetSkeletalMesh))
  (bind _healthbar_2 (Variables|Default|GetHealthbar))
  (bind _relativelocation (Variables|/Script/Engine.SceneComponent|GetRelativeLocation _skeletalmesh))
  (bind _relativelocation_2 (Variables|/Script/Engine.SceneComponent|GetRelativeLocation _healthbar))
  (bind _relativelocation_3 (Variables|/Script/Engine.SceneComponent|GetRelativeLocation _skeletalmesh_2))
  (bind _relativelocation_4 (Variables|/Script/Engine.SceneComponent|GetRelativeLocation _healthbar_2))
  ;[0.5345 0.6157 1] Shift to side
  (bind _alpha (Timeline|Timeline_StartUnitShifting PlayFromStart)
    (:Update
      (Transformation|SetRelativeLocation (Variables|Default|GetSkeletalMesh) (Math|Vector|MakeVector (.x _relativelocation) (Math|Float|Lerp (.y Starting%20Shift%20Location) (.y Destination%20Shift%20Location) _alpha) (.z _relativelocation)) false false)
      (Transformation|SetRelativeLocation (Variables|Default|GetHealthbar) (Math|Vector|MakeVector (.x _relativelocation_2) (Math|Float|Lerp (.y Starting%20Shift%20Location) (.y Destination%20Shift%20Location) _alpha) (.z _relativelocation_2)) false false))
    (:Finished
      (Utilities|FlowControl|Delay (Variables|Shift|GetshiftDuration))
      (CallFunction|SetHealthBarOpacity true)
      (bind _alpha_2 (Timeline|Timeline_ReturnUnitShifting PlayFromStart)
        (:Update
          (Transformation|SetRelativeLocation (Variables|Default|GetSkeletalMesh) (Math|Vector|MakeVector (.x _relativelocation_3) (Math|Float|Lerp (.y Destination%20Shift%20Location) (.y (Variables|/Script/Engine.SceneComponent|GetRelativeLocation (Variables|Default|GetShiftReturnPoint))) _alpha_2) (.z _relativelocation_3)) false false)
          (Transformation|SetRelativeLocation (Variables|Default|GetHealthbar) (Math|Vector|MakeVector (.x _relativelocation_4) (Math|Float|Lerp (.y Destination%20Shift%20Location) (.y (Variables|/Script/Engine.SceneComponent|GetRelativeLocation (Variables|Default|GetShiftReturnPoint))) _alpha_2) (.z _relativelocation_4)) false false))
        (:Finished
          (Variables|Shift|SetisAlreadyShifting false))))))

(event Custom|Full%20DOT
  (params (damage :type Float%20%28double-precision%29) (intervalDuration :type Float%20%28single-precision%29) (Duration :type Float%20%28single-precision%29))
  ;[1 1 1] Damage Over Time
  (if (not (Variables|DOT|GetisDamagingOverTime))
    (Variables|DOT|SetisDamagingOverTime true)
    (CallFunction|DOTTick damage intervalDuration)
    (Utilities|FlowControl|Delay Duration)
    (Variables|DOT|SetcanDOT false)
    (Variables|DOT|SetisDamagingOverTime false)))

(event Custom|DOT%20Tick
  (params (damage :type Float%20%28double-precision%29) (intervalDuration :type Float%20%28single-precision%29))
  ;[1 1 1] Damage Over Time
  (if (Variables|DOT|GetcanDOT)
    (Utilities|FlowControl|Delay intervalDuration)
    (bind _iskilled (Stats|TakeDamage damage))
    (CallFunction|KillUnit _iskilled)
    (CallFunction|DOTTick damage intervalDuration)))

(event Custom|Set%20Speed%20For%20Duration
  (params (speed :type Float%20%28single-precision%29) (Duration :type Float%20%28single-precision%29))
  (Stats|SetSpeed speed)
  (Utilities|FlowControl|Delay Duration)
  (Stats|SetSpeed (Variables|Unit|Getspeed)))

(event Custom|Set%20Damage%20Multiplier%20For%20Duration
  (params (New%20Damage%20Multiplier :type Float%20%28double-precision%29) (Duration :type Float%20%28single-precision%29))
  (Stats|SetDamageMultiplier New%20Damage%20Multiplier)
  (Utilities|FlowControl|Delay Duration)
  (Stats|SetDamageMultiplier (Variables|Unit|GetpreviousDamageMultiplier)))

(event EventDestroyed
  (Default|CallOnUnitDied (CallFunction|GetGMLevelGameMode)))

(event EventBeginPlay
  (EventDispatchers|BindEventtoOnChangeTimeDilation (CallFunction|GetGMLevelGameMode) (delegate Custom|Change%20Custom%20Time%20Dilation))
  (bind _asw_unit_health_bar (Utilities|Casting|CastToW_UnitHealthBar (UserInterface|GetWidget (Variables|Default|GetHealthbar))))
  (Variables|Unit|SethealthBarWidget _asw_unit_health_bar))

(fn ConstructionScript)

(fn SetStats
  (params (Unit%20Object :type BP%20Unit%20Object%20Object%20Reference) (startingPathBlock :type BP%20Path%20Block%20Object%20Reference) (nextPathBlock :type BP%20Path%20Block%20Object%20Reference) (Custom%20Time%20Dilation :type Float%20%28single-precision%29))
  (Variables|Default|SetCustomTimeDilation Custom%20Time%20Dilation)
  (bind _output_get (Variables|Unit|SetUnit%20Object Unit%20Object))
  (Variables|Movement|SetpreviousPath startingPathBlock)
  (Variables|Movement|SetnextPath nextPathBlock)
  (bind _output_get_2 (Variables|Unit|SetData (Variables|/Game/BluePrint/Units/BP_UnitObject.BP_UnitObject_C|GetUnit%20Data _output_get)))
  (bind _output_get_3 (Variables|Unit|SetmaxHealth (Variables|/Game/BluePrint/Units/DataAssets/DA_Unit.DA_Unit_C|Gethealth _output_get_2)))
  (Variables|Unit|SetcurrentHealth _output_get_3)
  (Variables|Unit|Setspeed (Variables|/Game/BluePrint/Units/DataAssets/DA_Unit.DA_Unit_C|Getspeed _output_get_2))
  (Variables|Unit|Setpower (Variables|/Game/BluePrint/Units/DataAssets/DA_Unit.DA_Unit_C|Getpower _output_get_2))
  (Variables|Unit|SetspawnTime 0.0)
  (Gems|ApplyGems)
  (Rendering|Material|SetMaterial (Variables|Default|GetSkeletalMesh) 0 (Variables|/Game/BluePrint/Units/DataAssets/DA_Unit.DA_Unit_C|Getmaterial (Variables|Unit|GetData)))
  (Stats|SetSpeed (Variables|Unit|Getspeed))
  (Default|SetHealthUI (Variables|Unit|GethealthBarWidget) (Variables|Unit|GetcurrentHealth) (Variables|Unit|GetmaxHealth)))

(fn DeactivateUnit
  (Rendering|SetVisibility (Variables|Default|GetSkeletalMesh) false true)
  (Variables|/Script/Engine.PrimitiveComponent|SetbGenerateOverlapEvents (Variables|Default|GetUnitToUnitCollision) false)
  (Variables|/Script/Engine.PrimitiveComponent|SetbGenerateOverlapEvents (Variables|Default|GetSphere) false)
  (Variables|Movement|SetcanMove false)
  (Variables|Unit|SetcanBeAggro false)
  (Rendering|SetVisibility (Variables|Default|GetHealthbar) false false))

(fn ActivateUnit
  (Rendering|SetVisibility (Variables|Default|GetSkeletalMesh) true true)
  (Variables|/Script/Engine.PrimitiveComponent|SetbGenerateOverlapEvents (Variables|Default|GetUnitToUnitCollision) true)
  (Variables|/Script/Engine.PrimitiveComponent|SetbGenerateOverlapEvents (Variables|Default|GetSphere) true)
  (Variables|Movement|SetcanMove true)
  (Variables|Unit|SetcanBeAggro true)
  (Rendering|SetVisibility (Variables|Default|GetHealthbar) true false)
  (CallFunction|MovetoNextPathBlock))

(fn TakeDamage
  (params (Damage :type Float%20%28double-precision%29))
  (bind _output_get (Variables|Unit|SetcurrentHealth (- (Variables|Unit|GetcurrentHealth) (* (Variables|Unit|GetcurrentDamageMultiplier) Damage))))
  (Default|SetHealthUI (Variables|Unit|GethealthBarWidget) _output_get (Variables|Unit|GetmaxHealth))
  (if (<= (Variables|Unit|GetcurrentHealth) 0.0)
    (Variables|Unit|SetcurrentHealth 0.0)
    (Default|RemoveSpawnedUnit (CallFunction|GetGMLevelGameMode) self)
    (LocalVariables|Setkilled true)
    (else
      (LocalVariables|Setkilled false)))
  (return (LocalVariables|Getkilled) self))

(fn Heal
  (params (healAmount :type Float%20%28double-precision%29))
  (bind _maxhealth (Variables|Unit|GetmaxHealth))
  (bind _output_get (Variables|Unit|SetcurrentHealth (+ (Variables|Unit|GetcurrentHealth) healAmount)))
  (if (> _output_get (Variables|Unit|GetmaxHealth))
    (bind _output_get_2 (Variables|Unit|SetcurrentHealth _maxhealth)))
  (Default|SetHealthUI (Variables|Unit|GethealthBarWidget) _output_get_2 _maxhealth))

(fn SetSpeed
  (params (speed :type Float%20%28single-precision%29))
  (Components|Timeline|SetPlayRate (Variables|Default|GetTimeline_UnitMovement) speed)
  (Components|Timeline|SetPlayRate (Variables|Default|GetSkeletalMesh) speed))

(fn SetUpShift
  (params (speed_A :type Float%20%28double-precision%29) (speed_B :type Float%20%28double-precision%29))
  (bind _shiftpoint_l (Variables|Default|GetShiftPoint%20L))
  (bind _shiftpoint_r (Variables|Default|GetShiftPoint%20R))
  (bind _relativelocation (Variables|/Script/Engine.SceneComponent|GetRelativeLocation _shiftpoint_r))
  (bind _relativelocation_2 (Variables|/Script/Engine.SceneComponent|GetRelativeLocation _shiftpoint_l))
  (Variables|Shift|SetisAlreadyShifting true)
  (Movement|SetShiftDuration speed_A speed_B)
  (if (Math|Random|RandomBool)
    (CallFunction|StartShiftUnit (Variables|/Script/Engine.SceneComponent|GetRelativeLocation (Variables|Default|GetSkeletalMesh)) _relativelocation_2)
    (CallFunction|StartShiftUnit (Variables|/Script/Engine.SceneComponent|GetRelativeLocation (Variables|Default|GetHealthbar)) _relativelocation_2)
    (else
      (CallFunction|StartShiftUnit (Variables|/Script/Engine.SceneComponent|GetRelativeLocation (Variables|Default|GetSkeletalMesh)) _relativelocation)
      (CallFunction|StartShiftUnit (Variables|/Script/Engine.SceneComponent|GetRelativeLocation (Variables|Default|GetHealthbar)) _relativelocation))))

(fn SetShiftDuration
  (params (speed_A :type Float%20%28double-precision%29) (speed_B :type Float%20%28double-precision%29))
  (Variables|Shift|SetshiftDuration (/ 1.0 (Math|Float|Absolute(Float) (- speed_A speed_B)))))

(fn CollectCoin
  (params (coins :type Integer))
  (Variables|Unit|Setgold (+ coins (Variables|Unit|Getgold))))

(fn ApplyGems
  (for _array_element (Variables|/Game/BluePrint/Units/BP_UnitObject.BP_UnitObject_C|GetgemsInPossession (Variables|Unit|GetUnit%20Object))
    (for _array_element_2 (Variables|/Game/BluePrint/Gems/Data_Assets/DA_Gem.DA_Gem_C|GetstatModifiers _array_element)
      (Gems|ApplyStatModifier _array_element_2))
    (for _array_element_3 (Variables|/Game/BluePrint/Gems/Data_Assets/DA_Gem.DA_Gem_C|GetspacialAbilities _array_element)
      (bind _returnvalue (AddComponent|AddChildActorComponent false))
      (ChildActorComponent|SetChildActorClass _returnvalue _array_element_3)
      (bind _asbp_gem_ability (Utilities|Casting|CastToBP_Gem_Ability (Variables|/Script/Engine.ChildActorComponent|GetChildActor _returnvalue)))
      (Variables|/Game/BluePrint/Gems/Gem_Abilities/BP_Gem_Ability.BP_Gem_Ability_C|SetUnit _asbp_gem_ability self))))

(fn ApplyStatModifier
  (params (Modifier :type BS%20Unit%20Stat%20Modifier%20Structure))
  (LocalVariables|SetStatType (.modifiablestat Modifier))
  (LocalVariables|SetincrementType (.increaseamounttype Modifier))
  (LocalVariables|SetAmount (.amount Modifier))
  (switch Utilities|FlowControl|Switch|SwitchonE_UnitStat_Type (LocalVariables|GetStatType)
    (:NewEnumerator0
      (Gems|IncrementStat (Variables|Unit|GetmaxHealth) (LocalVariables|GetincrementType) (LocalVariables|GetAmount))
      (Gems|IncrementStat (Variables|Unit|GetcurrentHealth) (LocalVariables|GetincrementType) (LocalVariables|GetAmount)))
    (:NewEnumerator1
      (Gems|IncrementStat (Variables|Unit|Getspeed) (LocalVariables|GetincrementType) (LocalVariables|GetAmount)))
    (:NewEnumerator2
      (Gems|IncrementStat (Variables|Unit|Getpower) (LocalVariables|GetincrementType) (LocalVariables|GetAmount)))
    (:NewEnumerator3
      (Gems|IncrementStat (Math|Conversions|ToFloat(Integer) (Variables|Unit|GetendLevelBonusGold)) "NewEnumerator0" (LocalVariables|GetAmount)))))

(fn IncrementStat
  (params (stat :type Float%20%28double-precision%29%20%28by%20ref%29) (incrementType :type E_UnitStat_IncrementAmountType%20Enum :default "NewEnumerator0") (incrementAmount :type Float%20%28double-precision%29))
  (switch Utilities|FlowControl|Switch|SwitchonE_UnitStat_IncrementAmountType incrementType
    (:NewEnumerator0
      (|SetBy-RefVar stat (+ stat incrementAmount)))
    (:NewEnumerator1
      (|SetBy-RefVar stat (* stat incrementAmount)))))

(fn SaveGold
  (bind _asgi_reverse_td (CallFunction|GetGIReverseTD))
  (Default|GainGold _asgi_reverse_td (Variables|Unit|Getgold))
  (Default|GainGold _asgi_reverse_td (Variables|Unit|GetendLevelBonusGold)))

(fn StartDamageOverTime
  (params (damage :type Float%20%28double-precision%29) (intervalDuration :type Float%20%28double-precision%29) (duration :type Float%20%28double-precision%29))
  (Variables|DOT|SetcanDOT true)
  (CallFunction|FullDOT damage intervalDuration duration))

(fn SetDamageMultiplier
  (params (New%20Damage%20Multiplier :type Float%20%28double-precision%29))
  (Variables|Unit|SetpreviousDamageMultiplier (Variables|Unit|GetcurrentDamageMultiplier))
  (Variables|Unit|SetcurrentDamageMultiplier New%20Damage%20Multiplier))

(fn IsDead
  (return (<= (Variables|Unit|GetcurrentHealth) 0.0)))