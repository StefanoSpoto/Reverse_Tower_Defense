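; BP_UnitObject holds a unit's runtime stats and socketed gems, initialized from its UnitData asset, with an extra ability cooldown for commanders.
; AddGem checks socket cost and troop/commander targeting, then spends sockets and applies the gem's stat modifiers.
; Modifiers change stats in place by reference, adding fixed amounts or multiplying percentages.
; Removal refunds sockets and applies inverse operations rather than recomputing from base values.
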(fn Init
  (Variables|Gems|SetaviableSockets (Variables|/Game/BluePrint/Units/DataAssets/DA_Unit.DA_Unit_C|GetavailableGemSockets (Variables|Data|GetUnit%20Data)))
  (Variables|Data|SetHealth (Variables|/Game/BluePrint/Units/DataAssets/DA_Unit.DA_Unit_C|Gethealth (Variables|Data|GetUnit%20Data)))
  (Variables|Data|SetSpeed (Variables|/Game/BluePrint/Units/DataAssets/DA_Unit.DA_Unit_C|Getspeed (Variables|Data|GetUnit%20Data)))
  (Variables|Data|SetPower (Variables|/Game/BluePrint/Units/DataAssets/DA_Unit.DA_Unit_C|Getpower (Variables|Data|GetUnit%20Data)))
  (bind _asda_commander (Utilities|Casting|CastToDA_Commander (Variables|Data|GetUnit%20Data)))
  (Variables|Data|SetCommander%20Active%20Ability%20Cooldown (Variables|/Game/BluePrint/Units/DataAssets/Commanders/DA_Commander.DA_Commander_C|GetabilityCooldown _asda_commander)))

(fn AddGem
  (params (gem :type DA%20Gem%20Object%20Reference))
  (if (Gems|CanAddGem gem)
    (Variables|Gems|SetaviableSockets (- (Variables|Gems|GetaviableSockets) (Variables|/Game/BluePrint/Gems/Data_Assets/DA_Gem.DA_Gem_C|GetsocketCost gem)))
    (Utilities|Array|Add (Variables|Gems|GetgemsInPossession) gem)
    (for _array_element (Variables|/Game/BluePrint/Gems/Data_Assets/DA_Gem.DA_Gem_C|GetstatModifiers gem)
      (Stats|ApplyStatModifier _array_element false))
    (return true)
    (else
      (return false))))

(fn CanAddGem
  (params (gem :type DA%20Gem%20Object%20Reference))
  (bind _aviablesockets (Variables|Gems|GetaviableSockets))
  (bind _unit_data (Variables|Data|GetUnit%20Data))
  (bind _socketcost (Variables|/Game/BluePrint/Gems/Data_Assets/DA_Gem.DA_Gem_C|GetsocketCost gem))
  (bind _returnvalue (<= _socketcost _aviablesockets))
  (switch Utilities|FlowControl|Switch|SwitchonE_GemTarget (Variables|/Game/BluePrint/Gems/Data_Assets/DA_Gem.DA_Gem_C|Gettarget gem)
    (:NewEnumerator2
      (return _returnvalue))
    (:NewEnumerator0
      (Utilities|Casting|CastToDA_Troop _unit_data
        (:then
          (return _returnvalue))
        (:CastFailed
          (return false))))
    (:NewEnumerator1
      (Utilities|Casting|CastToDA_Commander _unit_data
        (:then
          (return _returnvalue))
        (:CastFailed
          (return false))))))

(fn RemoveGem
  (params (indexToRemove :type Integer))
  (for _array_element (Variables|/Game/BluePrint/Gems/Data_Assets/DA_Gem.DA_Gem_C|GetstatModifiers (Utilities|Array|Get(acopy) (Variables|Gems|GetgemsInPossession) indexToRemove))
    (Stats|ApplyStatModifier _array_element true))
  (Variables|Gems|SetaviableSockets (+ (Variables|Gems|GetaviableSockets) (Variables|/Game/BluePrint/Gems/Data_Assets/DA_Gem.DA_Gem_C|GetsocketCost (Utilities|Array|Get(acopy) (Variables|Gems|GetgemsInPossession) indexToRemove))))
  (Utilities|Array|RemoveIndex (Variables|Gems|GetgemsInPossession) indexToRemove))

(fn SetGemSockets
  (Variables|Gems|SetaviableSockets (Variables|/Game/BluePrint/Units/DataAssets/DA_Unit.DA_Unit_C|GetavailableGemSockets (Variables|Data|GetUnit%20Data))))

(fn HasGems
  (return (Utilities|Array|IsNotEmpty (Variables|Gems|GetgemsInPossession))))

(fn ApplyStatModifier
  (params (Modifier :type BS%20Unit%20Stat%20Modifier%20Structure) (Decrement :type Boolean))
  (LocalVariables|SetStatType (.modifiablestat Modifier))
  (LocalVariables|SetincrementType (.increaseamounttype Modifier))
  (LocalVariables|SetAmount (.amount Modifier))
  (if Decrement
    (switch Utilities|FlowControl|Switch|SwitchonE_UnitStat_Type (LocalVariables|GetStatType)
      (:NewEnumerator0
        (Stats|DecrementStat (Variables|Data|GetHealth) (LocalVariables|GetincrementType) (LocalVariables|GetAmount)))
      (:NewEnumerator1
        (Stats|DecrementStat (Variables|Default|Getspeed) (LocalVariables|GetincrementType) (LocalVariables|GetAmount)))
      (:NewEnumerator2
        (Stats|DecrementStat (Variables|Default|Getpower) (LocalVariables|GetincrementType) (LocalVariables|GetAmount)))
      (:NewEnumerator3
        (Stats|DecrementStat (Variables|Data|GetEnd%20Level%20Gold%20Bonus) (LocalVariables|GetincrementType) (LocalVariables|GetAmount)))
      (:NewEnumerator4
        (Utilities|Casting|CastToDA_Commander (Variables|Data|GetUnit%20Data))
        (Stats|DecrementStat (Variables|Data|GetCommander%20Active%20Ability%20Cooldown) (LocalVariables|GetincrementType) (LocalVariables|GetAmount))))
    (else
      (switch Utilities|FlowControl|Switch|SwitchonE_UnitStat_Type (LocalVariables|GetStatType)
        (:NewEnumerator0
          (Stats|IncrementStat (Variables|Data|GetHealth) (LocalVariables|GetincrementType) (LocalVariables|GetAmount)))
        (:NewEnumerator1
          (Stats|IncrementStat (Variables|Default|Getspeed) (LocalVariables|GetincrementType) (LocalVariables|GetAmount)))
        (:NewEnumerator2
          (Stats|IncrementStat (Variables|Default|Getpower) (LocalVariables|GetincrementType) (LocalVariables|GetAmount)))
        (:NewEnumerator3
          (Stats|IncrementStat (Variables|Data|GetEnd%20Level%20Gold%20Bonus) (LocalVariables|GetincrementType) (LocalVariables|GetAmount)))
        (:NewEnumerator4
          (Utilities|Casting|CastToDA_Commander (Variables|Data|GetUnit%20Data))
          (Stats|IncrementStat (Variables|Data|GetCommander%20Active%20Ability%20Cooldown) (LocalVariables|GetincrementType) (LocalVariables|GetAmount)))))))

(fn IncrementStat
  (params (stat :type Float%20%28double-precision%29%20%28by%20ref%29) (incrementType :type E_UnitStat_IncrementAmountType%20Enum :default "NewEnumerator0") (incrementAmount :type Float%20%28double-precision%29))
  (switch Utilities|FlowControl|Switch|SwitchonE_UnitStat_IncrementAmountType incrementType
    (:NewEnumerator0
      (|SetBy-RefVar stat (+ stat incrementAmount)))
    (:NewEnumerator1
      (|SetBy-RefVar stat (* stat incrementAmount)))))

(fn DecrementStat
  (params (stat :type Float%20%28double-precision%29%20%28by%20ref%29) (incrementType :type E_UnitStat_IncrementAmountType%20Enum :default "NewEnumerator0") (DecrementAmount :type Float%20%28double-precision%29))
  (switch Utilities|FlowControl|Switch|SwitchonE_UnitStat_IncrementAmountType incrementType
    (:NewEnumerator0
      (|SetBy-RefVar stat (- stat DecrementAmount)))
    (:NewEnumerator1
      (|SetBy-RefVar stat (/ stat DecrementAmount)))))

(fn RemoveAllGems
  (bind _output_get (LocalVariables|SetGemsLastIndex (Utilities|Array|LastIndex (Variables|Gems|GetgemsInPossession))))
  (for _index (range 0 _output_get)
    (Gems|RemoveGem)))