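; BP_ShadowGoblinAbility is the Shadow Goblin troop's shadow step ability, periodically making the troop unable to be aggroed.
; Tick drives a latent Delay loop timed by ShadowStepDelay, with no separate timer.
; After the first delay it clears the Troop's CanBeAggro flag if the troop is not already aggroed, then restores it after a second delay.
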(event EventBeginPlay
  (|CallParentFunction))

(event Collision|EventActorBeginOverlap
  (params (OtherActor :type Actor%20Object%20Reference))
  (|CallParentFunction OtherActor) ; This node is disabled and will not be called.\nDrag off pins to build functionality.
)

(event EventTick
  (params (DeltaSeconds :type Float%20%28single-precision%29))
  (|CallParentFunction DeltaSeconds)
  (Utilities|FlowControl|Delay (Variables|Default|GetshadowStepDelay))
  (if (Variables|/Game/BluePrint/Units/BP_Unit.BP_Unit_C|GetisAggroed (Variables|Default|GetTroop))
    _
    (else
      (Variables|/Game/BluePrint/Units/BP_Unit.BP_Unit_C|SetcanBeAggro (Variables|Default|GetTroop) false)))
  (Utilities|FlowControl|Delay (Variables|Default|GetshadowStepDelay))
  (Variables|/Game/BluePrint/Units/BP_Unit.BP_Unit_C|SetcanBeAggro (Variables|Default|GetTroop) true))

(fn ConstructionScript
  (|CallParentFunction))