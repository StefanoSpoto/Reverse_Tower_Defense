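; BP_TamerGoblinAbility is a troop ability that leaves a Tamer unit behind when the ability actor is destroyed.
; On Destroyed, it spawns a BP_Unit at its own location and rotation and initializes it with DAT_Tamer stats.
; The new unit receives the Troop's previous and next path blocks, then moves toward the next one to continue along the route.
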(event EventBeginPlay
  (|CallParentFunction) ; This node is disabled and will not be called.\nDrag off pins to build functionality.
)

(event Collision|EventActorBeginOverlap
  (params (OtherActor :type Actor%20Object%20Reference))
  (|CallParentFunction OtherActor) ; This node is disabled and will not be called.\nDrag off pins to build functionality.
)

(event EventTick
  (params (DeltaSeconds :type Float%20%28single-precision%29))
  (|CallParentFunction DeltaSeconds) ; This node is disabled and will not be called.\nDrag off pins to build functionality.
)

(event EventDestroyed
  (bind _troop (Variables|Default|GetTroop))
  (bind _returnvalue (Game|SpawnActorfromClass "/Game/BluePrint/Units/BP_Unit.BP_Unit_C" (Math|Transform|MakeTransform (Transformation|GetActorLocation) (Transformation|GetActorRotation) "1.000000,1.000000,1.000000") "Undefined" "MultiplyWithRoot" 0 0))
  (Default|SetStats _returnvalue "/Game/BluePrint/Units/DataAssets/Troops/DAT_Tamer.DAT_Tamer" (Variables|/Game/BluePrint/Units/BP_Unit.BP_Unit_C|GetpreviousPath _troop) (Variables|/Game/BluePrint/Units/BP_Unit.BP_Unit_C|GetnextPath _troop))
  (Default|MovetoNextPathBlock _returnvalue))

(fn ConstructionScript
  (|CallParentFunction))