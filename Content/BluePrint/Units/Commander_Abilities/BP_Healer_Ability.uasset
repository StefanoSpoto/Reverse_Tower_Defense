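; BP_Healer_Ability is a healer commander ability with an active and a passive heal.
; The active heals every unit in the level game mode's SpawnedUnits list by a set amount.
; The passive waits out a cooldown, then sphere-overlaps around its location and heals each BP_Unit found except its parent actor.
; The passive does not re-trigger itself within this graph.
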(event EventActiveAbility
  (for _array_element (Variables|/Game/BluePrint/Player/GM_LevelGameMode.GM_LevelGameMode_C|GetspawnedUnits (CallFunction|GetGMLevelGameMode))
    (Default|Heal _array_element (Variables|Active|GetactiveHealAmount))))

(event EventPassiveAbility
  (Utilities|FlowControl|Delay (Variables|Passive|GetpassiveCooldown))
  (bind (_outactors _returnvalue) (Collision|SphereOverlapActors (Transformation|GetActorLocation) (Variables|Passive|GetpassiveRadius) (Utilities|Array|MakeArray "ObjectTypeQuery7") 0))
  (if _returnvalue
    (for _array_element _outactors
      (bind _asbp_unit (Utilities|Casting|CastToBP_Unit _array_element))
      (if (!= _asbp_unit (Actor|GetParentActor))
        (Default|Heal _asbp_unit (Variables|Passive|GetpassiveHealAmount))))))

(fn ConstructionScript
  (|CallParentFunction))