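; Bard commander ability that combines a timed speed boost with a passive health aura for units.
; ActiveAbility raises the speed of every unit in the game mode's SpawnedUnits, then subtracts it after a delay from whatever units are listed then.
; The sphere adds max and current health to overlapping BP_Units and subtracts it on exit, calling Heal in both cases.
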(event OnComponentBeginOverlap(Sphere)
  (params (OverlappedComponent :type Primitive%20Component%20Object%20Reference) (OtherActor :type Actor%20Object%20Reference) (OtherComp :type Primitive%20Component%20Object%20Reference) (OtherBodyIndex :type Integer) (bFromSweep :type Boolean) (SweepResult :type Hit%20Result%20Structure%20%28by%20ref%29))
  (bind _asbp_unit (Utilities|Casting|CastToBP_Unit OtherActor))
  (Variables|/Game/BluePrint/Units/BP_Unit.BP_Unit_C|SetmaxHealth _asbp_unit (+ (Variables|/Game/BluePrint/Units/BP_Unit.BP_Unit_C|GetmaxHealth _asbp_unit) (Variables|Passive|GethealthIncrease)))
  (Variables|/Game/BluePrint/Units/BP_Unit.BP_Unit_C|SetcurrentHealth _asbp_unit (+ (Variables|/Game/BluePrint/Units/BP_Unit.BP_Unit_C|GetcurrentHealth _asbp_unit) (Variables|Passive|GethealthIncrease)))
  (Default|Heal _asbp_unit (Variables|Passive|GethealthIncrease)))

(event OnComponentEndOverlap(Sphere)
  (params (OverlappedComponent :type Primitive%20Component%20Object%20Reference) (OtherActor :type Actor%20Object%20Reference) (OtherComp :type Primitive%20Component%20Object%20Reference) (OtherBodyIndex :type Integer))
  (bind _asbp_unit (Utilities|Casting|CastToBP_Unit OtherActor))
  (Variables|/Game/BluePrint/Units/BP_Unit.BP_Unit_C|SetmaxHealth _asbp_unit (- (Variables|/Game/BluePrint/Units/BP_Unit.BP_Unit_C|GetmaxHealth _asbp_unit) (Variables|Passive|GethealthIncrease)))
  (Variables|/Game/BluePrint/Units/BP_Unit.BP_Unit_C|SetcurrentHealth _asbp_unit (- (Variables|/Game/BluePrint/Units/BP_Unit.BP_Unit_C|GetcurrentHealth _asbp_unit) (Variables|Passive|GethealthIncrease)))
  (Default|Heal _asbp_unit (Variables|Passive|GethealthIncrease)))

(event EventActiveAbility
  (for _array_element (Variables|/Game/BluePrint/Player/GM_LevelGameMode.GM_LevelGameMode_C|GetspawnedUnits (CallFunction|GetGMLevelGameMode))
    (bind _output_get (Variables|/Game/BluePrint/Units/BP_Unit.BP_Unit_C|Setspeed _array_element (+ (Variables|/Game/BluePrint/Units/BP_Unit.BP_Unit_C|Getspeed _array_element) (Variables|Active|GetspeedIncrement))))
    (Default|SetSpeed _array_element _output_get))
  (Utilities|FlowControl|Delay (Variables|Active|GetactiveDuration))
  (for _array_element_2 (Variables|/Game/BluePrint/Player/GM_LevelGameMode.GM_LevelGameMode_C|GetspawnedUnits (CallFunction|GetGMLevelGameMode))
    (bind _output_get_2 (Variables|/Game/BluePrint/Units/BP_Unit.BP_Unit_C|Setspeed _array_element_2 (- (Variables|/Game/BluePrint/Units/BP_Unit.BP_Unit_C|Getspeed _array_element_2) (Variables|Active|GetspeedIncrement))))
    (Default|SetSpeed _array_element_2 _output_get_2)))

(fn ConstructionScript
  (|CallParentFunction))