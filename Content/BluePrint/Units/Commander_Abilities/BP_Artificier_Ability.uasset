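; Artificier commander ability Blueprint that hampers nearby BP_Turret actors through a passive aura and an active pulse.
; The passive Sphere, sized from PassiveRadius at construction, lengthens a turret's shot recharge time on overlap and reverts it on exit.
; ActiveAbility sphere-overlaps turrets within ActiveRadius, flashing a debug sphere, and disables their shooting.
; After ActiveDuration it re-enables every turret stored in DeactivatedTurrets, an array it never clears.
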(event OnComponentBeginOverlap(Sphere)
  (params (OverlappedComponent :type Primitive%20Component%20Object%20Reference) (OtherActor :type Actor%20Object%20Reference) (OtherComp :type Primitive%20Component%20Object%20Reference) (OtherBodyIndex :type Integer) (bFromSweep :type Boolean) (SweepResult :type Hit%20Result%20Structure%20%28by%20ref%29))
  (bind _asbp_turret (Utilities|Casting|CastToBP_Turret OtherActor))
  (Variables|/Game/BluePrint/Turrets/BP_Turret.BP_Turret_C|SetshootRechargeTime _asbp_turret (+ (Variables|/Game/BluePrint/Turrets/BP_Turret.BP_Turret_C|GetshootRechargeTime _asbp_turret) (Variables|Passive|GetshootRechargeTimeIncrease))))

(event OnComponentEndOverlap(Sphere)
  (params (OverlappedComponent :type Primitive%20Component%20Object%20Reference) (OtherActor :type Actor%20Object%20Reference) (OtherComp :type Primitive%20Component%20Object%20Reference) (OtherBodyIndex :type Integer))
  (bind _asbp_turret (Utilities|Casting|CastToBP_Turret OtherActor))
  (Variables|/Game/BluePrint/Turrets/BP_Turret.BP_Turret_C|SetshootRechargeTime _asbp_turret (- (Variables|/Game/BluePrint/Turrets/BP_Turret.BP_Turret_C|GetshootRechargeTime _asbp_turret) (Variables|Passive|GetshootRechargeTimeIncrease))))

(event EventActiveAbility
  (Rendering|Debug|DrawDebugSphere (Transformation|GetActorLocation) (Variables|Active|GetactiveRadius) 12 "(R=1.000000,G=0.318225,B=0.000000,A=1.000000)" 0.2 1.0)
  (bind (_outactors _returnvalue) (Collision|SphereOverlapActors (Transformation|GetActorLocation) (Variables|Active|GetactiveRadius) (Utilities|Array|MakeArray "ObjectTypeQuery2") "/Game/BluePrint/Turrets/BP_Turret.BP_Turret_C"))
  (if _returnvalue
    (for _array_element _outactors
      (bind _asbp_turret (Utilities|Casting|CastToBP_Turret _array_element))
      (Utilities|Array|Add (Variables|Active|GetdeactivatedTurrets) _asbp_turret)
      (Variables|/Game/BluePrint/Turrets/BP_Turret.BP_Turret_C|SetcanShoot _asbp_turret false))
    (Utilities|FlowControl|Delay (Variables|Active|GetactiveDuration))
    (for _array_element_2 (Variables|Active|GetdeactivatedTurrets)
      (Variables|/Game/BluePrint/Turrets/BP_Turret.BP_Turret_C|SetcanShoot _array_element_2 true))))

(fn ConstructionScript
  (|CallParentFunction)
  (Components|Sphere|SetSphereRadius (Variables|Default|GetSphere) (Variables|Passive|GetpassiveRadius) true))