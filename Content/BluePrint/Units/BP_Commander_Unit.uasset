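; Commander unit Blueprint that extends a parent unit with an ability chosen by its DA_Commander data asset.
; SetStats runs the parent setup, then sets a child actor component's class to the data asset's AbilityType and caches the spawned BP_Commander_Ability.
; ActivateActiveAbility forwards to that ability.
; Tick calls ActivatePassiveAbility every frame, but that event is empty and the PassiveAbility call is disconnected.
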(event Custom|ActivateActiveAbility
  (Default|ActiveAbility (Variables|Default|GetAbility)))

(event Custom|ActivatePassiveAbility)

(event EventTick
  (params (DeltaSeconds :type Float%20%28single-precision%29))
  (CallFunction|ActivatePassiveAbility))

(fn ConstructionScript
  (|CallParentFunction))

(fn SetStats
  (params (Unit%20Object :type BP%20Unit%20Object%20Object%20Reference) (startingPathBlock :type BP%20Path%20Block%20Object%20Reference) (nextPathBlock :type BP%20Path%20Block%20Object%20Reference) (Custom%20Time%20Dilation :type Float%20%28single-precision%29))
  (bind _childactor (Variables|Default|GetChildActor))
  (|CallParentFunction Unit%20Object startingPathBlock nextPathBlock Custom%20Time%20Dilation)
  (bind _asda_commander (Utilities|Casting|CastToDA_Commander (Variables|/Game/BluePrint/Units/BP_UnitObject.BP_UnitObject_C|GetUnit%20Data Unit%20Object)))
  (ChildActorComponent|SetChildActorClass _childactor (Variables|/Game/BluePrint/Units/DataAssets/Commanders/DA_Commander.DA_Commander_C|GetabilityType _asda_commander))
  (bind _asbp_commander_ability (Utilities|Casting|CastToBP_Commander_Ability (Variables|/Script/Engine.ChildActorComponent|GetChildActor _childactor)))
  (Variables|Default|SetAbility _asbp_commander_ability))