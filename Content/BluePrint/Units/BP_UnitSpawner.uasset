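; BP_UnitSpawner spawns the ordered army as BP_Unit actors at its own transform in a reverse tower defense game.
; It binds to the GIReverseTD start-spawning event, then copies OrderedArmy and enables spawning.
; A flag-gated Tick waits each entry's SpawnTime, spawns a unit and passes it that entry's stats.
; Spawning stops after the last entry, and the index is never reset.
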(event Custom|SpawnStart
  (Variables|Spawn|SetcanSpawn true)
  (Development|PrintString "start!!!")
  (Variables|Default|Setarmy (Variables|/Game/BluePrint/Player/GI_ReverseTD.GI_ReverseTD_C|GetorderedArmy (stale EventBeginPlay _asgi_reverse_td))))

(event EventBeginPlay
  (bind _asgi_reverse_td (CallFunction|GetGIReverseTD))
  (EventDispatchers|BindEventtoOnStartSpawning _asgi_reverse_td (delegate Custom|SpawnStart))
  (Variables|Spawn|SetcanSpawn false))

(event EventTick
  (params (DeltaSeconds :type Float%20%28single-precision%29))
  (bind _army (Variables|Default|Getarmy))
  (bind _index (Variables|Default|Getindex))
  (bind _output (Utilities|Array|Get(acopy) _army _index))
  (if (Variables|Spawn|GetcanSpawn)
    (Variables|Spawn|SetcanSpawn false)
    (Utilities|FlowControl|Delay (Variables|/Game/BluePrint/Units/DataAssets/DA_Unit.DA_Unit_C|GetspawnTime _output))
    (bind _returnvalue (Game|SpawnActorfromClass "/Game/BluePrint/Units/BP_Unit.BP_Unit_C" (Transformation|GetActorTransform) "AlwaysSpawn" "MultiplyWithRoot" 0 0))
    (Default|SetStats _returnvalue _output)
    (bind _result (Math|Integer|IncrementInt (Variables|Default|Getindex))
      (:%20%20
        (if (> _result (Utilities|Array|LastIndex (Variables|Default|Getarmy)))
          (Variables|Spawn|SetcanSpawn false)
          (else
            (Variables|Spawn|SetcanSpawn true)))))))

(fn ConstructionScript)