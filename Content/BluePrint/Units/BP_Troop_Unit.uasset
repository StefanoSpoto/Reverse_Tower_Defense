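; BP_Troop_Unit is a troop unit Blueprint that equips itself with the ability defined in its troop data.
; SetStats extends the parent's setup, casts the unit data to DA_Troop and sets the ChildActor component's class to that data's Ability.
; It then hands the spawned BP_Troop_Ability a reference to itself as its Troop.
; The event graph and construction script add no logic of their own.
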(event EventBeginPlay
  (|CallParentFunction) ; This node is disabled and will not be called.\nDrag off pins to build functionality.
)

(event Collision|EventActorBeginOverlap
  (params (OtherActor :type Actor%20Object%20Reference)))

(event EventTick
  (params (DeltaSeconds :type Float%20%28single-precision%29)))

(fn ConstructionScript
  (|CallParentFunction))

(fn SetStats
  (params (Unit%20Object :type BP%20Unit%20Object%20Object%20Reference) (startingPathBlock :type BP%20Path%20Block%20Object%20Reference) (nextPathBlock :type BP%20Path%20Block%20Object%20Reference) (Custom%20Time%20Dilation :type Float%20%28single-precision%29))
  (|CallParentFunction Unit%20Object startingPathBlock nextPathBlock Custom%20Time%20Dilation)
  (bind _asda_troop (Utilities|Casting|CastToDA_Troop (Variables|/Game/BluePrint/Units/BP_UnitObject.BP_UnitObject_C|GetUnit%20Data Unit%20Object)))
  (ChildActorComponent|SetChildActorClass (Variables|Default|GetChildActor) (Variables|/Game/BluePrint/Units/DataAssets/Troops/DA_Troop.DA_Troop_C|Getability _asda_troop))
  (bind _asbp_troop_ability (Utilities|Casting|CastToBP_Troop_Ability (Variables|/Script/Engine.ChildActorComponent|GetChildActor (Variables|Default|GetChildActor))))
  (Variables|/Game/BluePrint/Units/Abilities/Troop_Abilities/BP_Troop_Ability.BP_Troop_Ability_C|SetTroop _asbp_troop_ability self))