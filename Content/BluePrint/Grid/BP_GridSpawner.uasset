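; Grid spawner actor that builds a Columns by Rows block grid with a predefined path through it.
; On BeginPlay, a 2D grid macro visits each cell and matches it against the Path array, spawning starting path, path or plain grid blocks.
; Path blocks receive their orientation and switch data.
; With Test enabled, the construction script previews the layout using static meshes, tinting starting cells red.
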(event EventBeginPlay
  (Variables|DEBUGGING|SetTest false)
  (if true
    (bind (_current_point _total_points _0_1_phase _poly_center _x_row _y_row) (Utilities|2DGridExecutionMacro (Variables|Grid|Getoffset) (Transformation|GetActorLocation) (Variables|Grid|Getcolumns) (Variables|Grid|Getrows))
      (:Per%20Poly%20Execution
        (Variables|Grid|SethasSpawnedPath false)
        (bind _array_element (Utilities|Array|ForEachLoopwithBreak (Variables|Grid|Getpath) :!label _label)
          (:LoopBody
            (if (and (== (.x _array_element) _x_row) (== (.y _array_element) _y_row))
              (if (.startingcell _array_element)
                (bind _returnvalue (Game|SpawnActorfromClass "/Game/BluePrint/Grid/Path/BP_StartingPathBlock.BP_StartingPathBlock_C" (Math|Conversions|ToTransform(Vector) _poly_center) "AlwaysSpawn" "MultiplyWithRoot" 0 0))
                (Default|SetPathBlock _returnvalue (.orientation _array_element) (.pathswitch _array_element))
                (else
                  (bind _returnvalue_2 (Game|SpawnActorfromClass "/Game/BluePrint/Grid/Path/BP_PathBlock.BP_PathBlock_C" (Math|Conversions|ToTransform(Vector) _poly_center) "AlwaysSpawn" "MultiplyWithRoot" 0 0))
                  (Default|SetPathBlock _returnvalue_2 (.orientation _array_element) (.pathswitch _array_element))))
              (Variables|Grid|SethasSpawnedPath true)
              (goto _label Break)))
          (:Completed
            (if (not (Variables|Grid|GethasSpawnedPath))
              ;[1 1 1] Grid Cell
              (Game|SpawnActorfromClass "/Game/BluePrint/Grid/BP_GridBlock.BP_GridBlock_C" (Math|Transform|MakeTransform (Math|Vector|MakeVector (.X (Math|Vector|BreakVector _poly_center)) (.Y (Math|Vector|BreakVector _poly_center)) (.Z (Math|Vector|BreakVector _poly_center))) "0, 0, 0" "1.000000,1.000000,1.000000") "AlwaysSpawn" "MultiplyWithRoot" 0 0))))))))

(fn ConstructionScript
  (if (Variables|DEBUGGING|GetTest)
    (bind (_current_point _total_points _0_1_phase _poly_center _x_row _y_row) (Utilities|2DGridExecutionMacro (Variables|Grid|Getoffset) (Transformation|GetActorLocation) (Variables|Grid|Getcolumns) (Variables|Grid|Getrows))
      (:Per%20Poly%20Execution
        (Variables|Grid|SethasSpawnedPath false)
        (bind _array_element (Utilities|Array|ForEachLoopwithBreak (Variables|Grid|Getpath) :!label _label)
          (:LoopBody
            (if (and (== (.x _array_element) _x_row) (== (.y _array_element) _y_row))
              (if (.canSwitch (Utilities|Struct|BreakS_PathSwitch (.pathswitch _array_element)))
                ;[1 1 1] Path Cell
                (bind _returnvalue (AddComponent|AddStaticMeshComponent false (Math|Transform|MakeTransform (Math|Vector|MakeVector (.X (Math|Vector|BreakVector _poly_center)) (.Y (Math|Vector|BreakVector _poly_center)) -5e+01) "0, 0, 0" "1.000000,1.000000,1.000000")))
                (else
                  (bind _returnvalue_2 (AddComponent|AddStaticMeshComponent false (Math|Transform|MakeTransform (Math|Vector|MakeVector (.X (Math|Vector|BreakVector _poly_center)) (.Y (Math|Vector|BreakVector _poly_center)) -5e+01) "0, 0, 0" "1.000000,1.000000,1.000000")))))
              (Variables|Grid|SethasSpawnedPath true)
              (if (.startingcell _array_element)
                (Rendering|Material|SetMaterial _returnvalue_2 0 "/Game/Materials/MI_Red.MI_Red")
                (goto _label Break))))
          (:Completed
            (if (not (Variables|Grid|GethasSpawnedPath))
              ;[1 1 1] Grid Cell
              (AddComponent|AddStaticMeshComponent false (Math|Transform|MakeTransform (Math|Vector|MakeVector (.X (Math|Vector|BreakVector _poly_center)) (.Y (Math|Vector|BreakVector _poly_center)) -5e+01) "0, 0, 0" "1.000000,1.000000,1.000000")))))))))