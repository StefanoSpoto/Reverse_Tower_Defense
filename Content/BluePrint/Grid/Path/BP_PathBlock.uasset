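; BP_PathBlock is a grid path cell that faces a compass direction and can switch between the directions listed in its Orientation array.
; Construction defaults an empty list to East, applies the first entry as yaw rotation, tints multi-direction blocks blue and trims a four-entry list to three.
; SwitchOrientation steps through the list with wraparound, rotating the actor.
; At BeginPlay, blocks without multiple directions hide their arrow.
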(event EventBeginPlay
  (if (not (> (Utilities|Array|Length (Variables|Path|Getorientation)) 1))
    (Rendering|SetVisibility (Variables|Default|GetArrow) false false)))

(event Collision|EventActorBeginOverlap
  (params (OtherActor :type Actor%20Object%20Reference)))

(fn ConstructionScript
  (bind _orientation (Variables|Path|Getorientation))
  (bind _orientation_2 (Variables|Path|Getorientation))
  (Orientation|SetPathCellOrientation)
  (if (> (Utilities|Array|Length (Variables|Path|Getorientation)) 1)
    (Rendering|Material|SetMaterial (Variables|Default|GetCube) 0 "/Game/Materials/Test/MI_Blue.MI_Blue")
    (if (== (Utilities|Array|Length _orientation) 4)
      (Utilities|Array|RemoveIndex _orientation 3))
    (elif (== (Utilities|Array|Length _orientation_2) 0)
      (Utilities|Array|Add _orientation_2 "NewEnumerator2"))))

(fn SetPathCellOrientation
  (params (orientationArrayIndex :type Integer))
  (switch Utilities|FlowControl|Switch|SwitchonE_PathOrientation (Utilities|Array|Get(acopy) (Variables|Path|Getorientation) orientationArrayIndex)
    (:NewEnumerator2
      (CallFunction|SetCellRotation "0, 0, 0"))
    (:NewEnumerator3
      (CallFunction|SetCellRotation "0.000000,180.000000,0.000000"))
    (:NewEnumerator0
      (CallFunction|SetCellRotation "0.000000,-90.000000,0.000000"))
    (:NewEnumerator1
      (CallFunction|SetCellRotation "0.000000,90.000000,0.000000"))))

(fn SetCellRotation
  (params (rotation :type Rotator))
  (Transformation|SetActorRotation rotation))

(fn GetPathCellOrientation
  (return (Transformation|GetWorldRotation (Variables|Default|GetCube))))

(fn SwitchOrientation
  (bind _result (Math|Integer|IncrementInt (Variables|Default|GetorientationsIndex))
    (:%20%20
      (if (< _result (Utilities|Array|Length (Variables|Path|Getorientation)))
        _
        (else
          (Variables|Default|SetorientationsIndex 0)))
      (Orientation|SetPathCellOrientation (Variables|Default|GetorientationsIndex)))))