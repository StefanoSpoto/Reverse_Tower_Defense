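; Grid block that holds an army of units and spawns them in the reverse tower defense level.
; Before spawning starts, clicking toggles selection through the level GameMode, whose selection event deselects spawners, with a highlight material showing the state.
; The GameInstance's start-spawning event disables clicking and enables spawning.
; Tick then uses a CanSpawn gate and per-unit Delay to spawn each BP_Unit in army order, applying its stats.
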(event Custom|SpawnStart
  (Variables|Default|SetcanSpawn true)
  (Rendering|Material|SetMaterial (Variables|Default|GetUnitSpawnHighlight) 0 "/Game/Materials/Programmers_Material/M_TransparentGradient.M_TransparentGradient")
  (Variables|Default|Setclickable false))

(event Custom|OnOtherSpawnerSelected
  (CallFunction|SelectSpawner false))

(event EventBeginPlay
  (|CallParentFunction)
  (EventDispatchers|BindEventtoOnStartSpawning (CallFunction|GetGIReverseTD) (delegate Custom|SpawnStart))
  (Variables|Default|SetcanSpawn false)
  (EventDispatchers|BindEventtoOnSelectSpawner (CallFunction|GetGMLevelGameMode) (delegate Custom|OnOtherSpawnerSelected)))

(event MouseInput|EventActorOnClicked
  (params (ButtonPressed :type Key%20Structure :default "None"))
  ;[1 1 1] Quando viene cliccato,viene salvata una sua reference dentro alla GameMode, in modo da essere accessibile dalla UI
  (if (Variables|Default|Getclickable)
    (if (Variables|Default|Getselected)
      (Default|SetClickedSpawner (CallFunction|GetGMLevelGameMode) self false)
      (else
        (Default|SetClickedSpawner (CallFunction|GetGMLevelGameMode) self true)))))

(event EventTick
  (params (DeltaSeconds :type Float%20%28single-precision%29))
  (bind _army (Variables|Default|Getarmy))
  (bind _spawnindex (Variables|Default|GetspawnIndex))
  (bind _output (Utilities|Array|Get(acopy) _army _spawnindex))
  (if (and (Variables|Default|GetcanSpawn) (> (Utilities|Array|Length (Variables|Default|Getarmy)) 0))
    (Variables|Default|SetcanSpawn false)
    (Utilities|FlowControl|Delay (Variables|/Game/BluePrint/Units/DataAssets/DA_Unit.DA_Unit_C|GetspawnTime _output))
    (bind _returnvalue (Game|SpawnActorfromClass "/Game/BluePrint/Units/BP_Unit.BP_Unit_C" (Transformation|GetWorldTransform (Variables|Default|GetUnitSpawnPoint)) "AlwaysSpawn" "MultiplyWithRoot" 0 0))
    (Default|SetStats _returnvalue _output)
    (bind _result (Math|Integer|IncrementInt (Variables|Default|GetspawnIndex))
      (:%20%20
        (if (> _result (Utilities|Array|LastIndex (Variables|Default|Getarmy)))
          (Variables|Default|SetcanSpawn false)
          (else
            (Variables|Default|SetcanSpawn true)))))))

(event Collision|EventActorBeginOverlap
  (params (OtherActor :type Actor%20Object%20Reference))
  (|CallParentFunction OtherActor) ; This node is disabled and will not be called.\nDrag off pins to build functionality.
)

(fn ConstructionScript
  (|CallParentFunction))

(fn SelectSpawner
  (params (selected :type Boolean))
  (bind _output_get (Variables|Default|Setselected selected))
  (if _output_get
    (Rendering|Material|SetMaterial (Variables|Default|GetUnitSpawnHighlight) 0 "/Game/Materials/Programmers_Material/MI_GreenTG.MI_GreenTG")
    (else
      (Rendering|Material|SetMaterial (Variables|Default|GetUnitSpawnHighlight) 0 "/Game/Materials/Programmers_Material/M_TransparentGradient.M_TransparentGradient"))))

(fn GetUnitSpawnPosition
  (return (Transformation|GetWorldLocation (Variables|Default|GetUnitSpawnHighlight))))

(fn AddUnittoArmy
  (params (Unit :type DA%20Unit%20Object%20Reference))
  (Utilities|Array|Add (Variables|Default|Getarmy) Unit))

(fn RemoveUnitfromArmy
  (params (unitIndex :type Integer))
  (Utilities|Array|RemoveIndex (Variables|Default|Getarmy) unitIndex))