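; BP_StartingPathBlock is a grid path block that serves as the starting point where units spawn.
; It exposes the world location of its UnitSpawnPosition component as the spawn point.
; SetDragUnitOn shows or hides that component according to whether a unit is dragged onto the block.
; The event graph holds no active logic.
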(event EventBeginPlay
  (|CallParentFunction) ; This node is disabled and will not be called.\nDrag off pins to build functionality.
)

(event Collision|EventActorBeginOverlap
  (params (OtherActor :type Actor%20Object%20Reference))
  (|CallParentFunction OtherActor) ; This node is disabled and will not be called.\nDrag off pins to build functionality.
)

(event EventTick
  (params (DeltaSeconds :type Float%20%28single-precision%29)))

(fn ConstructionScript
  (|CallParentFunction))

(fn SetDragUniton
  (params (draggedOn :type Boolean))
  (bind _unitspawnposition (Variables|Default|GetUnitSpawnPosition))
  (if draggedOn
    (Rendering|SetVisibility _unitspawnposition true false)
    (else
      (Rendering|SetVisibility _unitspawnposition false false))))

(fn GetUnitSpawnPosition
  (return (Transformation|GetWorldLocation (Variables|Default|GetUnitSpawnPosition))))