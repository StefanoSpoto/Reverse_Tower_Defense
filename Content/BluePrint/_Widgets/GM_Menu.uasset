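; Menu game mode that loads save data on BeginPlay, shows the main menu widget and switches to UI-only input with the mouse cursor.
; Navigation functions toggle visibility between main, hero selection, army selection and options screens.
; Army and options widgets are created once and reused, while hero selection is recreated on each visit.
; It also relays troop and commander picks to those widgets and saves to the SaveData slot.
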(event EventBeginPlay
  (bind _returnvalue (Game|GetPlayerController 0))
  (Default|LoadSaveData (CallFunction|GetGIReverseTD))
  (bind _returnvalue_2 (UserInterface|CreateWidget "/Game/BluePrint/_Widgets/Menus/W_MainMenu.W_MainMenu_C"))
  (UserInterface|Viewport|AddtoViewport _returnvalue_2 0)
  (bind _output_get (Variables|UI|SetmainMenu _returnvalue_2))
  (Variables|/Script/Engine.PlayerController|SetbShowMouseCursor _returnvalue true)
  (Input|SetInputModeUIOnly _returnvalue _output_get "DoNotLock" false))

(fn ConstructionScript)

(fn GotoArmySelection
  (Utilities|IsValid (Variables|UI|GetarmySelectionMenu)
    (:Is%20Valid
      (Widget|SetVisibility (Variables|UI|GetarmySelectionMenu) "Visible"))
    (:Is%20Not%20Valid
      (bind _returnvalue (UserInterface|CreateWidget "/Game/BluePrint/_Widgets/Menus/Army_Creation/W_ArmySelection.W_ArmySelection_C"))
      (UserInterface|Viewport|AddtoViewport _returnvalue 0)
      (Variables|UI|SetarmySelectionMenu _returnvalue))))

(fn GoBacktoChampionSelection
  (Widget|SetVisibility (Variables|UI|GetarmySelectionMenu) "Hidden")
  (Widget|SetVisibility (Variables|UI|GetcommanderSelectionMenu) "Visible"))

(fn SetSelectedTroop
  (params (troop :type DA%20Troop%20Object%20Reference))
  (bind _asw_army_selection (Utilities|Casting|CastToW_ArmySelection (Variables|UI|GetarmySelectionMenu)))
  (Default|SetSelectedTroop _asw_army_selection troop))

(fn GotoChampionSelection
  (Widget|SetVisibility (Variables|UI|GetmainMenu) "Hidden")
  (bind _returnvalue (UserInterface|CreateWidget "/Game/BluePrint/_Widgets/Menus/Commander_Selection/W_HeroSelection.W_HeroSelection_C"))
  (UserInterface|Viewport|AddtoViewport _returnvalue 0)
  (Variables|UI|SetcommanderSelectionMenu _returnvalue))

(fn GoBacktoMainMenu
  (Widget|SetVisibility (Variables|UI|GetcommanderSelectionMenu) "Hidden")
  (Widget|SetVisibility (Variables|UI|GetmainMenu) "Visible"))

(fn SetIndextoRemove
  (params (index :type Integer))
  (bind _asw_army_selection (Utilities|Casting|CastToW_ArmySelection (Variables|UI|GetarmySelectionMenu)))
  (Default|SetIndextoRemove _asw_army_selection index))

(fn CommanderSelected
  (params (commander :type DA%20Commander%20Object%20Reference))
  (bind _asw_hero_selection (Utilities|Casting|CastToW_HeroSelection (Variables|UI|GetcommanderSelectionMenu)))
  (Default|SetSelectedCommander _asw_hero_selection commander))

(fn SaveGame
  (bind _returnvalue (SaveGame|SaveGametoSlot (Variables|Default|GetSaveSystem) "SaveData"))
  (return _returnvalue))

(fn GotoOptionsMenu
  (Utilities|IsValid (Variables|UI|GetOptionsMenu)
    (:Is%20Valid
      (Widget|SetVisibility (Variables|UI|GetOptionsMenu) "Visible"))
    (:Is%20Not%20Valid
      (bind _returnvalue (UserInterface|CreateWidget "/Game/BluePrint/_Widgets/Menus/W_OptionMenu.W_OptionMenu_C"))
      (UserInterface|Viewport|AddtoViewport _returnvalue 0)
      (Variables|UI|SetOptionsMenu _returnvalue))))

(fn GoBackfromOptions
  (Widget|SetVisibility (Variables|UI|GetOptionsMenu) "Hidden"))